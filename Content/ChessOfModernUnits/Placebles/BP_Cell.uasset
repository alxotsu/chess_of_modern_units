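; BP_Cell is a placeable board tile for Chess of Modern Units, defined by its grid coordinates and landscape type.
; On BeginPlay it sets its material or hides the cube for player bases, then positions itself from its coordinates, raising hills.
; Left clicks send the coordinates to BP_PlayerController for selection.
; On hover, the controller's move check decides whether a point light shows and whether it is green or red.
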(event `self.ReceiveBeginPlay`
  (bind _cube1 (`self.Cube1`))
  (bind _cube1_2 (`self.Cube1`))
  (bind (_xcoord _ycoord) (break `/Game/ChessOfModernUnits/Placebles/SFieldCellCoords` (`self.Coords`)))
  (switch `/Game/ChessOfModernUnits/Placebles/ELandscapeType` (`self.LandscapeType`)
    (:`NewEnumerator0`
      (`PrimitiveComponent.SetMaterial` _cube1_2 0 (`self.CellMaterial`)))
    (:`NewEnumerator1`
      (`PrimitiveComponent.SetMaterial` _cube1_2 0 "/Game/ChessOfModernUnits/Placebles/Materials/MI_CellHill.MI_CellHill"))
    (:`NewEnumerator2`
      (`PrimitiveComponent.SetMaterial` _cube1 0 "/Game/ChessOfModernUnits/Placebles/Materials/MI_CellWater.MI_CellWater"))
    (:`NewEnumerator3`
      (`SceneComponent.SetVisibility` _cube1 false true)))
  (`SceneComponent.K2_SetWorldLocation` (`self.DefaultSceneRoot`) (`KismetMathLibrary.MakeVector` (`KismetMathLibrary.Conv_IntToDouble` (* _xcoord 100)) (`KismetMathLibrary.Conv_IntToDouble` (* _ycoord 100)) (select `/Game/ChessOfModernUnits/Placebles/ELandscapeType` (`self.LandscapeType`) :`NewEnumerator1` 40.0)) false false))

(event `self.ReceiveActorOnClicked`
  (params (ButtonPressed :type "Key Structure"))
  (if (== ButtonPressed "LeftMouseButton")
    (bind _asbp_player_controller (cast `/Game/ChessOfModernUnits/Controls/OneVsOne/BP_PlayerController` (`GameplayStatics.GetPlayerController` 0)))
    (`/Game/ChessOfModernUnits/Controls/OneVsOne/BP_PlayerController.SelectCelllEvent` _asbp_player_controller (`self.Coords`))))

(event `self.ReceiveActorBeginCursorOver`
  (bind _pointlight (`self.PointLight`))
  (bind _asbp_player_controller (cast `/Game/ChessOfModernUnits/Controls/OneVsOne/BP_PlayerController` (`GameplayStatics.GetPlayerController` 0)))
  (bind (_light _possible) (`/Game/ChessOfModernUnits/Controls/OneVsOne/BP_PlayerController.MoveOnCoordInPossibles` _asbp_player_controller (`self.Coords`)))
  (`SceneComponent.SetVisibility` _pointlight _light false)
  (`LightComponent.SetLightColor` _pointlight (select `bool` _possible :`false` (struct :`R` 1.0 :`A` 1.0) :`true` (struct :`R` 0.15 :`G` 1.0 :`B` 0.15 :`A` 1.0) :!type "LinearColor Structure") true))

(event `self.ReceiveActorEndCursorOver`
  (`SceneComponent.SetVisibility` (`self.PointLight`) false false))

(fn `UserConstructionScript`)