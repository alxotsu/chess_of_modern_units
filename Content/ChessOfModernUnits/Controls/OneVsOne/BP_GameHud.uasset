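; HUD for a one-vs-one unit game that previews planned moves with holograms and manages unit-control and game-status widgets.
; It replays moves through MoveMaker on a copy of the saved field, then spawns color-coded holograms for the moved unit and same-side or opposing units at target cells.
; Widgets route through a lazily created master widget.
; SelectUnit_1 is empty, and its apparent selection logic is disconnected.
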(event `OpenWayCalculator`
  (params (CalculatedWays :type "Map of /Game/ChessOfModernUnits/Units/Components/EDirection Enum to /Game/ChessOfModernUnits/Controls/OneVsOne/SMoveList Structure" :default _))
  (bind _aswbp_unit_control (cast `/Game/ChessOfModernUnits/Controls/OneVsOne/UI/WBP_UnitControl` (`/Game/ChessOfModernUnits/Controls/Common/WBP_MasterWidget.GetWidgetByClass` (`self.GetMasterWidget`) "/Game/ChessOfModernUnits/Controls/OneVsOne/UI/WBP_UnitControl.WBP_UnitControl_C")))
  (`/Game/ChessOfModernUnits/Controls/OneVsOne/UI/WBP_UnitControl.OpenMoveCalculator` _aswbp_unit_control CalculatedWays (`self.SelectedHologram`)))

(event `VisualizeMoves`
  (params (Moves :type "Array of /Game/ChessOfModernUnits/Units/SUnitMove Structure (by ref)") (EnableConfirmButton :type Boolean))
  (bind (_outputtempfield _outputtempunit) (`self.VisualizeMovesF` Moves))
  (`self.VisualizePossibleMoves` _outputtempfield _outputtempunit)
  (bind _aswbp_unit_control (cast `/Game/ChessOfModernUnits/Controls/OneVsOne/UI/WBP_UnitControl` (`/Game/ChessOfModernUnits/Controls/Common/WBP_MasterWidget.GetWidgetByClass` (`self.GetMasterWidget`) "/Game/ChessOfModernUnits/Controls/OneVsOne/UI/WBP_UnitControl.WBP_UnitControl_C")))
  (`/Game/ChessOfModernUnits/Controls/OneVsOne/UI/WBP_UnitControl.ShowUnitInfo` _aswbp_unit_control _outputtempunit)
  (`Widget.SetIsEnabled` (`/Game/ChessOfModernUnits/Controls/OneVsOne/UI/WBP_UnitControl.ButtonUndoMovement` _aswbp_unit_control) (> (`KismetArrayLibrary.Array_Length` Moves) 0))
  (`Widget.SetIsEnabled` (`/Game/ChessOfModernUnits/Controls/OneVsOne/UI/WBP_UnitControl.ButtonConfirmMove` _aswbp_unit_control) EnableConfirmButton))

(event `SelectUnit_1`
  (params (FieldState :type "/Game/ChessOfModernUnits/Placebles/SFieldConfig Structure")))

(event `UnselectUnit_1`
  (bind _aswbp_unit_control (cast `/Game/ChessOfModernUnits/Controls/OneVsOne/UI/WBP_UnitControl` (`/Game/ChessOfModernUnits/Controls/Common/WBP_MasterWidget.GetWidgetByClass` (`self.GetMasterWidget`) "/Game/ChessOfModernUnits/Controls/OneVsOne/UI/WBP_UnitControl.WBP_UnitControl_C")))
  (`/Game/ChessOfModernUnits/Controls/OneVsOne/UI/WBP_UnitControl.CloseMoveCalculator` _aswbp_unit_control)
  (bind _outactors (`GameplayStatics.GetAllActorsOfClass` "/Game/ChessOfModernUnits/Units/BP_UnitHologram.BP_UnitHologram_C"))
  (`self.K2_DestroyActor` _outactors)
  (`BlueprintSetLibrary.Set_Clear` (`self.PossibleUnitsHolograms`))
  (`/Game/ChessOfModernUnits/Controls/Common/WBP_MasterWidget.DeactivateWidget` (`self.GetMasterWidget`) "/Game/ChessOfModernUnits/Controls/OneVsOne/UI/WBP_UnitControl.WBP_UnitControl_C"))

(event `ShowGameState_1`
  (params (StateName :type Name))
  (bind _widget (`self.GetMasterWidget`))
  (if (== StateName "ReadyToMove")
    (`/Game/ChessOfModernUnits/Controls/Common/WBP_MasterWidget.ToggleWidget` _widget "/Game/ChessOfModernUnits/Controls/OneVsOne/UI/WBP_UnitControl.WBP_UnitControl_C")
    (`/Game/ChessOfModernUnits/Controls/Common/WBP_MasterWidget.ToggleWidget` _widget "/Game/ChessOfModernUnits/Controls/OneVsOne/UI/WBP_UnitControl.WBP_UnitControl_C")
    (else
      (bind _widgetobj (`/Game/ChessOfModernUnits/Controls/Common/WBP_MasterWidget.ActivateWidget` _widget "/Game/ChessOfModernUnits/Controls/OneVsOne/UI/WBP_GameStatus.WBP_GameStatus_C"))
      (bind _aswbp_game_status (cast `/Game/ChessOfModernUnits/Controls/OneVsOne/UI/WBP_GameStatus` _widgetobj))
      (`/Game/ChessOfModernUnits/Controls/OneVsOne/UI/WBP_GameStatus.ShowStatus` _aswbp_game_status StateName))))

(fn `GetMasterWidget`
  (returns (widget :type "/Game/ChessOfModernUnits/Controls/Common/WBP_MasterWidget Object Reference"))
  (bind _foundwidgets (`WidgetBlueprintLibrary.GetAllWidgetsOfClass` "/Game/ChessOfModernUnits/Controls/Common/WBP_MasterWidget.WBP_MasterWidget_C"))
  (bind _output (`|GetArrayItem` _foundwidgets))
  (`/Engine/EditorBlueprintResources/StandardMacros.IsValid` _output
    (:`Is Valid`
      (bind _aswbp_master_widget (cast `/Game/ChessOfModernUnits/Controls/Common/WBP_MasterWidget` _output))
      (return _aswbp_master_widget))
    (:`Is Not Valid`
      (bind _returnvalue (`|CreateWidget` "/Game/ChessOfModernUnits/Controls/Common/WBP_MasterWidget.WBP_MasterWidget_C" null (`|MakeMap` "/Game/ChessOfModernUnits/Controls/OneVsOne/UI/WBP_UnitControl.WBP_UnitControl_C" 0 "/Game/ChessOfModernUnits/Controls/OneVsOne/UI/WBP_GameStatus.WBP_GameStatus_C" :!type "UserWidget Class Reference")))
      (`UserWidget.AddToViewport` _returnvalue 0)
      (return _returnvalue))))

(fn `MakeHologram`
  (params (Config :type "FallbackStruct Structure") (Color :type "LinearColor Structure") (Light :type Boolean))
  (returns (Hologram :type "/Game/ChessOfModernUnits/Units/BP_UnitHologram Object Reference"))
  (bind _outactors (`GameplayStatics.GetAllActorsOfClass` "/Game/ChessOfModernUnits/Units/BP_UnitHologram.BP_UnitHologram_C"))
  (for _array_element _outactors
    (bind _unit_config_coords (break `` (`/Game/ChessOfModernUnits/Units/BP_Unit.Unit Config` _array_element)))
    (if (`/Game/ChessOfModernUnits/Core/BPFL_CustomUtilits.EqualCoords` _unit_config_coords (`.Coords_47_E98C47904C4A4C6B43CCA291531B50D8` (break `FallbackStruct` Config)))
      (`/Game/ChessOfModernUnits/Units/BP_Unit.SetConfig` _array_element Config)
      (`/Game/ChessOfModernUnits/Units/BP_UnitHologram.Set Color` _array_element (`local.Color`) (`local.Light`))
      (return _array_element)))
  (bind _returnvalue (`|SpawnActorFromClass` "/Game/ChessOfModernUnits/Units/BP_UnitHologram.BP_UnitHologram_C" (`KismetMathLibrary.MakeTransform` (0.0 0.0 0.0)) "Undefined" "MultiplyWithRoot" null Color Light (struct) null Config))
  (return _returnvalue))

(fn `UserConstructionScript`)

(fn `VisualizeMovesF`
  (params (Moves :type "Array of /Game/ChessOfModernUnits/Units/SUnitMove Structure"))
  (returns (OutputTempField :type "/Game/ChessOfModernUnits/Placebles/SFieldConfig Structure") (OutputTempUnit :type "FallbackStruct Structure"))
  (locals (TempUnit :type " Structure") (TempField :type "/Game/ChessOfModernUnits/Placebles/SFieldConfig Structure"))
  (bind _tempfield (`local.TempField`))
  (bind _tempunit (`local.TempUnit`))
  (bind (_coords _side) (break `FallbackStruct` (`local.TempUnit`)))
  (`|ExecutionSequence`
    (:`then_0`
      (bind _outactors (`GameplayStatics.GetAllActorsOfClass` "/Game/ChessOfModernUnits/Units/BP_UnitHologram.BP_UnitHologram_C"))
      (`self.K2_DestroyActor` _outactors)
      (set `local.TempUnit` (struct))
      (set `local.TempField` (`self.SavedFieldState`))
      (`BlueprintSetLibrary.Set_Clear` (`self.PossibleUnitsHolograms`)))
    (:`then_1`
      (for _array_element Moves
        (bind (_newfieldstate _possible _newunit) (`/Game/ChessOfModernUnits/Core/BP_MoveMakerComponent.ComputeOneMove` (`self.MoveMaker`) _tempfield _array_element _tempunit))
        (bind _output_get (set `local.TempField` _newfieldstate))
        (set `local.TempUnit` _newunit)
        (bind ((`TargetCoords_19_2070F9A84A98EEC52500C0B0A346909D` _targetcoords)) (break `/Game/ChessOfModernUnits/Units/SUnitMove` _array_element))
        (bind (_value _returnvalue) (`BlueprintMapLibrary.Map_Find` (`.Units_31_8194BC274A1D6B758B12AA93D64CC056` (break `/Game/ChessOfModernUnits/Placebles/SFieldConfig` _output_get)) _targetcoords))
        (if (and _returnvalue (not (`/Game/ChessOfModernUnits/Core/BPFL_CustomUtilits.EqualCoords` _targetcoords _coords)))
          (`self.MakeHologram` (select `bool` (`|EnumEquality` (`.Side_59_393DC6B94AC999E7C6758C8FD57E2723` (break `FallbackStruct` _value)) _side) :`false` (struct :`R` 1.0 :`A` 0.7) :`true` (struct :`G` 1.0 :`B` 1.0 :`A` 0.7) :!type "LinearColor Structure") true _value))))
    (:`then_2`
      (bind _hologram (`self.MakeHologram` (struct :`G` 1.0 :`A` 0.7) true (`local.TempUnit`)))
      (set `self.SelectedHologram` _hologram)
      (return _tempfield _tempunit))))

(fn `VisualizePossibleMoves`
  (params (FieldState :type "/Game/ChessOfModernUnits/Placebles/SFieldConfig Structure") (UnitConfig :type "FallbackStruct Structure"))
  (bind _possibleunitsholograms (`self.PossibleUnitsHolograms`))
  (bind (_coords _side) (break `FallbackStruct` (`/Game/ChessOfModernUnits/Units/BP_Unit.Unit Config` (`self.SelectedHologram`))))
  (bind _result (`BlueprintSetLibrary.Set_ToArray` _possibleunitsholograms))
  (`self.K2_DestroyActor` _result)
  (`BlueprintSetLibrary.Set_Clear` _possibleunitsholograms)
  (bind _socket (`self.GetSelectedSocket`))
  (bind _moves (`/Game/ChessOfModernUnits/Core/BP_MoveMakerComponent.GetPossibleMoves` (`self.MoveMaker`) FieldState UnitConfig))
  (bind _result_2 (`BlueprintSetLibrary.Set_ToArray` _moves))
  (for _array_element _result_2
    (bind ((`ActiveComponent_20_EA598D07478AB8A33D4C1F99ECAC8CF4` _activecomponent) (`TargetCoords_19_2070F9A84A98EEC52500C0B0A346909D` _targetcoords)) (break `/Game/ChessOfModernUnits/Units/SUnitMove` _array_element))
    (bind (_value _returnvalue) (`BlueprintMapLibrary.Map_Find` (`.Units_31_8194BC274A1D6B758B12AA93D64CC056` (break `/Game/ChessOfModernUnits/Placebles/SFieldConfig` (`self.SavedFieldState`))) _targetcoords))
    (if (and (or (== _activecomponent "Main") (== _activecomponent _socket)) _returnvalue (not (`/Game/ChessOfModernUnits/Core/BPFL_CustomUtilits.EqualCoords` _targetcoords _coords)))
      (bind _hologram (`self.MakeHologram` (select `bool` (`|EnumEquality` (`.Side_59_393DC6B94AC999E7C6758C8FD57E2723` (break `FallbackStruct` _value)) _side) :`false` (struct :`R` 1.0 :`A` 0.7) :`true` (struct :`G` 1.0 :`B` 1.0 :`A` 0.7) :!type "LinearColor Structure") false _value))
      (`BlueprintSetLibrary.Set_Add` (`self.PossibleUnitsHolograms`) _hologram))))