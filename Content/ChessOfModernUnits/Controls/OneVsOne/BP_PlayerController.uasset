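; Player controller for a one-versus-one, turn-based grid unit game that handles unit selection and move planning on the player's turn.
; Cell selection picks a friendly unit and caches possible moves from MoveMaker for its main and socket components.
; Chosen socket moves accumulate, are validated by MoveMaker against a saved field copy, and are previewed through the HUD.
; Confirm, cancel, undo and server submission are empty stubs, and main-component moves are only checked.
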(event `self.ReceiveBeginPlay`
  (bind _returnvalue (subsystem `EnhancedInputLocalPlayerSubsystem`))
  (`/Engine/EditorBlueprintResources/StandardMacros.IsValid` _returnvalue
    (:`Is Valid`
      (`EnhancedInputSubsystemInterface.AddMappingContext` _returnvalue "/Game/ChessOfModernUnits/Controls/OneVsOne/Input/IMC_MainGameActions.IMC_MainGameActions" 0 (struct))
      (bind _asbp_game_state (cast `/Game/ChessOfModernUnits/Core/BP_GameState` (`GameplayStatics.GetGameState`)))
      (set `self.Move Maker` (`/Game/ChessOfModernUnits/Core/BP_GameState.MoveMaker` _asbp_game_state))
      (bind _output_get (set `self.SavedFieldState` (`/Game/ChessOfModernUnits/Core/BP_GameState.FieldState` _asbp_game_state)))
      (`KismetSystemLibrary.PrintString` (`KismetStringLibrary.Conv_IntToString` (`.SizeX_4_E00CBD1E48A314DE3ADC33A00597C3F1` (break `/Game/ChessOfModernUnits/Placebles/SFieldConfig` _output_get)))))))

(event `EnhancedInput|/Game/ChessOfModernUnits/Controls/OneVsOne/Input/Actions/TankControl/IA_ConfirmMove`
  (params (ActionValue :type Boolean) (ElapsedSeconds :type "Float (double-precision)") (TriggeredSeconds :type "Float (double-precision)") (InputAction :type "InputAction Object Reference" :default "/Game/ChessOfModernUnits/Controls/OneVsOne/Input/Actions/TankControl/IA_ConfirmMove.IA_ConfirmMove"))
  (:`Started`
    (`self.MakeMove`)))

(event `EnhancedInput|/Game/ChessOfModernUnits/Controls/OneVsOne/Input/Actions/TankControl/IA_CancelMove`
  (params (ActionValue :type Boolean) (ElapsedSeconds :type "Float (double-precision)") (TriggeredSeconds :type "Float (double-precision)") (InputAction :type "InputAction Object Reference" :default "/Game/ChessOfModernUnits/Controls/OneVsOne/Input/Actions/TankControl/IA_CancelMove.IA_CancelMove"))
  (:`Started`
    (`self.ResetMove`)))

(event `EnhancedInput|/Game/ChessOfModernUnits/Controls/OneVsOne/Input/Actions/TankControl/IA_UndoMovement`
  (params (ActionValue :type Boolean) (ElapsedSeconds :type "Float (double-precision)") (TriggeredSeconds :type "Float (double-precision)") (InputAction :type "InputAction Object Reference" :default "/Game/ChessOfModernUnits/Controls/OneVsOne/Input/Actions/TankControl/IA_UndoMovement.IA_UndoMovement"))
  (:`Started`
    (`self.UndoMovement`)))

(event `SelectCelllEvent`
  (params (Coords :type "/Game/ChessOfModernUnits/Placebles/SFieldCellCoords Structure"))
  (bind _move_maker (`self.Move Maker`))
  (bind _savedfieldstate (`self.SavedFieldState`))
  (bind (_landscape _cellfound _unit _unitfound) (`/Game/ChessOfModernUnits/Core/BPFL_CustomUtilits.GetCellFromField` (`self.SavedFieldState`) Coords))
  (bind (_value _returnvalue) (`BlueprintMapLibrary.Map_Find` (`self.PossibleMovesOther`) (`self.SelectedSocket`)))
  (bind ((`Alive_1_4876116A47F2527D46E553BF84858816` _alive) (`Side_4_4F74B15B4D5D30D6A78E1BA957F509DB` _side)) (break `/Game/ChessOfModernUnits/Units/SUnitConfig` _unit))
  (bind ((`Coords_7_9C7BED8F4B2205EF8B5C87A1962D4680` _coords)) (break `/Game/ChessOfModernUnits/Units/SUnitConfig` _unit))
  (bind _asbp_player_state (cast `/Game/ChessOfModernUnits/Core/BP_PlayerState` (`self.PlayerState`)))
  (if (and (`self.CanMakeMove`) _cellfound)
    (if (`self.UnitSelected`)
      (if _unitfound
        (if _returnvalue
          (for _array_element (`.Moves_6_0ACB620140D29225A4E09AAB1EB5BCE4` (break `/Game/ChessOfModernUnits/Controls/OneVsOne/SMoveList` _value))
            (bind ((`TargetCoords_19_2070F9A84A98EEC52500C0B0A346909D` _targetcoords) (`CoordsSpecified_25_1FDD0DC440D63BA9B8E7B8835DEA6D28` _coordsspecified)) (break `/Game/ChessOfModernUnits/Units/SUnitMove` _array_element))
            (if (and (`/Game/ChessOfModernUnits/Core/BPFL_CustomUtilits.EqualCoords` _targetcoords Coords) _coordsspecified)
              (`self.AddMove` _array_element)
              (break)))
          (elif (`.Possible` (`self.MoveOnCoordInPossibles` Coords))
            _)))
      (elif (and (`|EnumEquality` (`/Game/ChessOfModernUnits/Core/BP_PlayerState.side` _asbp_player_state) _side) _alive _unitfound)
        (set `self.UnitSelected` true)
        (set `self.SelectedUnit` _unit)
        (bind _possiblemoves (`/Game/ChessOfModernUnits/Core/BP_MoveMakerComponent.GetPossibleMovesViaMainComponent` _move_maker _savedfieldstate _coords))
        (set `self.PossibleMovesMain` _possiblemoves)
        (bind _possiblemoves_2 (`/Game/ChessOfModernUnits/Core/BP_MoveMakerComponent.GetPossibleMovesViaSocketComponents` _move_maker _savedfieldstate _coords))
        (set `self.PossibleMovesOther` _possiblemoves_2)))))

(event `MakeMove`)

(event `MakeMoveServer`
  (params (UnitCoords :type "/Game/ChessOfModernUnits/Placebles/SFieldCellCoords Structure") (Moves :type "Array of /Game/ChessOfModernUnits/Units/SUnitMove Structure (by ref)")))

(event `ResetMove`)

(event `UndoMovement`)

(event `PreMove`
  (`self.ResetMove`)
  (cast `/Game/ChessOfModernUnits/Core/BP_GameState` (`GameplayStatics.GetGameState`)))

(fn `AddMove`
  (params (Move :type "/Game/ChessOfModernUnits/Units/SUnitMove Structure"))
  (returns (Possible :type Boolean))
  (bind _moves (`self.Moves`))
  (if (and (`self.CanMakeMove`) (`self.UnitSelected`))
    (`KismetArrayLibrary.Array_Add` (`self.Moves`) Move)
    (bind (_possible _valid _fieldoutput) (`/Game/ChessOfModernUnits/Core/BP_MoveMakerComponent.ComputeMoves` (`self.Move Maker`) (`self.SavedFieldState`) (`.Coords_7_9C7BED8F4B2205EF8B5C87A1962D4680` (break `/Game/ChessOfModernUnits/Units/SUnitConfig` (`self.SelectedUnit`))) (`self.Moves`)))
    (if _possible
      (set `self.SavedFieldState` _fieldoutput)
      (bind _asbp_game_hud (cast `/Game/ChessOfModernUnits/Controls/OneVsOne/BP_GameHud` (`self.GetHUD`)))
      (`/Game/ChessOfModernUnits/Controls/OneVsOne/BP_GameHud.VisualizeMoves` _asbp_game_hud (`self.Moves`) _valid)
      (return true)
      (else
        (`KismetArrayLibrary.Array_Remove` _moves (- (`KismetArrayLibrary.Array_Length` _moves) 1))
        (return false)))
    (else
      (return false))))

(fn `CanMakeMove`
  (returns (Enabled :type Boolean))
  (bind _asbp_player_state (cast `/Game/ChessOfModernUnits/Core/BP_PlayerState` (`self.PlayerState`)))
  (bind _asbp_game_state (cast `/Game/ChessOfModernUnits/Core/BP_GameState` (`GameplayStatics.GetGameState`)))
  (return (and (`|EnumEquality` (`/Game/ChessOfModernUnits/Core/BP_GameState.Now Move Side` _asbp_game_state) (`/Game/ChessOfModernUnits/Core/BP_PlayerState.side` _asbp_player_state)) (== (`/Game/ChessOfModernUnits/Core/BP_GameState.StateName` _asbp_game_state) "ReadyToMove"))))

(fn `MoveOnCoordInPossibles`
  (params (Coords :type "/Game/ChessOfModernUnits/Placebles/SFieldCellCoords Structure"))
  (returns (Light :type Boolean) (Possible :type Boolean))
  (bind _returnvalue (and (`self.CanMakeMove`) (`self.UnitSelected`)))
  (if _returnvalue
    (bind _enumvalue (foreach `/Game/ChessOfModernUnits/Units/Components/EDirection` false)
      (:`LoopBody`
        (return true (`.ReturnValue` (`BlueprintMapLibrary.Map_Find` (`self.PossibleMovesMain`) (make `/Game/ChessOfModernUnits/Controls/OneVsOne/SDirectonAndCoords` _enumvalue Coords)))))
      (:`then`
        _)))
  (return _returnvalue false))

(fn `UserConstructionScript`)