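; Unit actor for a chess game, assembled and posed from a Config struct holding alive state, side, coords and components.
; BeginPlay passes Config through BPReplicationComponent when replicated, then runs four setters that each store their values and update visuals.
; These pitch dead units over, tint dynamic materials black or white, and place units on a 50-unit grid.
; SetComponents rebuilds the main skeletal mesh and attaches extra meshes to its named sockets.
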(event `self.ReceiveBeginPlay`
  (bind (_alive _side _coords _maincomponent _socketcomponents) (break `/Game/ChessOfModernUnits/Units/SUnitConfig` (`self.Config`)))
  (if (`self.bReplicates`)
    (bind _replconfig (`/Game/ChessOfModernUnits/Core/BP_ReplicationComponent.ReplicateUnitConfig` (`self.BP_ReplicationComponent`) (`self.Config`)))
    (set `self.Config` _replconfig))
  (`self.SetAlive` _alive)
  (`self.SetSide` _side)
  (`self.SetCoords` _coords)
  (`self.SetComponents` _maincomponent _socketcomponents))

(fn `SetAlive`
  (params (Alive :type Boolean))
  (bind _defaultsceneroot (`self.DefaultSceneRoot`))
  (bind (_returnvalue_roll _returnvalue_pitch _returnvalue_yaw) (`KismetMathLibrary.BreakRotator` (`SceneComponent.K2_GetComponentRotation` _defaultsceneroot)))
  (setmembers `/Game/ChessOfModernUnits/Units/SUnitConfig` :`StructRef` (`self.Config`) :`Alive` Alive)
  (`SceneComponent.K2_SetWorldRotation` _defaultsceneroot (`KismetMathLibrary.MakeRotator` _returnvalue_roll (select `bool` Alive :`false` 90.0 :!type "Float (single-precision)") _returnvalue_yaw) false false))

(fn `SetComponents`
  (params (MainComponent :type "/Game/ChessOfModernUnits/Units/Components/SUnitComponentConfig Structure") (SocketComponents :type "Map of Name to /Game/ChessOfModernUnits/Units/Components/SUnitComponentConfig Structure"))
  (bind _mesh (`self.Mesh`))
  (bind _defaultsceneroot (`self.DefaultSceneRoot`))
  (bind _config (`self.Config`))
  (bind ((`SocketComponents_19_0467C64B42DB044005745F8E30DB9361` _socketcomponents)) (break `/Game/ChessOfModernUnits/Units/SUnitConfig` (`self.Config`)))
  (bind (_returnvalue_roll _returnvalue_pitch) (`KismetMathLibrary.BreakRotator` (`SceneComponent.K2_GetComponentRotation` _defaultsceneroot)))
  (bind (_skeletalmesh _relativetransform) (`/Game/ChessOfModernUnits/Core/BPFL_CustomUtilits.GetMeshForUnitComponentConfig` (`.MainComponent_20_960460F54E1FCEC2EF6C488D79BB28EF` (break `/Game/ChessOfModernUnits/Units/SUnitConfig` _config)) true))
  (setmembers `/Game/ChessOfModernUnits/Units/SUnitConfig` :`StructRef` _config :`MainComponent` MainComponent :`SocketComponents` SocketComponents)
  (`ActorComponent.K2_DestroyComponent` (`SceneComponent.GetChildrenComponents` _mesh true))
  (`SkeletalMeshComponent.SetSkeletalMeshAsset` _mesh _skeletalmesh)
  (`SceneComponent.K2_SetRelativeTransform` _mesh (`KismetMathLibrary.MakeTransform` (.location _relativetransform) (`KismetMathLibrary.MakeRotator` (.roll (.rotation _relativetransform)) (.pitch (.rotation _relativetransform))) (.scale _relativetransform)) false false)
  (`SceneComponent.K2_SetWorldRotation` _defaultsceneroot (`KismetMathLibrary.MakeRotator` _returnvalue_roll _returnvalue_pitch (.yaw (.rotation _relativetransform))) false false)
  (bind _keys (`BlueprintMapLibrary.Map_Keys` _socketcomponents))
  (for _array_element _keys
    (bind (_skeletalmesh_2 _relativetransform_2) (`/Game/ChessOfModernUnits/Core/BPFL_CustomUtilits.GetMeshForUnitComponentConfig` (`BlueprintMapLibrary.Map_Find` _socketcomponents _array_element)))
    (bind _returnvalue (`|AddComponentByClass` "/Script/Engine.SkeletalMeshComponent" true _relativetransform_2))
    (`SkeletalMeshComponent.SetSkeletalMeshAsset` _returnvalue _skeletalmesh_2)
    (`SceneComponent.K2_AttachToComponent` _returnvalue (`self.Mesh`) _array_element "KeepRelative" "KeepRelative" "KeepRelative" false)))

(fn `SetCoords`
  (params (NewCoords :type "/Game/ChessOfModernUnits/Placebles/SFieldCellCoords Structure"))
  (bind (_xcoord _ycoord) (break `/Game/ChessOfModernUnits/Placebles/SFieldCellCoords` NewCoords))
  (setmembers `/Game/ChessOfModernUnits/Units/SUnitConfig` :`StructRef` (`self.Config`) :`Coords` NewCoords)
  (`SceneComponent.K2_SetWorldLocation` (`self.DefaultSceneRoot`) (`KismetMathLibrary.MakeVector` (* _xcoord 50) (* _ycoord 50)) false false))

(fn `SetSide`
  (params (Side :type "/Game/ChessOfModernUnits/Core/EPlayerSide Enum" :default "NewEnumerator0"))
  (locals (MIDynamic :type "MaterialInstanceDynamic Object Reference"))
  (setmembers `/Game/ChessOfModernUnits/Units/SUnitConfig` :`StructRef` (`self.Config`) :`Side` Side)
  (for _array_element (`self.GetComponentsByTag` "/Script/Engine.PrimitiveComponent")
    (for _index (range (`PrimitiveComponent.GetNumMaterials` _array_element))
      (bind _returnvalue (`PrimitiveComponent.GetMaterial` _array_element _index))
      (bind _asmaterial_instance_dynamic (cast `MaterialInstanceDynamic` _returnvalue)
        (:`then`
          (bind _output_get (set `local.MIDynamic` _asmaterial_instance_dynamic)))
        (:`CastFailed`
          (bind _returnvalue_2 (`KismetMaterialLibrary.CreateDynamicMaterialInstance` _returnvalue))
          (bind _output_get_2 (set `local.MIDynamic` _returnvalue_2))
          (`PrimitiveComponent.SetMaterial` _array_element _index _output_get_2)))
      (`MaterialInstanceDynamic.SetVectorParameterValue` _output_get "Color" (select `/Game/ChessOfModernUnits/Core/EPlayerSide` (`.Side_4_4F74B15B4D5D30D6A78E1BA957F509DB` (break `/Game/ChessOfModernUnits/Units/SUnitConfig` (`self.Config`))) :`NewEnumerator1` (struct :`R` 1.0 :`G` 1.0 :`B` 1.0 :`A` 1.0) :!type "LinearColor Structure")))))

(fn `UserConstructionScript`)