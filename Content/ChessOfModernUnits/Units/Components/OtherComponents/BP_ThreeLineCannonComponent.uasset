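; Tank cannon unit component for the chess-like tactics game, firing along three lines: the hull direction and two rotations of it.
; Variant sets gun power; shots need a living enemy beyond the blind zone, with one landscape type blocking the line.
; GetPossibleMoves and ComputeMove simulate shots on field data through the target main component's ApplyDamage.
; MakeMove applies damage to the real unit actor; firing zeroes main and cannon move points.
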(event `self.ReceiveBeginPlay`
  (bind _variant (`self.Variant`))
  (`parent.ReceiveBeginPlay`)
  (switch `/Game/ChessOfModernUnits/Units/Components/EUnitComponentVariant` _variant
    (:`NewEnumerator0`
      (`KismetSystemLibrary.PrintString` (`KismetTextLibrary.Conv_TextToString` (`|FormatText` "CRITICAL ERROR IMPOSSIBLE VARIANT ({variant}) FOR {class}" (`|GetEnumeratorNameAsString` _variant) (`KismetSystemLibrary.GetClassDisplayName` (`GameplayStatics.GetObjectClass` self)))) true true (struct :`R` 1.0 :`A` 1.0) :!label _label))
    (:`NewEnumerator1`
      (goto _label))
    (:`NewEnumerator2`
      (goto _label))
    (:`NewEnumerator3`
      (set `self.GunPower` 1))
    (:`NewEnumerator4`
      (set `self.GunPower` 2))
    (:`NewEnumerator5`
      (set `self.GunPower` 3))
    (:`NewEnumerator6`
      (goto _label))))

(fn `ComputeMove`
  (params (Field :type "/Game/ChessOfModernUnits/Placebles/SFieldConfig Structure") (Coords :type "/Game/ChessOfModernUnits/Placebles/SFieldCellCoords Structure") (Move :type "/Game/ChessOfModernUnits/Units/SUnitMove Structure"))
  (returns (Possible :type Boolean) (FieldOutput :type "/Game/ChessOfModernUnits/Placebles/SFieldConfig Structure") (CoordsOutput :type "/Game/ChessOfModernUnits/Placebles/SFieldCellCoords Structure"))
  (locals (Index :type Integer :default 1) (Delta :type "/Game/ChessOfModernUnits/Placebles/SFieldCellCoords Structure"))
  (bind ((`ActiveComponent_20_EA598D07478AB8A33D4C1F99ECAC8CF4` _activecomponent) (`TargetCoords_19_2070F9A84A98EEC52500C0B0A346909D` _targetcoords)) (break `/Game/ChessOfModernUnits/Units/SUnitMove` Move))
  (bind _coords (`local.Coords`))
  (bind ((`Side_4_4F74B15B4D5D30D6A78E1BA957F509DB` _side) (`MainComponent_20_960460F54E1FCEC2EF6C488D79BB28EF` _maincomponent) (`SocketComponents_19_0467C64B42DB044005745F8E30DB9361` _socketcomponents)) (break `/Game/ChessOfModernUnits/Units/SUnitConfig` (`/Game/ChessOfModernUnits/Core/BPFL_CustomUtilits.GetUnitFromField` Field Coords)))
  (bind ((`ActiveComponent_20_EA598D07478AB8A33D4C1F99ECAC8CF4` _activecomponent_2) (`TargetCoords_19_2070F9A84A98EEC52500C0B0A346909D` _targetcoords_2)) (break `/Game/ChessOfModernUnits/Units/SUnitMove` (`local.Move`)))
  (bind (_unit _found) (`/Game/ChessOfModernUnits/Core/BPFL_CustomUtilits.GetUnitFromField` (`local.Field`) _targetcoords))
  (bind _unit_2 (`/Game/ChessOfModernUnits/Core/BPFL_CustomUtilits.GetUnitFromField` (`local.Field`) (`local.Coords`)))
  (bind (_direction _correct) (`/Game/ChessOfModernUnits/Core/BPFL_CustomUtilits.GetDirectionForCoords` Coords _targetcoords))
  (bind (_alive _side_2) (break `/Game/ChessOfModernUnits/Units/SUnitConfig` _unit))
  (bind ((`Direction_8_21FECD5E4D1EA9D2C82B07BD2D049BC7` _direction_2)) (break `/Game/ChessOfModernUnits/Units/Components/SUnitComponentConfig` _maincomponent))
  (bind ((`MainComponent_20_960460F54E1FCEC2EF6C488D79BB28EF` _maincomponent_2) (`SocketComponents_19_0467C64B42DB044005745F8E30DB9361` _socketcomponents_2)) (break `/Game/ChessOfModernUnits/Units/SUnitConfig` _unit_2))
  (bind _coords_2 (`/Game/ChessOfModernUnits/Core/BPFL_CustomUtilits.GetDeltaCoordForDirection` _direction))
  (bind _newcoords (`/Game/ChessOfModernUnits/Core/BPFL_CustomUtilits.AddCoords` (`local.Coords`) (`/Game/ChessOfModernUnits/Core/BPFL_CustomUtilits.ScalarMultiplyCoords` _coords_2 (`local.Index`))))
  (bind (_landscape _cellfound) (`/Game/ChessOfModernUnits/Core/BPFL_CustomUtilits.GetCellFromField` (`local.Field`) _newcoords))
  (if (and _correct (> (`.MovePoints_5_70E1D9294A119D81C594699875F94696` (break `/Game/ChessOfModernUnits/Units/Components/SUnitComponentConfig` (`BlueprintMapLibrary.Map_Find` _socketcomponents _activecomponent))) 0) (`KismetArrayLibrary.Array_Contains` (`|MakeArray` _direction_2 (`/Game/ChessOfModernUnits/Core/BPFL_CustomUtilits.GetDirectionRotated` _direction_2 "NewEnumerator2") (`/Game/ChessOfModernUnits/Core/BPFL_CustomUtilits.GetDirectionRotated` _direction_2 "NewEnumerator3")) _direction))
    (if (and (`|EnumInequality` _side _side_2) _alive (not _found))
      (set `local.Delta` _coords_2)
      (while (not (`/Game/ChessOfModernUnits/Core/BPFL_CustomUtilits.EqualCoords` _newcoords _targetcoords))
        (if (or (`|EnumEquality` _landscape "NewEnumerator1") (not _cellfound))
          (return false)
          (else
            (`/Engine/EditorBlueprintResources/StandardMacros.IncrementInt` (`local.Index`)))))
      (if (> (`local.Index`) (`self.BlindZone`))
        (bind _asbp_base_main_unit_component (cast `/Game/ChessOfModernUnits/Units/Components/BP_BaseMainUnitComponent` (`/Game/ChessOfModernUnits/Core/BP_MoveMakerComponent.GetUnitComponent` (`self.Movemaker`) _unit "Main")))
        (bind _unitafter (`/Game/ChessOfModernUnits/Units/Components/BP_BaseMainUnitComponent.ApplyDamage` _asbp_base_main_unit_component _unit _direction (`self.GunPower`)))
        (if (not (`.Alive_1_4876116A47F2527D46E553BF84858816` (break `/Game/ChessOfModernUnits/Units/SUnitConfig` _unitafter)))
          (setmembers `/Game/ChessOfModernUnits/Units/Components/SUnitComponentConfig` :`StructRef` _maincomponent_2 :`MovePoints` 0)
          (setmembers `/Game/ChessOfModernUnits/Units/Components/SUnitComponentConfig` :`StructRef` (`BlueprintMapLibrary.Map_Find` _socketcomponents_2 _activecomponent_2) :`MovePoints` 0)
          (return true (`/Game/ChessOfModernUnits/Core/BPFL_CustomUtilits.ChangeUnitOnField` (`/Game/ChessOfModernUnits/Core/BPFL_CustomUtilits.ChangeUnitOnField` (`local.Field`) _targetcoords_2 _unitafter) _coords _unit_2) _coords)
          (else
            (return false)))
        (else
          _))))
  (return false))

(fn `GetPossibleMoves`
  (params (Socket :type Name) (Field :type "/Game/ChessOfModernUnits/Placebles/SFieldConfig Structure") (Coords :type "/Game/ChessOfModernUnits/Placebles/SFieldCellCoords Structure"))
  (returns (Moves :type "Map of /Game/ChessOfModernUnits/Units/SUnitMove Structure to /Game/ChessOfModernUnits/Units/Components/SPossibleMoveResult Structure"))
  (locals (FireDirection :type "/Game/ChessOfModernUnits/Units/Components/EDirection Enum") (Delta :type "/Game/ChessOfModernUnits/Placebles/SFieldCellCoords Structure") (Index :type Integer) (OutputMoves :type "Map of /Game/ChessOfModernUnits/Units/SUnitMove Structure to /Game/ChessOfModernUnits/Units/Components/SPossibleMoveResult Structure") (OutputField :type "/Game/ChessOfModernUnits/Placebles/SFieldConfig Structure"))
  (bind _unit (`/Game/ChessOfModernUnits/Core/BPFL_CustomUtilits.GetUnitFromField` Field Coords))
  (bind ((`Side_4_4F74B15B4D5D30D6A78E1BA957F509DB` _side) (`MainComponent_20_960460F54E1FCEC2EF6C488D79BB28EF` _maincomponent) (`SocketComponents_19_0467C64B42DB044005745F8E30DB9361` _socketcomponents)) (break `/Game/ChessOfModernUnits/Units/SUnitConfig` _unit))
  (bind ((`Direction_8_21FECD5E4D1EA9D2C82B07BD2D049BC7` _direction)) (break `/Game/ChessOfModernUnits/Units/Components/SUnitComponentConfig` _maincomponent))
  (bind _value (`BlueprintMapLibrary.Map_Find` _socketcomponents Socket))
  (bind _newcoords (`/Game/ChessOfModernUnits/Core/BPFL_CustomUtilits.AddCoords` (`local.Coords`) (`/Game/ChessOfModernUnits/Core/BPFL_CustomUtilits.ScalarMultiplyCoords` (`local.Delta`) (`local.Index`))))
  (bind (_landscape _cellfound _unit_2 _unitfound) (`/Game/ChessOfModernUnits/Core/BPFL_CustomUtilits.GetCellFromField` (`local.Field`) (`/Game/ChessOfModernUnits/Core/BPFL_CustomUtilits.AddCoords` (`local.Coords`) (`/Game/ChessOfModernUnits/Core/BPFL_CustomUtilits.ScalarMultiplyCoords` (`local.Delta`) (`local.Index`)))))
  (bind (_alive _side_2) (break `/Game/ChessOfModernUnits/Units/SUnitConfig` _unit_2))
  (if (> (`.MovePoints_5_70E1D9294A119D81C594699875F94696` (break `/Game/ChessOfModernUnits/Units/Components/SUnitComponentConfig` _value)) 0)
    (setmembers `/Game/ChessOfModernUnits/Units/Components/SUnitComponentConfig` :`StructRef` _maincomponent :`MovePoints` 0)
    (setmembers `/Game/ChessOfModernUnits/Units/Components/SUnitComponentConfig` :`StructRef` _value :`MovePoints` 0)
    (set `local.OutputField` (`/Game/ChessOfModernUnits/Core/BPFL_CustomUtilits.ChangeUnitOnField` Field Coords _unit))
    (`|ExecutionSequence`
      (:`then_0`
        (bind _output_get (set `local.FireDirection` _direction)))
      (:`then_1`
        (set `local.FireDirection` (`/Game/ChessOfModernUnits/Core/BPFL_CustomUtilits.GetDirectionRotated` _direction "NewEnumerator2")))
      (:`then_2`
        (set `local.FireDirection` (`/Game/ChessOfModernUnits/Core/BPFL_CustomUtilits.GetDirectionRotated` _direction "NewEnumerator3")))
      (:`then_3`
        (return (`local.OutputMoves`))))
    (set `local.Delta` (`/Game/ChessOfModernUnits/Core/BPFL_CustomUtilits.GetDeltaCoordForDirection` _output_get))
    (set `local.Index` 1)
    (while (and (`|EnumInequality` _landscape "NewEnumerator1") _cellfound)
      (if (and _unitfound _alive (`|EnumInequality` _side_2 _side) (> (`local.Index`) (`self.BlindZone`)))
        (bind _asbp_base_main_unit_component (cast `/Game/ChessOfModernUnits/Units/Components/BP_BaseMainUnitComponent` (`/Game/ChessOfModernUnits/Core/BP_MoveMakerComponent.GetUnitComponent` (`self.Movemaker`) _unit_2 "Main")))
        (bind (_unitafter _valid) (`/Game/ChessOfModernUnits/Units/Components/BP_BaseMainUnitComponent.ApplyDamage` _asbp_base_main_unit_component _unit_2 (`local.FireDirection`) (`self.GunPower`)))
        (if _valid
          (`BlueprintMapLibrary.Map_Add` (`local.OutputMoves`) (make `/Game/ChessOfModernUnits/Units/SUnitMove` (`local.Socket`) _newcoords true) (make `/Game/ChessOfModernUnits/Units/Components/SPossibleMoveResult` (`/Game/ChessOfModernUnits/Core/BPFL_CustomUtilits.ChangeUnitOnField` (`local.OutputField`) _newcoords _unitafter) (`local.Coords`)))
          (`/Engine/EditorBlueprintResources/StandardMacros.IncrementInt` (`local.Index`))
          (else
            (`/Engine/EditorBlueprintResources/StandardMacros.IncrementInt` (`local.Index`))))
        (else
          (`/Engine/EditorBlueprintResources/StandardMacros.IncrementInt` (`local.Index`)))))))

(fn `MakeMove`
  (params (Unit :type "/Game/ChessOfModernUnits/Units/BP_Unit Object Reference") (NowMove :type "/Game/ChessOfModernUnits/Units/SUnitMove Structure") (NextMove :type "/Game/ChessOfModernUnits/Units/SUnitMove Structure") (NextMoveValid :type Boolean))
  (bind ((`ActiveComponent_20_EA598D07478AB8A33D4C1F99ECAC8CF4` _activecomponent) (`TargetCoords_19_2070F9A84A98EEC52500C0B0A346909D` _targetcoords)) (break `/Game/ChessOfModernUnits/Units/SUnitMove` NowMove))
  (bind ((`MainComponent_20_960460F54E1FCEC2EF6C488D79BB28EF` _maincomponent) (`SocketComponents_19_0467C64B42DB044005745F8E30DB9361` _socketcomponents)) (break `/Game/ChessOfModernUnits/Units/SUnitConfig` (`/Game/ChessOfModernUnits/Units/BP_Unit.Config` Unit)))
  (setmembers `/Game/ChessOfModernUnits/Units/Components/SUnitComponentConfig` :`StructRef` _maincomponent :`MovePoints` 0)
  (setmembers `/Game/ChessOfModernUnits/Units/Components/SUnitComponentConfig` :`StructRef` (`BlueprintMapLibrary.Map_Find` _socketcomponents _activecomponent) :`MovePoints` 0)
  (bind _outactors (`GameplayStatics.GetAllActorsOfClass` "/Game/ChessOfModernUnits/Units/BP_Unit.BP_Unit_C"))
  (for _array_element _outactors
    (cast `/Game/ChessOfModernUnits/Units/BP_UnitHologram` _array_element
      (:`CastFailed`
        (bind _config (`/Game/ChessOfModernUnits/Units/BP_Unit.Config` _array_element))
        (bind ((`Coords_7_9C7BED8F4B2205EF8B5C87A1962D4680` _coords)) (break `/Game/ChessOfModernUnits/Units/SUnitConfig` _config))
        (if (`/Game/ChessOfModernUnits/Core/BPFL_CustomUtilits.EqualCoords` _targetcoords _coords)
          (bind _asbp_base_main_unit_component (cast `/Game/ChessOfModernUnits/Units/Components/BP_BaseMainUnitComponent` (`/Game/ChessOfModernUnits/Core/BP_MoveMakerComponent.GetUnitComponent` (`self.Movemaker`) _config "Main")))
          (bind (_unitafter _valid) (`/Game/ChessOfModernUnits/Units/Components/BP_BaseMainUnitComponent.ApplyDamage` _asbp_base_main_unit_component _config (`/Game/ChessOfModernUnits/Core/BPFL_CustomUtilits.GetDirectionForCoords` (`.Coords_7_9C7BED8F4B2205EF8B5C87A1962D4680` (break `/Game/ChessOfModernUnits/Units/SUnitConfig` (`/Game/ChessOfModernUnits/Units/BP_Unit.Config` (`local.Unit`)))) _coords) (`self.GunPower`)))
          (if _valid
            (`/Game/ChessOfModernUnits/Units/BP_Unit.SetAlive` _array_element (`.Alive_1_4876116A47F2527D46E553BF84858816` (break `/Game/ChessOfModernUnits/Units/SUnitConfig` _unitafter)))
            (break)
            (else
              (break))))))))