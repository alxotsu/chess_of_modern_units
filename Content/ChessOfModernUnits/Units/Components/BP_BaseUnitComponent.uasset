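; BP_BaseUnitComponent is the base component for units in Chess of Modern Units, defining a common interface for move logic.
; On BeginPlay it caches the owner's BP_MoveMakerComponent.
; GetPossibleMoves, ComputeMove and MakeMove are stubs, apparently for child components to override, with ComputeMove reporting moves as impossible by default.
; ReloadComponent resets the move points in a unit component config to the starting value.
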(event `self.ReceiveBeginPlay`
  (set `self.Movemaker` (`Actor.GetComponentByClass` (`self.GetOwner`) "/Game/ChessOfModernUnits/Core/BP_MoveMakerComponent.BP_MoveMakerComponent_C")))

(fn `ComputeMove`
  (params (Field :type "/Game/ChessOfModernUnits/Placebles/SFieldConfig Structure") (Coords :type "/Game/ChessOfModernUnits/Placebles/SFieldCellCoords Structure") (Move :type "/Game/ChessOfModernUnits/Units/SUnitMove Structure"))
  (returns (Possible :type Boolean) (FieldOutput :type "/Game/ChessOfModernUnits/Placebles/SFieldConfig Structure") (CoordsOutput :type "/Game/ChessOfModernUnits/Placebles/SFieldCellCoords Structure"))
  (return false))

(fn `GetPossibleMoves`
  (params (Socket :type Name) (Field :type "/Game/ChessOfModernUnits/Placebles/SFieldConfig Structure") (Coords :type "/Game/ChessOfModernUnits/Placebles/SFieldCellCoords Structure"))
  (returns (Moves :type "Map of /Game/ChessOfModernUnits/Units/SUnitMove Structure to /Game/ChessOfModernUnits/Units/Components/SPossibleMoveResult Structure"))
  (return))

(fn `MakeMove`
  (params (Unit :type "/Game/ChessOfModernUnits/Units/BP_Unit Object Reference") (NowMove :type "/Game/ChessOfModernUnits/Units/SUnitMove Structure") (NextMove :type "/Game/ChessOfModernUnits/Units/SUnitMove Structure") (NextMoveValid :type Boolean)))

(fn `ReloadComponent`
  (params (Component :type "/Game/ChessOfModernUnits/Units/Components/SUnitComponentConfig Structure"))
  (returns (ComponentOut :type "/Game/ChessOfModernUnits/Units/Components/SUnitComponentConfig Structure (by ref)"))
  (bind _structout (setmembers `/Game/ChessOfModernUnits/Units/Components/SUnitComponentConfig` :`StructRef` Component :`MovePoints` (`self.StartMovePoints`)))
  (return _structout))