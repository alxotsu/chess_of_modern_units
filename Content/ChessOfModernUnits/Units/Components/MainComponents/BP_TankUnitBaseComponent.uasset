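; Base hull component for tanks in a turn-based grid tactics game, setting move points and per-direction armor for light, medium and heavy variants.
; ApplyDamage kills the unit when attack power beats the armor facing it.
; GetPossibleMoves simulates each step or turn through ComputeMove on field data, gating one terrain type by commander antenna and side.
; MakeMove applies moves to the actor; reversing spends all remaining points.
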(event `self.ReceiveBeginPlay`
  (bind _map (`|MakeMap` "NewEnumerator0" 3 "NewEnumerator1" 1 "NewEnumerator2" 2 "NewEnumerator3" 2 "NewEnumerator4" 2 "NewEnumerator5" 2 "NewEnumerator6" 2 "NewEnumerator7" 2 :!type "/Game/ChessOfModernUnits/Units/Components/EDirection Enum"))
  (bind _variant (`self.Variant`))
  (bind _armor (`self.Armor`))
  (bind _armor_2 (`self.Armor`))
  (`parent.ReceiveBeginPlay`)
  (switch `/Game/ChessOfModernUnits/Units/Components/EUnitComponentVariant` _variant
    (:`NewEnumerator0`
      (set `self.StartMovePoints` 5)
      (set `self.Armor` _map)
      (bind _enumvalue (foreach `/Game/ChessOfModernUnits/Units/Components/EDirection` false)
        (:`LoopBody`
          (`BlueprintMapLibrary.Map_Add` _armor _enumvalue (`KismetMathLibrary.Max` (- (`BlueprintMapLibrary.Map_Find` _armor _enumvalue) 2))))))
    (:`NewEnumerator1`
      (set `self.StartMovePoints` 4)
      (set `self.Armor` _map)
      (bind _enumvalue_2 (foreach `/Game/ChessOfModernUnits/Units/Components/EDirection` false)
        (:`LoopBody`
          (`BlueprintMapLibrary.Map_Add` _armor_2 _enumvalue_2 (- (`BlueprintMapLibrary.Map_Find` _armor_2 _enumvalue_2) 1)))))
    (:`NewEnumerator2`
      (set `self.StartMovePoints` 3)
      (set `self.Armor` _map))
    (:`NewEnumerator3`
      (`KismetSystemLibrary.PrintString` (`KismetTextLibrary.Conv_TextToString` (`|FormatText` "CRITICAL ERROR IMPOSSIBLE VARIANT ({variant}) FOR {class}" (`|GetEnumeratorNameAsString` _variant) (`KismetSystemLibrary.GetClassDisplayName` (`GameplayStatics.GetObjectClass` self)))) true true (struct :`R` 1.0 :`A` 1.0) :!label _label))
    (:`NewEnumerator4`
      (goto _label))
    (:`NewEnumerator5`
      (goto _label))
    (:`NewEnumerator6`
      (goto _label))))

(fn `ApplyDamage`
  (params (Unit :type "/Game/ChessOfModernUnits/Units/SUnitConfig Structure") (Direction :type "/Game/ChessOfModernUnits/Units/Components/EDirection Enum" :default "NewEnumerator0") (Power :type Integer))
  (returns (UnitAfter :type "/Game/ChessOfModernUnits/Units/SUnitConfig Structure") (Valid :type Boolean))
  (if (< (`BlueprintMapLibrary.Map_Find` (`self.Armor`) (`/Game/ChessOfModernUnits/Core/BPFL_CustomUtilits.GetDiametralDirection` (`/Game/ChessOfModernUnits/Core/BPFL_CustomUtilits.GetRelativeDirection` Direction (`.Direction_8_21FECD5E4D1EA9D2C82B07BD2D049BC7` (break `/Game/ChessOfModernUnits/Units/Components/SUnitComponentConfig` (`.MainComponent_20_960460F54E1FCEC2EF6C488D79BB28EF` (break `/Game/ChessOfModernUnits/Units/SUnitConfig` Unit))))))) Power)
    (bind _structout (setmembers `/Game/ChessOfModernUnits/Units/SUnitConfig` :`StructRef` Unit :`Alive` false))
    (return _structout true)
    (else
      (return Unit false))))

(fn `ComputeMove`
  (params (Field :type "/Game/ChessOfModernUnits/Placebles/SFieldConfig Structure") (Coords :type "/Game/ChessOfModernUnits/Placebles/SFieldCellCoords Structure") (Move :type "/Game/ChessOfModernUnits/Units/SUnitMove Structure"))
  (returns (Possible :type Boolean) (FieldOutput :type "/Game/ChessOfModernUnits/Placebles/SFieldConfig Structure") (CoordsOutput :type "/Game/ChessOfModernUnits/Placebles/SFieldCellCoords Structure"))
  (locals (NewCoords :type "/Game/ChessOfModernUnits/Placebles/SFieldCellCoords Structure"))
  (bind _unit (`/Game/ChessOfModernUnits/Core/BPFL_CustomUtilits.GetUnitFromField` Field Coords))
  (bind _coords (`local.Coords`))
  (bind ((`Movement_23_9D0598D440526568FDBB37AF3C3EF979` _movement)) (break `/Game/ChessOfModernUnits/Units/SUnitMove` (`local.Move`)))
  (bind ((`Coords_7_9C7BED8F4B2205EF8B5C87A1962D4680` _coords_2)) (break `/Game/ChessOfModernUnits/Units/SUnitConfig` _unit))
  (bind (_landscape _cellfound _unit_2 _unitfound) (`/Game/ChessOfModernUnits/Core/BPFL_CustomUtilits.GetCellFromField` (`local.Field`) (`local.NewCoords`)))
  (bind _unit_3 (`/Game/ChessOfModernUnits/Core/BPFL_CustomUtilits.GetUnitFromField` (`local.Field`) (`local.Coords`)))
  (bind _unit_4 (`/Game/ChessOfModernUnits/Core/BPFL_CustomUtilits.GetUnitFromField` (`local.Field`) (`local.Coords`)))
  (bind ((`Side_4_4F74B15B4D5D30D6A78E1BA957F509DB` _side) (`SocketComponents_19_0467C64B42DB044005745F8E30DB9361` _socketcomponents)) (break `/Game/ChessOfModernUnits/Units/SUnitConfig` _unit_4))
  (bind (_variantname _movepoints _direction) (break `/Game/ChessOfModernUnits/Units/Components/SUnitComponentConfig` (`.MainComponent_20_960460F54E1FCEC2EF6C488D79BB28EF` (break `/Game/ChessOfModernUnits/Units/SUnitConfig` _unit))))
  (bind (_variantname_2 _movepoints_2 _direction_2) (break `/Game/ChessOfModernUnits/Units/Components/SUnitComponentConfig` (`.MainComponent_20_960460F54E1FCEC2EF6C488D79BB28EF` (break `/Game/ChessOfModernUnits/Units/SUnitConfig` _unit_3))))
  (if (> (`.MovePoints_5_70E1D9294A119D81C594699875F94696` (break `/Game/ChessOfModernUnits/Units/Components/SUnitComponentConfig` (`.MainComponent_20_960460F54E1FCEC2EF6C488D79BB28EF` (break `/Game/ChessOfModernUnits/Units/SUnitConfig` _unit)))) 0)
    (switch `/Game/ChessOfModernUnits/Units/Components/EMovement` _movement
      (:`NewEnumerator0`
        (set `local.NewCoords` (`/Game/ChessOfModernUnits/Core/BPFL_CustomUtilits.AddCoords` _coords_2 (`/Game/ChessOfModernUnits/Core/BPFL_CustomUtilits.GetDeltaCoordForDirection` _direction))))
      (:`NewEnumerator1`
        (set `local.NewCoords` (`/Game/ChessOfModernUnits/Core/BPFL_CustomUtilits.AddCoords` _coords_2 (`/Game/ChessOfModernUnits/Core/BPFL_CustomUtilits.GetDeltaCoordForDirection` (`/Game/ChessOfModernUnits/Core/BPFL_CustomUtilits.GetDiametralDirection` _direction)))))
      (:`NewEnumerator2`
        (bind _structout (setmembers `/Game/ChessOfModernUnits/Units/SUnitConfig` :`StructRef` _unit :`MainComponent` (make `/Game/ChessOfModernUnits/Units/Components/SUnitComponentConfig` _variantname (- _movepoints 1) (`/Game/ChessOfModernUnits/Core/BPFL_CustomUtilits.GetDirectionRotated` _direction _movement)) :!label _label))
        (return true (`/Game/ChessOfModernUnits/Core/BPFL_CustomUtilits.ChangeUnitOnField` (`local.Field`) _coords _structout) _coords))
      (:`NewEnumerator3`
        (goto _label)))
    (if (and _cellfound (`KismetArrayLibrary.Array_Contains` (`|MakeArray` "NewEnumerator0" "NewEnumerator3" :!type "/Game/ChessOfModernUnits/Placebles/ELandscapeType Enum") _landscape) (not _unitfound))
      (if (`|EnumEquality` _landscape "NewEnumerator3")
        (bind _keys (`BlueprintMapLibrary.Map_Keys` _socketcomponents))
        (for _array_element _keys
          (cast `/Game/ChessOfModernUnits/Units/Components/OtherComponents/BP_ComanderTankAntenneComponent` (`/Game/ChessOfModernUnits/Core/BP_MoveMakerComponent.GetUnitComponent` (`self.Movemaker`) _unit_4 _array_element))
          (if (not (xor (< (`.YCoord_12_230624BA45D1462C62A7DA860B56371E` (break `/Game/ChessOfModernUnits/Placebles/SFieldCellCoords` (`local.NewCoords`))) 0) (`|EnumEquality` _side "NewEnumerator0")))
            (bind _structout_2 (setmembers `/Game/ChessOfModernUnits/Units/SUnitConfig` :`StructRef` _unit_3 :`Coords` (`local.NewCoords`) :`MainComponent` (make `/Game/ChessOfModernUnits/Units/Components/SUnitComponentConfig` _variantname_2 (select `bool` (`|EnumEquality` (`.Movement_23_9D0598D440526568FDBB37AF3C3EF979` (break `/Game/ChessOfModernUnits/Units/SUnitMove` (`local.Move`))) "NewEnumerator1") :`false` (- _movepoints_2 1)) _direction_2) :!label _label_2))
            (return true (`/Game/ChessOfModernUnits/Core/BPFL_CustomUtilits.ChangeUnitOnField` (`local.Field`) (`local.Coords`) _structout_2) (`local.NewCoords`))
            (else
              (return false))))
        (else
          (goto _label_2))))
    (return false)
    (else
      (return false))))

(fn `GetPossibleMoves`
  (params (Socket :type Name) (Field :type "/Game/ChessOfModernUnits/Placebles/SFieldConfig Structure") (Coords :type "/Game/ChessOfModernUnits/Placebles/SFieldCellCoords Structure"))
  (returns (Moves :type "Map of /Game/ChessOfModernUnits/Units/SUnitMove Structure to /Game/ChessOfModernUnits/Units/Components/SPossibleMoveResult Structure"))
  (locals (Output :type "Map of /Game/ChessOfModernUnits/Units/SUnitMove Structure to /Game/ChessOfModernUnits/Units/Components/SPossibleMoveResult Structure"))
  (bind _enumvalue (foreach `/Game/ChessOfModernUnits/Units/Components/EMovement` false)
    (:`LoopBody`
      (bind ((`SUnitMove` _sunitmove)) (make `/Game/ChessOfModernUnits/Units/SUnitMove` :`Movement` _enumvalue))
      (bind (_possible _fieldoutput _coordsoutput) (`self.ComputeMove` Field Coords _sunitmove))
      (if _possible
        (`BlueprintMapLibrary.Map_Add` (`local.Output`) _sunitmove (make `/Game/ChessOfModernUnits/Units/Components/SPossibleMoveResult` _fieldoutput _coordsoutput))))
    (:`then`
      (return (`local.Output`)))))

(fn `MakeMove`
  (params (Unit :type "/Game/ChessOfModernUnits/Units/BP_Unit Object Reference") (NowMove :type "/Game/ChessOfModernUnits/Units/SUnitMove Structure") (NextMove :type "/Game/ChessOfModernUnits/Units/SUnitMove Structure") (NextMoveValid :type Boolean))
  (bind ((`Movement_23_9D0598D440526568FDBB37AF3C3EF979` _movement)) (break `/Game/ChessOfModernUnits/Units/SUnitMove` NowMove))
  (bind _unit (`local.Unit`))
  (bind ((`Coords_7_9C7BED8F4B2205EF8B5C87A1962D4680` _coords) (`MainComponent_20_960460F54E1FCEC2EF6C488D79BB28EF` _maincomponent)) (break `/Game/ChessOfModernUnits/Units/SUnitConfig` (`/Game/ChessOfModernUnits/Units/BP_Unit.Config` Unit)))
  (bind ((`Movement_23_9D0598D440526568FDBB37AF3C3EF979` _movement_2)) (break `/Game/ChessOfModernUnits/Units/SUnitMove` (`local.NowMove`)))
  (bind _defaultsceneroot (`/Game/ChessOfModernUnits/Units/BP_Unit.DefaultSceneRoot` _unit))
  (bind ((`Direction_8_21FECD5E4D1EA9D2C82B07BD2D049BC7` _direction)) (break `/Game/ChessOfModernUnits/Units/Components/SUnitComponentConfig` _maincomponent))
  (bind ((`MainComponent_20_960460F54E1FCEC2EF6C488D79BB28EF` _maincomponent_2)) (break `/Game/ChessOfModernUnits/Units/SUnitConfig` (`/Game/ChessOfModernUnits/Units/BP_Unit.Config` (`local.Unit`))))
  (bind (_returnvalue_roll _returnvalue_pitch) (`KismetMathLibrary.BreakRotator` (`SceneComponent.K2_GetComponentRotation` _defaultsceneroot)))
  (bind ((`MovePoints_5_70E1D9294A119D81C594699875F94696` _movepoints) (`Direction_8_21FECD5E4D1EA9D2C82B07BD2D049BC7` _direction_2)) (break `/Game/ChessOfModernUnits/Units/Components/SUnitComponentConfig` _maincomponent_2))
  (switch `/Game/ChessOfModernUnits/Units/Components/EMovement` _movement
    (:`NewEnumerator0`
      (`/Game/ChessOfModernUnits/Units/BP_Unit.SetCoords` (`local.Unit`) (`/Game/ChessOfModernUnits/Core/BPFL_CustomUtilits.AddCoords` _coords (`/Game/ChessOfModernUnits/Core/BPFL_CustomUtilits.GetDeltaCoordForDirection` _direction))))
    (:`NewEnumerator1`
      (`/Game/ChessOfModernUnits/Units/BP_Unit.SetCoords` _unit (`/Game/ChessOfModernUnits/Core/BPFL_CustomUtilits.AddCoords` _coords (`/Game/ChessOfModernUnits/Core/BPFL_CustomUtilits.GetDeltaCoordForDirection` (`/Game/ChessOfModernUnits/Core/BPFL_CustomUtilits.GetDiametralDirection` _direction)))))
    (:`NewEnumerator2`
      (`SceneComponent.K2_SetWorldRotation` _defaultsceneroot (`KismetMathLibrary.MakeRotator` _returnvalue_roll _returnvalue_pitch (`/Game/ChessOfModernUnits/Core/BPFL_CustomUtilits.GetRotationForDirection` (`/Game/ChessOfModernUnits/Core/BPFL_CustomUtilits.GetDirectionRotated` _direction _movement) true)) false false :!label _label))
    (:`NewEnumerator3`
      (goto _label)))
  (setmembers `/Game/ChessOfModernUnits/Units/Components/SUnitComponentConfig` :`StructRef` _maincomponent_2 :`MovePoints` (select `bool` (`|EnumEquality` _movement_2 "NewEnumerator1") :`false` (- _movepoints 1)) :`Direction` (`/Game/ChessOfModernUnits/Core/BPFL_CustomUtilits.GetDirectionRotated` _direction_2 _movement_2)))