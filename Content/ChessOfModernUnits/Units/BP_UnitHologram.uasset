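; BP_UnitHologram is a hologram version of a unit in Chess of Modern Units, tinted by a color and light value.
; On BeginPlay it applies coordinates and main and socket components from its Config, then calls SetColor.
; SetColor creates one dynamic instance of M_TankHologram, sets its Color and Light parameters, and assigns it to every material slot on all skeletal mesh components.
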(event `self.ReceiveBeginPlay`
  (bind ((`Coords_7_9C7BED8F4B2205EF8B5C87A1962D4680` _coords) (`MainComponent_20_960460F54E1FCEC2EF6C488D79BB28EF` _maincomponent) (`SocketComponents_19_0467C64B42DB044005745F8E30DB9361` _socketcomponents)) (break `/Game/ChessOfModernUnits/Units/SUnitConfig` (`self.Config`)))
  (`self.SetCoords` _coords)
  (`self.SetComponents` _maincomponent _socketcomponents)
  (`self.Set Color` (`self.HologramColor`) (`self.Light`)))

(fn `Set Color`
  (params (Color :type "LinearColor Structure") (Light :type Boolean))
  (locals (HologramMaterial :type "MaterialInstanceDynamic Object Reference"))
  (set `self.HologramColor` Color)
  (set `self.Light` Light)
  (bind _returnvalue (`KismetMaterialLibrary.CreateDynamicMaterialInstance` "/Game/ChessOfModernUnits/Units/Materials/M_TankHologram.M_TankHologram"))
  (bind _output_get (set `local.HologramMaterial` _returnvalue))
  (`MaterialInstanceDynamic.SetVectorParameterValue` _output_get "Color" (`self.HologramColor`))
  (`MaterialInstanceDynamic.SetScalarParameterValue` _output_get "Light" (`KismetMathLibrary.Conv_BoolToDouble` (`self.Light`)))
  (for _array_element (`self.K2_GetComponentsByClass` "/Script/Engine.SkeletalMeshComponent")
    (for _index (range (`PrimitiveComponent.GetNumMaterials` _array_element))
      (`PrimitiveComponent.SetMaterial` _array_element _index (`local.HologramMaterial`)))))

(fn `UserConstructionScript`)