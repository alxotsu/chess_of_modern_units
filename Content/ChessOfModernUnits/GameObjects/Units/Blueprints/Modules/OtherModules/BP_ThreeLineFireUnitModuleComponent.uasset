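; Unit weapon module for the grid tactics game that fires at one chosen enemy along three lines: the unit's facing and two rotations of it.
; GetTargets scans each line within range, blind zone and allowed landscape, past intervening units, simulating damage through each unit's temporary Main movement module.
; That target map feeds GetPossibleMoves and ComputeMove, which spends the shooter's move on field state.
; VisualizeMove recomputes damage on live unit actors.
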(fn `ComputeMove`
  (params (FieldState :type "/Game/ChessOfModernUnits/GameObjects/Field/Blueprints/SFieldState Structure") (UnitConfig :type "/Game/ChessOfModernUnits/GameObjects/Units/Blueprints/SUnitConfig Structure") (Move :type "/Game/ChessOfModernUnits/GameObjects/Units/Blueprints/SUnitMove Structure"))
  (returns (NewFieldState :type "/Game/ChessOfModernUnits/GameObjects/Field/Blueprints/SFieldState Structure") (NewUnitConfig :type "/Game/ChessOfModernUnits/GameObjects/Units/Blueprints/SUnitConfig Structure") (Possible :type Boolean))
  (locals (newCanUse :type "Map of Name to Boolean"))
  (bind ((`Coords_47_E98C47904C4A4C6B43CCA291531B50D8` _coords) (`TempState_62_5ABFF3A34B4DD39392594A92040E2E81` _tempstate)) (break `/Game/ChessOfModernUnits/GameObjects/Units/Blueprints/SUnitConfig` UnitConfig))
  (bind (_activecomponent _targetcoords) (break `/Game/ChessOfModernUnits/GameObjects/Units/Blueprints/SUnitMove` Move))
  (bind _targets (`self.GetTargets` FieldState UnitConfig))
  (bind (_value _returnvalue) (`BlueprintMapLibrary.Map_Find` _targets _targetcoords))
  (if _returnvalue
    (`BlueprintMapLibrary.Map_Add` (`.CanUse_23_BE99ED37467B2319636ED0A69AB3D10F` (break `/Game/ChessOfModernUnits/GameObjects/Units/Blueprints/SUnitTempState` _tempstate)) _activecomponent)
    (bind _structout (setmembers `/Game/ChessOfModernUnits/GameObjects/Units/Blueprints/SUnitConfig` :`StructRef` (`|Copy` UnitConfig) :`TempState` (make `/Game/ChessOfModernUnits/GameObjects/Units/Blueprints/SUnitTempState` 0 (`.CanUse_23_BE99ED37467B2319636ED0A69AB3D10F` (break `/Game/ChessOfModernUnits/GameObjects/Units/Blueprints/SUnitTempState` _tempstate)))))
    (bind _newfieldstate (`/Game/ChessOfModernUnits/GameFramework/Player/BPFL_CellsAndUnits.ChangeUnit` FieldState _coords _structout))
    (bind _newfieldstate_2 (`/Game/ChessOfModernUnits/GameFramework/Player/BPFL_CellsAndUnits.ChangeUnit` _newfieldstate _targetcoords _value))
    (return _newfieldstate_2 _structout true)
    (else
      (return (struct) (struct) false))))

(fn `GetPossibleMoves`
  (params (FieldState :type "/Game/ChessOfModernUnits/GameObjects/Field/Blueprints/SFieldState Structure") (UnitConfig :type "/Game/ChessOfModernUnits/GameObjects/Units/Blueprints/SUnitConfig Structure"))
  (returns (PossibleMoves :type "Map of /Game/ChessOfModernUnits/GameObjects/Units/Blueprints/SUnitMove Structure to /Game/ChessOfModernUnits/GameObjects/Units/Blueprints/SUnitConfig Structure"))
  (locals (Moves :type "Map of /Game/ChessOfModernUnits/GameObjects/Units/Blueprints/SUnitMove Structure to /Game/ChessOfModernUnits/GameObjects/Units/Blueprints/SUnitConfig Structure"))
  (bind _returnvalue (`|Copy` UnitConfig))
  (bind ((`Coords_47_E98C47904C4A4C6B43CCA291531B50D8` _coords) (`TempState_62_5ABFF3A34B4DD39392594A92040E2E81` _tempstate)) (break `/Game/ChessOfModernUnits/GameObjects/Units/Blueprints/SUnitConfig` _returnvalue))
  (`BlueprintMapLibrary.Map_Add` (`.CanUse_23_BE99ED37467B2319636ED0A69AB3D10F` (break `/Game/ChessOfModernUnits/GameObjects/Units/Blueprints/SUnitTempState` _tempstate)) (`self.Socket`))
  (setmembers `/Game/ChessOfModernUnits/GameObjects/Units/Blueprints/SUnitConfig` :`StructRef` _returnvalue :`TempState` (make `/Game/ChessOfModernUnits/GameObjects/Units/Blueprints/SUnitTempState` 0 (`.CanUse_23_BE99ED37467B2319636ED0A69AB3D10F` (break `/Game/ChessOfModernUnits/GameObjects/Units/Blueprints/SUnitTempState` _tempstate))))
  (bind _targets (`self.GetTargets` FieldState UnitConfig))
  (bind _keys (`BlueprintMapLibrary.Map_Keys` _targets))
  (for _array_element _keys
    (`BlueprintMapLibrary.Map_Add` (`local.Moves`) (make `/Game/ChessOfModernUnits/GameObjects/Units/Blueprints/SUnitMove` (`self.Socket`) _array_element) _returnvalue))
  (return (`local.Moves`)))

(fn `GetTargets`
  (params (FieldState :type "/Game/ChessOfModernUnits/GameObjects/Field/Blueprints/SFieldState Structure") (UnitConfig :type "/Game/ChessOfModernUnits/GameObjects/Units/Blueprints/SUnitConfig Structure"))
  (returns (Targets :type "Map of /Game/ChessOfModernUnits/GameObjects/Field/Blueprints/SFieldCellCoords Structure to /Game/ChessOfModernUnits/GameObjects/Units/Blueprints/SUnitConfig Structure"))
  (locals (FireDirection :type "/Game/ChessOfModernUnits/GameObjects/Units/Blueprints/EDirection Enum") (Delta :type "/Game/ChessOfModernUnits/GameObjects/Field/Blueprints/SFieldCellCoords Structure") (index :type Integer) (TargetMap :type "Map of /Game/ChessOfModernUnits/GameObjects/Field/Blueprints/SFieldCellCoords Structure to /Game/ChessOfModernUnits/GameObjects/Units/Blueprints/SUnitConfig Structure"))
  (bind ((`Direction_56_4F2B10F847F49B1199F4DC823B142897` _direction) (`TempState_62_5ABFF3A34B4DD39392594A92040E2E81` _tempstate)) (break `/Game/ChessOfModernUnits/GameObjects/Units/Blueprints/SUnitConfig` UnitConfig))
  (bind (_unitconfig_mainmodule _unitconfig_moduleonsockets _unitconfig_coords) (break `/Game/ChessOfModernUnits/GameObjects/Units/Blueprints/SUnitConfig` (`local.UnitConfig`)))
  (bind (_unitconfig_mainmodule_2 _unitconfig_moduleonsockets_2 _unitconfig_coords_2 _unitconfig_direction _unitconfig_alive _unitconfig_side) (break `/Game/ChessOfModernUnits/GameObjects/Units/Blueprints/SUnitConfig` (`local.UnitConfig`)))
  (bind (_unitconfig_mainmodule_3 _unitconfig_moduleonsockets_3 _unitconfig_coords_3) (break `/Game/ChessOfModernUnits/GameObjects/Units/Blueprints/SUnitConfig` (`local.UnitConfig`)))
  (bind (_cellfound _unitfound _landscapetype _unitconfig) (`/Game/ChessOfModernUnits/GameFramework/Player/BPFL_CellsAndUnits.GetCell` (`local.FieldState`) (`/Game/ChessOfModernUnits/GameObjects/Units/Blueprints/BPFL_CoordsAndDirectionTransforms.AddCoords` _unitconfig_coords (`/Game/ChessOfModernUnits/GameObjects/Units/Blueprints/BPFL_CoordsAndDirectionTransforms.MultiplyCoords` (`local.Delta`) (`local.index`)))))
  (if (`BlueprintMapLibrary.Map_Find` (`.CanUse_23_BE99ED37467B2319636ED0A69AB3D10F` (break `/Game/ChessOfModernUnits/GameObjects/Units/Blueprints/SUnitTempState` _tempstate)) (`self.Socket`))
    (`|ExecutionSequence`
      (:`then_0`
        (bind _output_get (set `local.FireDirection` _direction))
        (bind _delta (`/Game/ChessOfModernUnits/GameObjects/Units/Blueprints/BPFL_CoordsAndDirectionTransforms.GetDeltaCoordsByDirection` _output_get))
        (set `local.Delta` _delta)
        (bind _moduledescription (`/Game/ChessOfModernUnits/GameFramework/Player/BPFL_CellsAndUnits.GetModuleDescription` (`local.UnitConfig`) (`self.Socket`))))
      (:`then_1`
        (bind _newdirection (`/Game/ChessOfModernUnits/GameObjects/Units/Blueprints/BPFL_CoordsAndDirectionTransforms.GetDirectionAfterRotate` "NewEnumerator2" _direction))
        (bind _output_get_2 (set `local.FireDirection` _newdirection))
        (bind _delta_2 (`/Game/ChessOfModernUnits/GameObjects/Units/Blueprints/BPFL_CoordsAndDirectionTransforms.GetDeltaCoordsByDirection` _output_get_2))
        (set `local.Delta` _delta_2))
      (:`then_2`
        (bind _newdirection_2 (`/Game/ChessOfModernUnits/GameObjects/Units/Blueprints/BPFL_CoordsAndDirectionTransforms.GetDirectionAfterRotate` "NewEnumerator3" _direction))
        (bind _output_get_3 (set `local.FireDirection` _newdirection_2))
        (bind _delta_3 (`/Game/ChessOfModernUnits/GameObjects/Units/Blueprints/BPFL_CoordsAndDirectionTransforms.GetDeltaCoordsByDirection` _output_get_3))
        (set `local.Delta` _delta_3))
      (:`then_3`
        (return (`local.TargetMap`))))
    (set `local.index` 1)
    (bind ((`FirePower_10_3428025D4CF403F8858B5B83C7B1041B` _firepower) (`BlindZone_12_98228E844B591E4CE72540B50D3DD78A` _blindzone) (`MaxFireDistance_14_939E1B2446C6D32BFFCF4AA41B57C7BE` _maxfiredistance) (`possibleLandscapeTypes_18_325AA1B743E4368F4960A1A4BF9C1399` _possiblelandscapetypes)) (break `/Game/ChessOfModernUnits/GameObjects/Units/Blueprints/Modules/TableStructures/SModuleSettings` (`.Settings_12_A8061B9948A0E1B34868A88E70641730` (break `/Game/ChessOfModernUnits/GameObjects/Units/Blueprints/Modules/TableStructures/SModuleDescription` _moduledescription))))
    (while (and _cellfound (`BlueprintSetLibrary.Set_Contains` _possiblelandscapetypes _landscapetype) (or (<= (`local.index`) _maxfiredistance) (== _maxfiredistance -1)))
      (if (and (> (`local.index`) _blindzone) _unitfound)
        (bind _module (`/Game/ChessOfModernUnits/GameFramework/Player/BPFL_CellsAndUnits.MakeModule` _unitconfig "Main" (`self.GetOwner`)))
        (bind _asbp_base_movement_unit_module_component (cast `/Game/ChessOfModernUnits/GameObjects/Units/Blueprints/Modules/MovementModules/BP_BaseMovementUnitModuleComponent` _module))
        (bind (_newunitconfig _possible) (`/Game/ChessOfModernUnits/GameObjects/Units/Blueprints/Modules/MovementModules/BP_BaseMovementUnitModuleComponent.ApplyDamage` _asbp_base_movement_unit_module_component _firepower (`local.FireDirection`) _unitconfig))
        (if (and _possible (`|EnumInequality` _unitconfig_side (`.Side_59_393DC6B94AC999E7C6758C8FD57E2723` (break `/Game/ChessOfModernUnits/GameObjects/Units/Blueprints/SUnitConfig` _unitconfig))))
          (`BlueprintMapLibrary.Map_Add` (`local.TargetMap`) (`/Game/ChessOfModernUnits/GameObjects/Units/Blueprints/BPFL_CoordsAndDirectionTransforms.AddCoords` _unitconfig_coords_3 (`/Game/ChessOfModernUnits/GameObjects/Units/Blueprints/BPFL_CoordsAndDirectionTransforms.MultiplyCoords` (`local.Delta`) (`local.index`))) _newunitconfig))
        (`/Engine/EditorBlueprintResources/StandardMacros.IncrementInt` (`local.index`)
          (:`  `
            (`self.K2_DestroyComponent` _module)))
        (else
          (`/Engine/EditorBlueprintResources/StandardMacros.IncrementInt` (`local.index`)))))
    (else
      (return))))

(fn `VisualizeMove`
  (params (Move :type "/Game/ChessOfModernUnits/GameObjects/Units/Blueprints/SUnitMove Structure"))
  (locals (FirePower :type Integer :default 0) (DeltaMap :type "Map of /Game/ChessOfModernUnits/GameObjects/Field/Blueprints/SFieldCellCoords Structure to /Game/ChessOfModernUnits/GameObjects/Units/Blueprints/EDirection Enum"))
  (bind ((`TargetCoords_19_2070F9A84A98EEC52500C0B0A346909D` _targetcoords)) (break `/Game/ChessOfModernUnits/GameObjects/Units/Blueprints/SUnitMove` Move))
  (set `local.DeltaMap` (`|MakeMap` (make `/Game/ChessOfModernUnits/GameObjects/Field/Blueprints/SFieldCellCoords` 0 1) "NewEnumerator0" (make `/Game/ChessOfModernUnits/GameObjects/Field/Blueprints/SFieldCellCoords` 0 -1) "NewEnumerator1" (make `/Game/ChessOfModernUnits/GameObjects/Field/Blueprints/SFieldCellCoords` 1 0) "NewEnumerator2" (make `/Game/ChessOfModernUnits/GameObjects/Field/Blueprints/SFieldCellCoords` -1 0) "NewEnumerator3" (make `/Game/ChessOfModernUnits/GameObjects/Field/Blueprints/SFieldCellCoords` 1 1) "NewEnumerator4" (make `/Game/ChessOfModernUnits/GameObjects/Field/Blueprints/SFieldCellCoords` -1 1) "NewEnumerator5" (make `/Game/ChessOfModernUnits/GameObjects/Field/Blueprints/SFieldCellCoords` 1 -1) "NewEnumerator6" (make `/Game/ChessOfModernUnits/GameObjects/Field/Blueprints/SFieldCellCoords` -1 -1) "NewEnumerator7" :!type "/Game/ChessOfModernUnits/GameObjects/Field/Blueprints/SFieldCellCoords Structure" :!valuetype "/Game/ChessOfModernUnits/GameObjects/Units/Blueprints/EDirection Enum"))
  (bind _asbp_unit (cast `/Game/ChessOfModernUnits/GameObjects/Units/Blueprints/BP_Unit` (`self.GetOwner`)))
  (bind _unit_config (`/Game/ChessOfModernUnits/GameObjects/Units/Blueprints/BP_Unit.Unit Config` _asbp_unit))
  (bind _moduledescription (`/Game/ChessOfModernUnits/GameFramework/Player/BPFL_CellsAndUnits.GetModuleDescription` _unit_config (`self.Socket`)))
  (set `local.FirePower` (`.FirePower_10_3428025D4CF403F8858B5B83C7B1041B` (break `/Game/ChessOfModernUnits/GameObjects/Units/Blueprints/Modules/TableStructures/SModuleSettings` (`.Settings_12_A8061B9948A0E1B34868A88E70641730` (break `/Game/ChessOfModernUnits/GameObjects/Units/Blueprints/Modules/TableStructures/SModuleDescription` _moduledescription)))))
  (bind _outactors (`GameplayStatics.GetAllActorsOfClass` "/Game/ChessOfModernUnits/GameObjects/Units/Blueprints/BP_Unit.BP_Unit_C"))
  (for _array_element _outactors
    (bind _unit_config_2 (`/Game/ChessOfModernUnits/GameObjects/Units/Blueprints/BP_Unit.Unit Config` _array_element))
    (if (`/Game/ChessOfModernUnits/GameObjects/Units/Blueprints/BPFL_CoordsAndDirectionTransforms.EqualCoords` (`.Coords_47_E98C47904C4A4C6B43CCA291531B50D8` (break `/Game/ChessOfModernUnits/GameObjects/Units/Blueprints/SUnitConfig` _unit_config_2)) _targetcoords)
      (bind _module (`/Game/ChessOfModernUnits/GameFramework/Player/BPFL_CellsAndUnits.MakeModule` _unit_config_2 "Main" (`self.GetOwner`)))
      (bind _asbp_base_movement_unit_module_component (cast `/Game/ChessOfModernUnits/GameObjects/Units/Blueprints/Modules/MovementModules/BP_BaseMovementUnitModuleComponent` _module))
      (bind (_xcoord _ycoord) (break `/Game/ChessOfModernUnits/GameObjects/Field/Blueprints/SFieldCellCoords` (`/Game/ChessOfModernUnits/GameObjects/Units/Blueprints/BPFL_CoordsAndDirectionTransforms.AddCoords` _targetcoords (`/Game/ChessOfModernUnits/GameObjects/Units/Blueprints/BPFL_CoordsAndDirectionTransforms.MultiplyCoords` (`.Coords_47_E98C47904C4A4C6B43CCA291531B50D8` (break `/Game/ChessOfModernUnits/GameObjects/Units/Blueprints/SUnitConfig` _unit_config)) -1))))
      (bind _unit_config_3 (`/Game/ChessOfModernUnits/GameObjects/Units/Blueprints/BP_Unit.Unit Config` _array_element))
      (bind _newunitconfig (`/Game/ChessOfModernUnits/GameObjects/Units/Blueprints/Modules/MovementModules/BP_BaseMovementUnitModuleComponent.ApplyDamage` _asbp_base_movement_unit_module_component (`local.FirePower`) (`BlueprintMapLibrary.Map_Find` (`local.DeltaMap`) (make `/Game/ChessOfModernUnits/GameObjects/Field/Blueprints/SFieldCellCoords` (`KismetMathLibrary.SignOfInteger` _xcoord) (`KismetMathLibrary.SignOfInteger` _ycoord))) _unit_config_3))
      (`/Game/ChessOfModernUnits/GameObjects/Units/Blueprints/BP_Unit.SetConfig` _array_element _newunitconfig)
      (`self.K2_DestroyComponent` _module)
      (bind (_tempstate_movepoints _tempstate_canuse) (break `/Game/ChessOfModernUnits/GameObjects/Units/Blueprints/SUnitTempState` (break `/Game/ChessOfModernUnits/GameObjects/Units/Blueprints/SUnitConfig` _unit_config_3)))
      (`BlueprintMapLibrary.Map_Add` _tempstate_canuse (`self.Socket`))
      (setmembers `/Game/ChessOfModernUnits/GameObjects/Units/Blueprints/SUnitConfig` :`StructRef` _unit_config_3 :`TempState` (make `/Game/ChessOfModernUnits/GameObjects/Units/Blueprints/SUnitTempState` 0 _tempstate_canuse)))))