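; Base movement module component for chess-like units, handling one-cell forward or backward steps, turns, and directional armor hits.
; ComputeMove simulates moves on field state, checking move points, occupancy and landscape; one landscape type is enterable only across the side boundary with ComTankAntenne.
; GetPossibleMoves collects valid results from ComputeMove, while VisualizeMove applies moves to the owning BP_Unit.
; Backing up spends all move points; ApplyDamage kills when firepower exceeds facing armor.
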(fn `ApplyDamage`
  (params (FirePower :type Integer) (Direction :type "/Game/ChessOfModernUnits/GameObjects/Units/Blueprints/EDirection Enum" :default "NewEnumerator0") (UnitConfig :type "/Game/ChessOfModernUnits/GameObjects/Units/Blueprints/SUnitConfig Structure"))
  (returns (NewUnitConfig :type "/Game/ChessOfModernUnits/GameObjects/Units/Blueprints/SUnitConfig Structure") (Possible :type Boolean))
  (bind ((`Direction_56_4F2B10F847F49B1199F4DC823B142897` _direction) (`Alive_50_F54C53F84EFA66D3B0170BB8E9F0CD80` _alive)) (break `/Game/ChessOfModernUnits/GameObjects/Units/Blueprints/SUnitConfig` UnitConfig))
  (bind _diametral (`/Game/ChessOfModernUnits/GameObjects/Units/Blueprints/BPFL_CoordsAndDirectionTransforms.GetDiametralDirection` Direction))
  (bind _moduledescription (`/Game/ChessOfModernUnits/GameFramework/Player/BPFL_CellsAndUnits.GetModuleDescription` UnitConfig))
  (bind _relativedirection (`/Game/ChessOfModernUnits/GameObjects/Units/Blueprints/BPFL_CoordsAndDirectionTransforms.GetRelativeDirection` _direction _diametral))
  (if (> FirePower (`BlueprintMapLibrary.Map_Find` (`.Armor_4_283E36774AD8634EAB99089208703545` (break `/Game/ChessOfModernUnits/GameObjects/Units/Blueprints/Modules/TableStructures/SModuleSettings` (`.Settings_12_A8061B9948A0E1B34868A88E70641730` (break `/Game/ChessOfModernUnits/GameObjects/Units/Blueprints/Modules/TableStructures/SModuleDescription` _moduledescription)))) _relativedirection))
    (bind _structout (setmembers `/Game/ChessOfModernUnits/GameObjects/Units/Blueprints/SUnitConfig` :`StructRef` (`|Copy` (`local.UnitConfig`)) :`Alive` false))
    (return _structout _alive)
    (else
      (return (struct) false))))

(fn `ComputeMove`
  (params (FieldState :type "/Game/ChessOfModernUnits/GameObjects/Field/Blueprints/SFieldState Structure") (UnitConfig :type "/Game/ChessOfModernUnits/GameObjects/Units/Blueprints/SUnitConfig Structure") (Move :type "/Game/ChessOfModernUnits/GameObjects/Units/Blueprints/SUnitMove Structure"))
  (returns (NewFieldState :type "/Game/ChessOfModernUnits/GameObjects/Field/Blueprints/SFieldState Structure") (NewUnitConfig :type "/Game/ChessOfModernUnits/GameObjects/Units/Blueprints/SUnitConfig Structure") (Possible :type Boolean))
  (locals (Delta :type "/Game/ChessOfModernUnits/GameObjects/Field/Blueprints/SFieldCellCoords Structure"))
  (bind _tempstate_movepoints (break `/Game/ChessOfModernUnits/GameObjects/Units/Blueprints/SUnitTempState` (break `/Game/ChessOfModernUnits/GameObjects/Units/Blueprints/SUnitConfig` UnitConfig)))
  (bind (_move_activecomponent _move_targetcoords _move_movement) (break `/Game/ChessOfModernUnits/GameObjects/Units/Blueprints/SUnitMove` (`local.Move`)))
  (bind _unitconfig (`local.UnitConfig`))
  (bind (_move_activecomponent_2 _move_targetcoords_2 _move_movement_2) (break `/Game/ChessOfModernUnits/GameObjects/Units/Blueprints/SUnitMove` (`local.Move`)))
  (bind _unitconfig_2 (`local.UnitConfig`))
  (bind _unitconfig_3 (`local.UnitConfig`))
  (bind ((`Coords_47_E98C47904C4A4C6B43CCA291531B50D8` _coords) (`Direction_56_4F2B10F847F49B1199F4DC823B142897` _direction)) (break `/Game/ChessOfModernUnits/GameObjects/Units/Blueprints/SUnitConfig` _unitconfig_2))
  (bind ((`Coords_47_E98C47904C4A4C6B43CCA291531B50D8` _coords_2) (`Direction_56_4F2B10F847F49B1199F4DC823B142897` _direction_2) (`TempState_62_5ABFF3A34B4DD39392594A92040E2E81` _tempstate)) (break `/Game/ChessOfModernUnits/GameObjects/Units/Blueprints/SUnitConfig` _unitconfig))
  (bind ((`ModuleOnSockets_65_93C0F6A14F5C249A946557A0ACBCDE35` _moduleonsockets) (`Coords_47_E98C47904C4A4C6B43CCA291531B50D8` _coords_3) (`Side_59_393DC6B94AC999E7C6758C8FD57E2723` _side)) (break `/Game/ChessOfModernUnits/GameObjects/Units/Blueprints/SUnitConfig` (`local.UnitConfig`)))
  (bind ((`Coords_47_E98C47904C4A4C6B43CCA291531B50D8` _coords_4) (`TempState_62_5ABFF3A34B4DD39392594A92040E2E81` _tempstate_2)) (break `/Game/ChessOfModernUnits/GameObjects/Units/Blueprints/SUnitConfig` _unitconfig_3))
  (bind (_cellfound _unitfound _landscapetype) (`/Game/ChessOfModernUnits/GameFramework/Player/BPFL_CellsAndUnits.GetCell` (`local.FieldState`) (`/Game/ChessOfModernUnits/GameObjects/Units/Blueprints/BPFL_CoordsAndDirectionTransforms.AddCoords` _coords (`local.Delta`))))
  (if (> _tempstate_movepoints 0)
    (switch `/Game/ChessOfModernUnits/GameObjects/Units/Blueprints/Modules/MovementModules/EMovements` _move_movement_2
      (:`NewEnumerator0`
        _)
      (:`NewEnumerator1`
        _)
      (:`NewEnumerator2`
        (bind _newdirection (`/Game/ChessOfModernUnits/GameObjects/Units/Blueprints/BPFL_CoordsAndDirectionTransforms.GetDirectionAfterRotate` _move_movement_2 _direction_2 :!label _label))
        (bind _structout (setmembers `/Game/ChessOfModernUnits/GameObjects/Units/Blueprints/SUnitConfig` :`StructRef` (`|Copy` _unitconfig) :`Direction` _newdirection :`TempState` (make `/Game/ChessOfModernUnits/GameObjects/Units/Blueprints/SUnitTempState` (- (break `/Game/ChessOfModernUnits/GameObjects/Units/Blueprints/SUnitTempState` _tempstate) 1) (`.CanUse_23_BE99ED37467B2319636ED0A69AB3D10F` (break `/Game/ChessOfModernUnits/GameObjects/Units/Blueprints/SUnitTempState` _tempstate)))))
        (bind _newfieldstate (`/Game/ChessOfModernUnits/GameFramework/Player/BPFL_CellsAndUnits.ChangeUnit` (`local.FieldState`) _coords_2 _structout))
        (return _newfieldstate _structout true))
      (:`NewEnumerator3`
        (goto _label)))
    (bind _delta (`/Game/ChessOfModernUnits/GameObjects/Units/Blueprints/BPFL_CoordsAndDirectionTransforms.GetDeltaCoordsByDirection` _direction))
    (bind _output_get (set `local.Delta` _delta))
    (if (`|EnumEquality` _move_movement_2 "NewEnumerator1")
      (set `local.Delta` (`/Game/ChessOfModernUnits/GameObjects/Units/Blueprints/BPFL_CoordsAndDirectionTransforms.MultiplyCoords` _output_get -1)))
    (bind _moduledescription (`/Game/ChessOfModernUnits/GameFramework/Player/BPFL_CellsAndUnits.GetModuleDescription` _unitconfig_2))
    (if (and _cellfound (not _unitfound) (`BlueprintSetLibrary.Set_Contains` (`.possibleLandscapeTypes_18_325AA1B743E4368F4960A1A4BF9C1399` (break `/Game/ChessOfModernUnits/GameObjects/Units/Blueprints/Modules/TableStructures/SModuleSettings` (`.Settings_12_A8061B9948A0E1B34868A88E70641730` (break `/Game/ChessOfModernUnits/GameObjects/Units/Blueprints/Modules/TableStructures/SModuleDescription` _moduledescription)))) _landscapetype))
      (if (`|EnumEquality` _landscapetype "NewEnumerator3")
        (if (`|EnumInequality` (select `bool` (> (`.YCoord_12_230624BA45D1462C62A7DA860B56371E` (break `/Game/ChessOfModernUnits/GameObjects/Field/Blueprints/SFieldCellCoords` (`/Game/ChessOfModernUnits/GameObjects/Units/Blueprints/BPFL_CoordsAndDirectionTransforms.AddCoords` _coords_3 (`local.Delta`)))) 0) :`false` "NewEnumerator1" :`true` "NewEnumerator0" :!type "/Game/ChessOfModernUnits/GameFramework/Player/EPlayerSide Enum") _side)
          (bind _values (`BlueprintMapLibrary.Map_Values` _moduleonsockets))
          (if (`KismetArrayLibrary.Array_Contains` _values "ComTankAntenne")
            _
            (else
              (return (struct) (struct) false)))
          (else
            (return (struct) (struct) false))))
      (bind _structout_2 (setmembers `/Game/ChessOfModernUnits/GameObjects/Units/Blueprints/SUnitConfig` :`StructRef` (`|Copy` _unitconfig_3) :`Coords` (`/Game/ChessOfModernUnits/GameObjects/Units/Blueprints/BPFL_CoordsAndDirectionTransforms.AddCoords` _coords_4 (`local.Delta`)) :`TempState` (make `/Game/ChessOfModernUnits/GameObjects/Units/Blueprints/SUnitTempState` (select `bool` (`|EnumEquality` _move_movement "NewEnumerator1") :`false` (- (break `/Game/ChessOfModernUnits/GameObjects/Units/Blueprints/SUnitTempState` _tempstate_2) 1)) (`.CanUse_23_BE99ED37467B2319636ED0A69AB3D10F` (break `/Game/ChessOfModernUnits/GameObjects/Units/Blueprints/SUnitTempState` _tempstate_2)))))
      (bind _newfieldstate_2 (`/Game/ChessOfModernUnits/GameFramework/Player/BPFL_CellsAndUnits.ChangeUnit` (`local.FieldState`) _coords_4 _structout_2))
      (return _newfieldstate_2 _structout_2 true)
      (else
        (return (struct) (struct) false)))
    (else
      (return (struct) (struct) false))))

(fn `GetPossibleMoves`
  (params (FieldState :type "/Game/ChessOfModernUnits/GameObjects/Field/Blueprints/SFieldState Structure") (UnitConfig :type "/Game/ChessOfModernUnits/GameObjects/Units/Blueprints/SUnitConfig Structure"))
  (returns (PossibleMoves :type "Map of /Game/ChessOfModernUnits/GameObjects/Units/Blueprints/SUnitMove Structure to /Game/ChessOfModernUnits/GameObjects/Units/Blueprints/SUnitConfig Structure"))
  (locals (Moves :type "Map of /Game/ChessOfModernUnits/GameObjects/Units/Blueprints/SUnitMove Structure to /Game/ChessOfModernUnits/GameObjects/Units/Blueprints/SUnitConfig Structure"))
  (bind _enumvalue (foreach `/Game/ChessOfModernUnits/GameObjects/Units/Blueprints/Modules/MovementModules/EMovements` false)
    (:`LoopBody`
      (bind _sunitmove (make `/Game/ChessOfModernUnits/GameObjects/Units/Blueprints/SUnitMove` (`self.Socket`) (struct :`XCoord` -2 :`YCoord` -2) _enumvalue))
      (bind (_newfieldstate _newunitconfig _possible) (`self.ComputeMove` FieldState UnitConfig _sunitmove))
      (if _possible
        (`BlueprintMapLibrary.Map_Add` (`local.Moves`) _sunitmove _newunitconfig)))
    (:`then`
      (return (`local.Moves`)))))

(fn `VisualizeMove`
  (params (Move :type "/Game/ChessOfModernUnits/GameObjects/Units/Blueprints/SUnitMove Structure"))
  (locals (Delta :type "/Game/ChessOfModernUnits/GameObjects/Field/Blueprints/SFieldCellCoords Structure"))
  (bind (_activecomponent _targetcoords _movement) (break `/Game/ChessOfModernUnits/GameObjects/Units/Blueprints/SUnitMove` Move))
  (bind _asbp_unit (cast `/Game/ChessOfModernUnits/GameObjects/Units/Blueprints/BP_Unit` (`self.GetOwner`)))
  (switch `/Game/ChessOfModernUnits/GameObjects/Units/Blueprints/Modules/MovementModules/EMovements` _movement
    (:`NewEnumerator0`
      (bind ((`Coords_47_E98C47904C4A4C6B43CCA291531B50D8` _coords) (`Direction_56_4F2B10F847F49B1199F4DC823B142897` _direction)) (break `/Game/ChessOfModernUnits/GameObjects/Units/Blueprints/SUnitConfig` (`/Game/ChessOfModernUnits/GameObjects/Units/Blueprints/BP_Unit.Unit Config` _asbp_unit)))
      (bind _delta (`/Game/ChessOfModernUnits/GameObjects/Units/Blueprints/BPFL_CoordsAndDirectionTransforms.GetDeltaCoordsByDirection` _direction))
      (set `local.Delta` _delta)
      (`/Game/ChessOfModernUnits/GameObjects/Units/Blueprints/BP_Unit.SetCoords` _asbp_unit (`/Game/ChessOfModernUnits/GameObjects/Units/Blueprints/BPFL_CoordsAndDirectionTransforms.AddCoords` _coords (`local.Delta`)) :!label _label))
    (:`NewEnumerator1`
      (bind _delta_2 (`/Game/ChessOfModernUnits/GameObjects/Units/Blueprints/BPFL_CoordsAndDirectionTransforms.GetDeltaCoordsByDirection` _direction))
      (set `local.Delta` (`/Game/ChessOfModernUnits/GameObjects/Units/Blueprints/BPFL_CoordsAndDirectionTransforms.MultiplyCoords` _delta_2 -1))
      (goto _label))
    (:`NewEnumerator2`
      (bind _newdirection (`/Game/ChessOfModernUnits/GameObjects/Units/Blueprints/BPFL_CoordsAndDirectionTransforms.GetDirectionAfterRotate` _movement _direction :!label _label_2))
      (`/Game/ChessOfModernUnits/GameObjects/Units/Blueprints/BP_Unit.SetDirection` _asbp_unit _newdirection))
    (:`NewEnumerator3`
      (goto _label_2)))
  (bind _unit_config (`/Game/ChessOfModernUnits/GameObjects/Units/Blueprints/BP_Unit.Unit Config` _asbp_unit))
  (bind (_tempstate_movepoints _tempstate_canuse) (break `/Game/ChessOfModernUnits/GameObjects/Units/Blueprints/SUnitTempState` (break `/Game/ChessOfModernUnits/GameObjects/Units/Blueprints/SUnitConfig` _unit_config)))
  (setmembers `/Game/ChessOfModernUnits/GameObjects/Units/Blueprints/SUnitConfig` :`StructRef` _unit_config :`TempState` (make `/Game/ChessOfModernUnits/GameObjects/Units/Blueprints/SUnitTempState` (select `bool` (`|EnumEquality` _movement "NewEnumerator1") :`false` (- _tempstate_movepoints 1)) _tempstate_canuse)))