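; Blueprint function library of grid coordinate and direction math for units on the Chess of Modern Units field.
; Direction helpers use lookup maps to rotate left or right, find the opposite direction, and turn a direction into a cell delta.
; Relative direction comes from rotating observer and target right together until the observer reaches the first enum value.
; Coordinate helpers compare, add and scale cell coordinates.
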(fn `AddCoords`
  (params (Coords1 :type "/Game/ChessOfModernUnits/GameObjects/Field/Blueprints/SFieldCellCoords Structure") (Coords2 :type "/Game/ChessOfModernUnits/GameObjects/Field/Blueprints/SFieldCellCoords Structure"))
  (returns (CoordsOut :type "/Game/ChessOfModernUnits/GameObjects/Field/Blueprints/SFieldCellCoords Structure"))
  (bind (_xcoord _ycoord) (break `/Game/ChessOfModernUnits/GameObjects/Field/Blueprints/SFieldCellCoords` Coords1))
  (bind (_xcoord_2 _ycoord_2) (break `/Game/ChessOfModernUnits/GameObjects/Field/Blueprints/SFieldCellCoords` Coords2))
  (return (make `/Game/ChessOfModernUnits/GameObjects/Field/Blueprints/SFieldCellCoords` (+ _xcoord _xcoord_2) (+ _ycoord_2 _ycoord))))

(fn `EqualCoords`
  (params (Coords1 :type "/Game/ChessOfModernUnits/GameObjects/Field/Blueprints/SFieldCellCoords Structure") (Coords2 :type "/Game/ChessOfModernUnits/GameObjects/Field/Blueprints/SFieldCellCoords Structure"))
  (returns (Equal :type Boolean))
  (bind (_xcoord _ycoord) (break `/Game/ChessOfModernUnits/GameObjects/Field/Blueprints/SFieldCellCoords` Coords1))
  (bind (_xcoord_2 _ycoord_2) (break `/Game/ChessOfModernUnits/GameObjects/Field/Blueprints/SFieldCellCoords` Coords2))
  (return (and (== _xcoord _xcoord_2) (== _ycoord _ycoord_2))))

(fn `GetDeltaCoordsByDirection`
  (params (Direction :type "/Game/ChessOfModernUnits/GameObjects/Units/Blueprints/EDirection Enum" :default "NewEnumerator0"))
  (returns (Delta :type "/Game/ChessOfModernUnits/GameObjects/Field/Blueprints/SFieldCellCoords Structure"))
  (locals (DeltaMap :type "Map of /Game/ChessOfModernUnits/GameObjects/Units/Blueprints/EDirection Enum to /Game/ChessOfModernUnits/GameObjects/Field/Blueprints/SFieldCellCoords Structure"))
  (return (`BlueprintMapLibrary.Map_Find` (`local.DeltaMap`) Direction)))

(fn `GetDiametralDirection`
  (params (Direction :type "/Game/ChessOfModernUnits/GameObjects/Units/Blueprints/EDirection Enum" :default "NewEnumerator0"))
  (returns (Diametral :type "/Game/ChessOfModernUnits/GameObjects/Units/Blueprints/EDirection Enum"))
  (locals (Directions :type "Map of /Game/ChessOfModernUnits/GameObjects/Units/Blueprints/EDirection Enum to /Game/ChessOfModernUnits/GameObjects/Units/Blueprints/EDirection Enum"))
  (return (`BlueprintMapLibrary.Map_Find` (`local.Directions`) Direction)))

(fn `GetDirectionAfterRotate`
  (params (Rotate :type "/Game/ChessOfModernUnits/GameObjects/Units/Blueprints/Modules/MovementModules/EMovements Enum" :default "NewEnumerator0") (Direction :type "/Game/ChessOfModernUnits/GameObjects/Units/Blueprints/EDirection Enum" :default "NewEnumerator0"))
  (returns (NewDirection :type "/Game/ChessOfModernUnits/GameObjects/Units/Blueprints/EDirection Enum"))
  (locals (LeftRotate :type "Map of /Game/ChessOfModernUnits/GameObjects/Units/Blueprints/EDirection Enum to /Game/ChessOfModernUnits/GameObjects/Units/Blueprints/EDirection Enum") (RightRotate :type "Map of /Game/ChessOfModernUnits/GameObjects/Units/Blueprints/EDirection Enum to /Game/ChessOfModernUnits/GameObjects/Units/Blueprints/EDirection Enum"))
  (switch `/Game/ChessOfModernUnits/GameObjects/Units/Blueprints/Modules/MovementModules/EMovements` Rotate
    (:`NewEnumerator2`
      (return (`BlueprintMapLibrary.Map_Find` (`local.LeftRotate`) Direction)))
    (:`NewEnumerator3`
      (return (`BlueprintMapLibrary.Map_Find` (`local.RightRotate`) Direction)))))

(fn `GetRelativeDirection`
  (params (AbsoluteDirection :type "/Game/ChessOfModernUnits/GameObjects/Units/Blueprints/EDirection Enum" :default "NewEnumerator0") (ObserverDirection :type "/Game/ChessOfModernUnits/GameObjects/Units/Blueprints/EDirection Enum" :default "NewEnumerator0"))
  (returns (RelativeDirection :type "/Game/ChessOfModernUnits/GameObjects/Units/Blueprints/EDirection Enum"))
  (locals (TempObserverDirection :type "/Game/ChessOfModernUnits/GameObjects/Units/Blueprints/EDirection Enum") (TempAbsoluteDirection :type "/Game/ChessOfModernUnits/GameObjects/Units/Blueprints/EDirection Enum"))
  (set `local.TempAbsoluteDirection` AbsoluteDirection)
  (set `local.TempObserverDirection` ObserverDirection)
  (while (`|EnumInequality` (`local.TempObserverDirection`) "NewEnumerator0")
    (bind _newdirection (`self.GetDirectionAfterRotate` "NewEnumerator3" (`local.TempObserverDirection`)))
    (set `local.TempObserverDirection` _newdirection)
    (bind _newdirection_2 (`self.GetDirectionAfterRotate` "NewEnumerator3" (`local.TempAbsoluteDirection`)))
    (set `local.TempAbsoluteDirection` _newdirection_2))
  (return (`local.TempAbsoluteDirection`)))

(fn `MultiplyCoords`
  (params (Coords :type "/Game/ChessOfModernUnits/GameObjects/Field/Blueprints/SFieldCellCoords Structure") (Multyplier :type Integer))
  (returns (CoordsOut :type "/Game/ChessOfModernUnits/GameObjects/Field/Blueprints/SFieldCellCoords Structure"))
  (bind (_xcoord _ycoord) (break `/Game/ChessOfModernUnits/GameObjects/Field/Blueprints/SFieldCellCoords` Coords))
  (return (make `/Game/ChessOfModernUnits/GameObjects/Field/Blueprints/SFieldCellCoords` (* _xcoord Multyplier) (* _ycoord Multyplier))))