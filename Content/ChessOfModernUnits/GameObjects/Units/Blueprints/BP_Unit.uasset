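; Modular chess-style unit that builds, places and tints itself from a UnitConfig, optionally passed through a replication component.
; Socketed skeletal meshes form its body; grid coords, direction, alive state and side drive transform and color.
; Moves are visualized by temporary module objects, then the field state is saved to player controllers.
; It resets move points and usable modules, binds to end-move on authority, and selects its cell on left click.
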(event `self.ReceiveBeginPlay`
  (bind _unit_config (`self.Unit Config`))
  (if (`self.bReplicates`)
    (bind _replconfig (`/Game/ChessOfModernUnits/Core/BP_ReplicationComponent.ReplicateUnitConfig` (`self.BP_ReplicationComponent`) _unit_config))
    (`self.SetConfig` _replconfig)
    (set `self.Unit Config` _replconfig)
    (else
      (`self.SetConfig` _unit_config)))
  (`self.ReloadTempState`)
  (`/Engine/EditorBlueprintResources/ActorMacros.Switch Has Authority`
    (:`Authority`
      (bind _asbp_game_mode (cast `/Game/ChessOfModernUnits/GameFramework/Singletons/BP_GameMode` (`GameplayStatics.GetGameMode`)))
      (add `/Game/ChessOfModernUnits/GameFramework/Singletons/BP_GameMode.onEndMove` _asbp_game_mode (`|CreateDelegate` :!event `ReloadTempState`)))))

(event `MakeMove`
  (params (Moves :type "Array of /Game/ChessOfModernUnits/GameObjects/Units/Blueprints/SUnitMove Structure (by ref)"))
  (`self.MakeMoves` Moves)
  (bind _fieldstate (`/Game/ChessOfModernUnits/GameFramework/Player/BPFL_CellsAndUnits.GetFieldConfigFromWorld`))
  (bind _outactors (`GameplayStatics.GetAllActorsOfClass` "/Game/ChessOfModernUnits/GameFramework/Player/BP_PlayerController.BP_PlayerController_C"))
  (for _array_element _outactors
    (set `/Game/ChessOfModernUnits/GameFramework/Player/BP_PlayerController.SavedFieldState` _fieldstate _array_element)))

(event `ReloadTempState`
  (bind _unit_config (`self.Unit Config`))
  (`self.ReloadStateF`)
  (bind _outactors (`GameplayStatics.GetAllActorsOfClass` "/Game/ChessOfModernUnits/GameFramework/Player/BP_PlayerController.BP_PlayerController_C"))
  (for _array_element _outactors
    (bind _savedfieldstate (`/Game/ChessOfModernUnits/GameFramework/Player/BP_PlayerController.SavedFieldState` _array_element))
    (bind ((`Units_31_8194BC274A1D6B758B12AA93D64CC056` _units)) (break `/Game/ChessOfModernUnits/GameObjects/Field/Blueprints/SFieldState` _savedfieldstate))
    (`BlueprintMapLibrary.Map_Add` _units (`.Coords_47_E98C47904C4A4C6B43CCA291531B50D8` (break `/Game/ChessOfModernUnits/GameObjects/Units/Blueprints/SUnitConfig` _unit_config)) _unit_config)
    (setmembers `/Game/ChessOfModernUnits/GameObjects/Field/Blueprints/SFieldState` :`StructRef` _savedfieldstate :`Units` _units)))

(event `self.ReceiveActorOnClicked`
  (params (ButtonPressed :type "Key Structure"))
  (if (== ButtonPressed "LeftMouseButton")
    (bind _asbp_player_controller (cast `/Game/ChessOfModernUnits/GameFramework/Player/BP_PlayerController` (`GameplayStatics.GetPlayerController` 0)))
    (`/Game/ChessOfModernUnits/GameFramework/Player/BP_PlayerController.SelectCelllEvent` _asbp_player_controller (`.Coords_47_E98C47904C4A4C6B43CCA291531B50D8` (break `/Game/ChessOfModernUnits/GameObjects/Units/Blueprints/SUnitConfig` (`self.Unit Config`))))))

(fn `MakeMoves`
  (params (Moves :type "Array of /Game/ChessOfModernUnits/GameObjects/Units/Blueprints/SUnitMove Structure"))
  (for _array_element Moves
    (bind _module (`/Game/ChessOfModernUnits/GameFramework/Player/BPFL_CellsAndUnits.MakeModule` (`self.Unit Config`) (`.ActiveComponent_20_EA598D07478AB8A33D4C1F99ECAC8CF4` (break `/Game/ChessOfModernUnits/GameObjects/Units/Blueprints/SUnitMove` _array_element)) self))
    (`/Game/ChessOfModernUnits/GameObjects/Units/Blueprints/Modules/BP_BaseUnitModuleComponent.VisualizeMove` _module _array_element)
    (`ActorComponent.K2_DestroyComponent` _module)))

(fn `ReloadStateF`
  (locals (NewCanUse :type "Map of Name to Boolean"))
  (bind _unit_config (`self.Unit Config`))
  (bind _keys (`BlueprintMapLibrary.Map_Keys` (`.ModuleOnSockets_65_93C0F6A14F5C249A946557A0ACBCDE35` (break `/Game/ChessOfModernUnits/GameObjects/Units/Blueprints/SUnitConfig` (`self.Unit Config`)))))
  (for _array_element _keys
    (bind _moduledescription (`/Game/ChessOfModernUnits/GameFramework/Player/BPFL_CellsAndUnits.GetModuleDescription` _unit_config _array_element))
    (if (`.Useable_21_9A2852C141ECCCC31EE7CCB10640289D` (break `/Game/ChessOfModernUnits/GameObjects/Units/Blueprints/Modules/TableStructures/SModuleSettings` (`.Settings_12_A8061B9948A0E1B34868A88E70641730` (break `/Game/ChessOfModernUnits/GameObjects/Units/Blueprints/Modules/TableStructures/SModuleDescription` _moduledescription))))
      (`BlueprintMapLibrary.Map_Add` (`local.NewCanUse`) _array_element true)))
  (bind _moduledescription_2 (`/Game/ChessOfModernUnits/GameFramework/Player/BPFL_CellsAndUnits.GetModuleDescription` _unit_config))
  (setmembers `/Game/ChessOfModernUnits/GameObjects/Units/Blueprints/SUnitConfig` :`StructRef` (`self.Unit Config`) :`TempState` (make `/Game/ChessOfModernUnits/GameObjects/Units/Blueprints/SUnitTempState` (`.MovePointsForStart_8_D00DFDC148C67B0F0303A685945E14EB` (break `/Game/ChessOfModernUnits/GameObjects/Units/Blueprints/Modules/TableStructures/SModuleSettings` (`.Settings_12_A8061B9948A0E1B34868A88E70641730` (break `/Game/ChessOfModernUnits/GameObjects/Units/Blueprints/Modules/TableStructures/SModuleDescription` _moduledescription_2)))) (`local.NewCanUse`))))

(fn `SetAlive`
  (params (Alive :type Boolean))
  (bind (_unit_config_mainmodule _unit_config_moduleonsockets _unit_config_coords _unit_config_direction _unit_config_alive _unit_config_side _unit_config_tempstate) (break `/Game/ChessOfModernUnits/GameObjects/Units/Blueprints/SUnitConfig` (`self.Unit Config`)))
  (set `self.Unit Config` (make `/Game/ChessOfModernUnits/GameObjects/Units/Blueprints/SUnitConfig` _unit_config_mainmodule _unit_config_moduleonsockets _unit_config_coords _unit_config_direction Alive _unit_config_side _unit_config_tempstate))
  (`SceneComponent.K2_SetRelativeRotation` (`self.Mesh`) (`KismetMathLibrary.MakeRotator` (select `bool` Alive :`false` 90.0 :!type "Float (single-precision)")) false false))

(fn `SetConfig`
  (params (UnitConfig :type "/Game/ChessOfModernUnits/GameObjects/Units/Blueprints/SUnitConfig Structure"))
  (bind (_mainmodule _moduleonsockets _coords _direction _alive _side _tempstate) (break `/Game/ChessOfModernUnits/GameObjects/Units/Blueprints/SUnitConfig` UnitConfig))
  (`|ExecutionSequence`
    (:`then_0`
      (`self.SetUpModules` _mainmodule _moduleonsockets))
    (:`then_1`
      (`self.SetCoords` _coords))
    (:`then_2`
      (`self.SetDirection` _direction))
    (:`then_3`
      (`self.SetAlive` _alive))
    (:`then_4`
      (`self.SetSide` _side))
    (:`then_5`
      (setmembers `/Game/ChessOfModernUnits/GameObjects/Units/Blueprints/SUnitConfig` :`StructRef` (`self.Unit Config`) :`TempState` _tempstate))))

(fn `SetCoords`
  (params (Coords :type "/Game/ChessOfModernUnits/GameObjects/Field/Blueprints/SFieldCellCoords Structure"))
  (bind (_xcoord _ycoord) (break `/Game/ChessOfModernUnits/GameObjects/Field/Blueprints/SFieldCellCoords` Coords))
  (bind (_unit_config_mainmodule _unit_config_moduleonsockets _unit_config_coords _unit_config_direction _unit_config_alive _unit_config_side _unit_config_tempstate) (break `/Game/ChessOfModernUnits/GameObjects/Units/Blueprints/SUnitConfig` (`self.Unit Config`)))
  (set `self.Unit Config` (make `/Game/ChessOfModernUnits/GameObjects/Units/Blueprints/SUnitConfig` _unit_config_mainmodule _unit_config_moduleonsockets Coords _unit_config_direction _unit_config_alive _unit_config_side _unit_config_tempstate))
  (`SceneComponent.K2_SetWorldLocation` (`self.DefaultSceneRoot`) (`KismetMathLibrary.MakeVector` (`KismetMathLibrary.Conv_IntToDouble` (* _xcoord 100)) (`KismetMathLibrary.Conv_IntToDouble` (* _ycoord 100))) false false))

(fn `SetDirection`
  (params (Direction :type "/Game/ChessOfModernUnits/GameObjects/Units/Blueprints/EDirection Enum" :default "NewEnumerator0"))
  (locals (RotateForDirection :type "Map of /Game/ChessOfModernUnits/GameObjects/Units/Blueprints/EDirection Enum to Float (double-precision)"))
  (bind (_unit_config_mainmodule _unit_config_moduleonsockets _unit_config_coords _unit_config_direction _unit_config_alive _unit_config_side _unit_config_tempstate) (break `/Game/ChessOfModernUnits/GameObjects/Units/Blueprints/SUnitConfig` (`self.Unit Config`)))
  (bind _defaultsceneroot (`self.DefaultSceneRoot`))
  (bind (_returnvalue_roll _returnvalue_pitch) (`KismetMathLibrary.BreakRotator` (`SceneComponent.K2_GetComponentRotation` _defaultsceneroot)))
  (set `self.Unit Config` (make `/Game/ChessOfModernUnits/GameObjects/Units/Blueprints/SUnitConfig` _unit_config_mainmodule _unit_config_moduleonsockets _unit_config_coords Direction _unit_config_alive _unit_config_side _unit_config_tempstate))
  (`SceneComponent.K2_SetWorldRotation` _defaultsceneroot (`KismetMathLibrary.MakeRotator` _returnvalue_roll _returnvalue_pitch (`BlueprintMapLibrary.Map_Find` (`local.RotateForDirection`) Direction)) false false))

(fn `SetSide`
  (params (Side :type "/Game/ChessOfModernUnits/GameFramework/Player/EPlayerSide Enum" :default "NewEnumerator0"))
  (locals (Color :type "LinearColor Structure") (DynmMI :type "MaterialInstanceDynamic Object Reference"))
  (bind (_unit_config_mainmodule _unit_config_moduleonsockets _unit_config_coords _unit_config_direction _unit_config_alive _unit_config_side _unit_config_tempstate) (break `/Game/ChessOfModernUnits/GameObjects/Units/Blueprints/SUnitConfig` (`self.Unit Config`)))
  (bind _dynmmi (`local.DynmMI`))
  (set `self.Unit Config` (make `/Game/ChessOfModernUnits/GameObjects/Units/Blueprints/SUnitConfig` _unit_config_mainmodule _unit_config_moduleonsockets _unit_config_coords _unit_config_direction _unit_config_alive Side _unit_config_tempstate))
  (set `local.Color` (select `/Game/ChessOfModernUnits/GameFramework/Player/EPlayerSide` Side :`NewEnumerator1` (struct :`R` 1.0 :`G` 1.0 :`B` 1.0 :`A` 1.0) :!type "LinearColor Structure"))
  (for _array_element (`self.K2_GetComponentsByClass` "/Script/Engine.SkeletalMeshComponent")
    (for _index (range (`PrimitiveComponent.GetNumMaterials` _array_element))
      (bind _returnvalue (`PrimitiveComponent.GetMaterial` _array_element _index))
      (bind _asmaterial_instance_dynamic (cast `MaterialInstanceDynamic` _returnvalue)
        (:`then`
          (set `local.DynmMI` _asmaterial_instance_dynamic))
        (:`CastFailed`
          (bind _returnvalue_2 (`KismetMaterialLibrary.CreateDynamicMaterialInstance` _returnvalue))
          (set `local.DynmMI` _returnvalue_2)))
      (`MaterialInstanceDynamic.SetVectorParameterValue` _dynmmi "SideColor" (`local.Color`))
      (`PrimitiveComponent.SetMaterial` _array_element _index _dynmmi))))

(fn `SetUpModules`
  (params (MainModule :type Name) (ModuleOnSockets :type "Map of Name to Name"))
  (bind (_unit_config_mainmodule _unit_config_moduleonsockets _unit_config_coords _unit_config_direction _unit_config_alive _unit_config_side _unit_config_tempstate) (break `/Game/ChessOfModernUnits/GameObjects/Units/Blueprints/SUnitConfig` (`self.Unit Config`)))
  (set `self.Unit Config` (make `/Game/ChessOfModernUnits/GameObjects/Units/Blueprints/SUnitConfig` MainModule ModuleOnSockets _unit_config_coords _unit_config_direction _unit_config_alive _unit_config_side _unit_config_tempstate))
  (`ActorComponent.K2_DestroyComponent` (`SceneComponent.GetChildrenComponents` (`self.Mesh`) false))
  (bind _moduledescription (`/Game/ChessOfModernUnits/GameFramework/Player/BPFL_CellsAndUnits.GetModuleDescription` (`self.Unit Config`)))
  (`SkeletalMeshComponent.SetSkeletalMeshAsset` (`self.Mesh`) (`.SkeletalMesh_7_2A2D0F5A4F381951D55B90AC50BD1F5D` (break `/Game/ChessOfModernUnits/GameObjects/Units/Blueprints/Modules/TableStructures/SModuleDescription` _moduledescription)))
  (bind _keys (`BlueprintMapLibrary.Map_Keys` (`local.ModuleOnSockets`)))
  (for _array_element _keys
    (bind _moduledescription_2 (`/Game/ChessOfModernUnits/GameFramework/Player/BPFL_CellsAndUnits.GetModuleDescription` (`self.Unit Config`) _array_element))
    (bind _returnvalue (`AddComponent|NODE_AddSkeletalMeshComponent-0`))
    (`SkeletalMeshComponent.SetSkeletalMeshAsset` _returnvalue (`.SkeletalMesh_7_2A2D0F5A4F381951D55B90AC50BD1F5D` (break `/Game/ChessOfModernUnits/GameObjects/Units/Blueprints/Modules/TableStructures/SModuleDescription` _moduledescription_2)))
    (`SceneComponent.K2_AttachToComponent` _returnvalue (`self.Mesh`) _array_element "KeepRelative" "KeepRelative" "KeepRelative" true)))

(fn `UserConstructionScript`)