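; Player controller for a turn-based, grid-based unit game, letting the player select their side's living units and plan moves on their turn.
; Cell clicks queue possible moves validated by MoveMaker, or open a HUD way-calculator when none is added.
; Enhanced Input confirms, cancels or undoes the queue, with the HUD visualizing it.
; Confirming calls MakeMoveServer, which revalidates, executes on the unit and notifies the game mode.
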(event `self.ReceiveBeginPlay`
  (bind _returnvalue (subsystem `EnhancedInputLocalPlayerSubsystem`))
  (`/Engine/EditorBlueprintResources/StandardMacros.IsValid` _returnvalue
    (:`Is Valid`
      (`EnhancedInputSubsystemInterface.AddMappingContext` _returnvalue "/Game/ChessOfModernUnits/GameFramework/Player/Input/IMC_MainGameActions.IMC_MainGameActions" 0 (struct))
      (bind _fieldstate (`/Game/ChessOfModernUnits/GameFramework/Player/BPFL_CellsAndUnits.GetFieldConfigFromWorld`))
      (set `self.SavedFieldState` _fieldstate))))

(event `EnhancedInput|/Game/ChessOfModernUnits/GameFramework/Player/Input/Actions/TankControl/IA_ConfirmMove`
  (params (ActionValue :type Boolean) (ElapsedSeconds :type "Float (double-precision)") (TriggeredSeconds :type "Float (double-precision)") (InputAction :type "InputAction Object Reference" :default "/Game/ChessOfModernUnits/GameFramework/Player/Input/Actions/TankControl/IA_ConfirmMove.IA_ConfirmMove"))
  (:`Started`
    (`self.MakeMove`)))

(event `SelectCelllEvent`
  (params (Coords :type "/Game/ChessOfModernUnits/GameObjects/Field/Blueprints/SFieldCellCoords Structure"))
  (bind _movemaker (`self.MoveMaker`))
  (bind (_cellfound _unitfound _landscapetype _unitconfig) (`/Game/ChessOfModernUnits/GameFramework/Player/BPFL_CellsAndUnits.GetCell` (`self.SavedFieldState`) Coords))
  (bind ((`Alive_50_F54C53F84EFA66D3B0170BB8E9F0CD80` _alive) (`Side_59_393DC6B94AC999E7C6758C8FD57E2723` _side)) (break `/Game/ChessOfModernUnits/GameObjects/Units/Blueprints/SUnitConfig` _unitconfig))
  (if (and _cellfound (`self.CanMakeMove`))
    (bind _asbp_player_state (cast `/Game/ChessOfModernUnits/GameFramework/Player/BP_PlayerState` (`self.PlayerState`)))
    (if (`KismetSystemLibrary.IsValid` (`self.SelectedUnit`))
      (bind _added (`self.AddMoveFromPossibles` Coords))
      (if (not _added)
        (bind (_newfieldstate _newunitconfig) (`/Game/ChessOfModernUnits/GameFramework/Player/BP_MoveMakerComponent.ComputeMoves` _movemaker (`.Coords_47_E98C47904C4A4C6B43CCA291531B50D8` (break `/Game/ChessOfModernUnits/GameObjects/Units/Blueprints/SUnitConfig` (`/Game/ChessOfModernUnits/GameObjects/Units/Blueprints/BP_Unit.Unit Config` (`self.SelectedUnit`)))) (`self.Moves`)))
        (bind _ways (`/Game/ChessOfModernUnits/GameFramework/Player/BP_MoveMakerComponent.CalculateWays` _movemaker _newfieldstate _newunitconfig Coords))
        (if (> (`BlueprintMapLibrary.Map_Length` _ways) 0)
          (message `/Game/ChessOfModernUnits/GameFramework/Player/BPI_GameHud.OpenWayCalculator` (`self.GetHUD`) _ways)))
      (elif (and _unitfound _alive (`|EnumEquality` (`/Game/ChessOfModernUnits/GameFramework/Player/BP_PlayerState.side` _asbp_player_state) _side))
        (bind _outactors (`GameplayStatics.GetAllActorsOfClass` "/Game/ChessOfModernUnits/GameObjects/Units/Blueprints/BP_Unit.BP_Unit_C"))
        (for _array_element _outactors
          (bind _unit_config (`/Game/ChessOfModernUnits/GameObjects/Units/Blueprints/BP_Unit.Unit Config` _array_element))
          (if (`/Game/ChessOfModernUnits/GameObjects/Units/Blueprints/BPFL_CoordsAndDirectionTransforms.EqualCoords` Coords (`.Coords_47_E98C47904C4A4C6B43CCA291531B50D8` (break `/Game/ChessOfModernUnits/GameObjects/Units/Blueprints/SUnitConfig` _unit_config)))
            (set `self.SelectedUnit` _array_element)
            (break)))
        (message `/Game/ChessOfModernUnits/GameFramework/Player/BPI_GameHud.SelectUnit` (`self.GetHUD`) _unit_config (`self.SavedFieldState`))))))

(event `EnhancedInput|/Game/ChessOfModernUnits/GameFramework/Player/Input/Actions/TankControl/IA_CancelMove`
  (params (ActionValue :type Boolean) (ElapsedSeconds :type "Float (double-precision)") (TriggeredSeconds :type "Float (double-precision)") (InputAction :type "InputAction Object Reference" :default "/Game/ChessOfModernUnits/GameFramework/Player/Input/Actions/TankControl/IA_CancelMove.IA_CancelMove"))
  (:`Started`
    (`self.ResetMove`)))

(event `EnhancedInput|/Game/ChessOfModernUnits/GameFramework/Player/Input/Actions/TankControl/IA_UndoMovement`
  (params (ActionValue :type Boolean) (ElapsedSeconds :type "Float (double-precision)") (TriggeredSeconds :type "Float (double-precision)") (InputAction :type "InputAction Object Reference" :default "/Game/ChessOfModernUnits/GameFramework/Player/Input/Actions/TankControl/IA_UndoMovement.IA_UndoMovement"))
  (:`Started`
    (`self.UndoMovement`)))

(event `MakeMove`
  (bind (_newfieldstate _newunitconfig _valid) (`/Game/ChessOfModernUnits/GameFramework/Player/BP_MoveMakerComponent.ComputeMoves` (`self.MoveMaker`) (`.Coords_47_E98C47904C4A4C6B43CCA291531B50D8` (break `/Game/ChessOfModernUnits/GameObjects/Units/Blueprints/SUnitConfig` (`/Game/ChessOfModernUnits/GameObjects/Units/Blueprints/BP_Unit.Unit Config` (`self.SelectedUnit`)))) (`self.Moves`)))
  (if _valid
    (`self.MakeMoveServer` (`self.SelectedUnit`) (`self.Moves`))
    (`self.ResetMove`)))

(event `MakeMoveServer`
  (params (Target :type "/Game/ChessOfModernUnits/GameObjects/Units/Blueprints/BP_Unit Object Reference") (Moves :type "Array of /Game/ChessOfModernUnits/GameObjects/Units/Blueprints/SUnitMove Structure (by ref)"))
  (bind (_newfieldstate _newunitconfig _valid) (`/Game/ChessOfModernUnits/GameFramework/Player/BP_MoveMakerComponent.ComputeMoves` (`self.MoveMaker`) (`.Coords_47_E98C47904C4A4C6B43CCA291531B50D8` (break `/Game/ChessOfModernUnits/GameObjects/Units/Blueprints/SUnitConfig` (`/Game/ChessOfModernUnits/GameObjects/Units/Blueprints/BP_Unit.Unit Config` Target))) Moves))
  (if (and _valid (`self.CanMakeMove`) (`KismetSystemLibrary.IsValid` Target))
    (`/Game/ChessOfModernUnits/GameObjects/Units/Blueprints/BP_Unit.MakeMove` Target Moves)
    (bind _asbp_game_mode (cast `/Game/ChessOfModernUnits/GameFramework/Singletons/BP_GameMode` (`GameplayStatics.GetGameMode`)))
    (`/Game/ChessOfModernUnits/GameFramework/Singletons/BP_GameMode.onEndMove` _asbp_game_mode)))

(event `ResetMove`
  (set `self.SelectedUnit` null)
  (`KismetArrayLibrary.Array_Clear` (`self.Moves`))
  (message `/Game/ChessOfModernUnits/GameFramework/Player/BPI_GameHud.UnselectUnit` (`self.GetHUD`)))

(event `UndoMovement`
  (bind _moves (`self.Moves`))
  (bind _moves_2 (`self.Moves`))
  (bind _returnvalue (`KismetArrayLibrary.Array_Length` _moves_2))
  (if (> _returnvalue 0)
    (`KismetArrayLibrary.Array_Remove` _moves_2 (- _returnvalue 1))
    (bind (_newfieldstate _newunitconfig _valid) (`/Game/ChessOfModernUnits/GameFramework/Player/BP_MoveMakerComponent.ComputeMoves` (`self.MoveMaker`) (`.Coords_47_E98C47904C4A4C6B43CCA291531B50D8` (break `/Game/ChessOfModernUnits/GameObjects/Units/Blueprints/SUnitConfig` (`/Game/ChessOfModernUnits/GameObjects/Units/Blueprints/BP_Unit.Unit Config` (`self.SelectedUnit`)))) _moves))
    (message `/Game/ChessOfModernUnits/GameFramework/Player/BPI_GameHud.VisualizeMoves` (`self.GetHUD`) _moves _valid)))

(event `PreMove`
  (params (StateName :type Name))
  (message `/Game/ChessOfModernUnits/GameFramework/Player/BPI_GameHud.ShowGameState` (`self.GetHUD`) StateName))

(fn `AddMove`
  (params (Move :type "/Game/ChessOfModernUnits/GameObjects/Units/Blueprints/SUnitMove Structure"))
  (returns (Possible :type Boolean))
  (bind _moves (`self.Moves`))
  (if (and (`self.CanMakeMove`) (`KismetSystemLibrary.IsValid` (`self.SelectedUnit`)))
    (`KismetArrayLibrary.Array_Add` (`self.Moves`) Move)
    (bind (_newfieldstate _newunitconfig _valid _possible) (`/Game/ChessOfModernUnits/GameFramework/Player/BP_MoveMakerComponent.ComputeMoves` (`self.MoveMaker`) (`.Coords_47_E98C47904C4A4C6B43CCA291531B50D8` (break `/Game/ChessOfModernUnits/GameObjects/Units/Blueprints/SUnitConfig` (`/Game/ChessOfModernUnits/GameObjects/Units/Blueprints/BP_Unit.Unit Config` (`self.SelectedUnit`)))) (`self.Moves`)))
    (if _possible
      (message `/Game/ChessOfModernUnits/GameFramework/Player/BPI_GameHud.VisualizeMoves` (`self.GetHUD`) (`self.Moves`) _valid)
      (return true)
      (else
        (`KismetArrayLibrary.Array_Remove` _moves (- (`KismetArrayLibrary.Array_Length` _moves) 1))
        (return false)))
    (else
      (return false))))

(fn `AddMoveFromPossibles`
  (params (Coords :type "/Game/ChessOfModernUnits/GameObjects/Field/Blueprints/SFieldCellCoords Structure"))
  (returns (Added :type Boolean))
  (locals (AddedMove :type Boolean :default false))
  (bind _movemaker (`self.MoveMaker`))
  (bind _socket (message `/Game/ChessOfModernUnits/GameFramework/Player/BPI_GameHud.GetSelectedSocket` (`self.GetHUD`)))
  (bind (_newfieldstate _newunitconfig) (`/Game/ChessOfModernUnits/GameFramework/Player/BP_MoveMakerComponent.ComputeMoves` _movemaker (`.Coords_47_E98C47904C4A4C6B43CCA291531B50D8` (break `/Game/ChessOfModernUnits/GameObjects/Units/Blueprints/SUnitConfig` (`/Game/ChessOfModernUnits/GameObjects/Units/Blueprints/BP_Unit.Unit Config` (`self.SelectedUnit`)))) (`self.Moves`)))
  (bind _moves (`/Game/ChessOfModernUnits/GameFramework/Player/BP_MoveMakerComponent.GetPossibleMoves` _movemaker _newfieldstate _newunitconfig))
  (bind _result (`BlueprintSetLibrary.Set_ToArray` _moves))
  (for _array_element _result
    (bind ((`ActiveComponent_20_EA598D07478AB8A33D4C1F99ECAC8CF4` _activecomponent) (`TargetCoords_19_2070F9A84A98EEC52500C0B0A346909D` _targetcoords)) (break `/Game/ChessOfModernUnits/GameObjects/Units/Blueprints/SUnitMove` _array_element))
    (if (and (`/Game/ChessOfModernUnits/GameObjects/Units/Blueprints/BPFL_CoordsAndDirectionTransforms.EqualCoords` _targetcoords Coords) (or (== _activecomponent "Main") (== _activecomponent _socket)))
      (bind _possible (`self.AddMove` _array_element))
      (bind _output_get (set `local.AddedMove` _possible))
      (if _output_get
        (break))))
  (return (`local.AddedMove`)))

(fn `CanMakeMove`
  (returns (Enabled :type Boolean))
  (bind _asbp_player_state (cast `/Game/ChessOfModernUnits/GameFramework/Player/BP_PlayerState` (`self.PlayerState`)))
  (bind _asbp_game_state (cast `/Game/ChessOfModernUnits/GameFramework/Singletons/BP_GameState` (`GameplayStatics.GetGameState`)))
  (return (and (`|EnumEquality` (`/Game/ChessOfModernUnits/GameFramework/Singletons/BP_GameState.Now Move Side` _asbp_game_state) (`/Game/ChessOfModernUnits/GameFramework/Player/BP_PlayerState.side` _asbp_player_state)) (== (`/Game/ChessOfModernUnits/GameFramework/Singletons/BP_GameState.StateName` _asbp_game_state) "ReadyToMove"))))

(fn `UserConstructionScript`)