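; Player component that simulates unit moves on field state data for a turn-based game, without applying them.
; Temporary unit modules list possible moves and compute single moves, gated on the unit being alive and on the side to move.
; CalculateWays searches exhaustively by growing its array mid-loop, keeping the route with most move points left per facing at the target.
; ComputeMoves chains moves from the PlayerController's saved state, reporting possibility and whether anything changed.
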(fn `CalculateWays`
  (params (FieldState :type "/Game/ChessOfModernUnits/GameObjects/Field/Blueprints/SFieldState Structure") (UnitConfig :type "/Game/ChessOfModernUnits/GameObjects/Units/Blueprints/SUnitConfig Structure") (TargetCoords :type "/Game/ChessOfModernUnits/GameObjects/Field/Blueprints/SFieldCellCoords Structure"))
  (returns (Ways :type "Map of /Game/ChessOfModernUnits/GameObjects/Units/Blueprints/EDirection Enum to /Game/ChessOfModernUnits/GameFramework/Player/SCalculatedWay Structure"))
  (locals (WaysForCheck :type "Array of /Game/ChessOfModernUnits/GameFramework/Player/SCalculatedWay Structure") (OutputWays :type "Map of /Game/ChessOfModernUnits/GameObjects/Units/Blueprints/EDirection Enum to /Game/ChessOfModernUnits/GameFramework/Player/SCalculatedWay Structure") (Sockets :type "Array of Name") (Moves :type "Array of /Game/ChessOfModernUnits/GameObjects/Units/Blueprints/SUnitMove Structure"))
  (`KismetArrayLibrary.Array_Add` (`local.WaysForCheck`) (make `/Game/ChessOfModernUnits/GameFramework/Player/SCalculatedWay` FieldState UnitConfig))
  (for _array_element (`local.WaysForCheck`)
    (bind (_fieldstate _unitconfig) (break `/Game/ChessOfModernUnits/GameFramework/Player/SCalculatedWay` _array_element))
    (bind (_value _returnvalue) (`BlueprintMapLibrary.Map_Find` (`local.OutputWays`) (`.Direction_56_4F2B10F847F49B1199F4DC823B142897` (break `/Game/ChessOfModernUnits/GameObjects/Units/Blueprints/SUnitConfig` _unitconfig))))
    (if (and (`/Game/ChessOfModernUnits/GameObjects/Units/Blueprints/BPFL_CoordsAndDirectionTransforms.EqualCoords` (`.Coords_47_E98C47904C4A4C6B43CCA291531B50D8` (break `/Game/ChessOfModernUnits/GameObjects/Units/Blueprints/SUnitConfig` _unitconfig)) (`local.TargetCoords`)) (or (> (break `/Game/ChessOfModernUnits/GameObjects/Units/Blueprints/SUnitTempState` (`.TempState_62_5ABFF3A34B4DD39392594A92040E2E81` (break `/Game/ChessOfModernUnits/GameObjects/Units/Blueprints/SUnitConfig` _unitconfig))) (break `/Game/ChessOfModernUnits/GameObjects/Units/Blueprints/SUnitTempState` (`.TempState_62_5ABFF3A34B4DD39392594A92040E2E81` (break `/Game/ChessOfModernUnits/GameObjects/Units/Blueprints/SUnitConfig` (`.UnitConfig_2_EAC4962249C2BC1D6D65DDB63682F041` (break `/Game/ChessOfModernUnits/GameFramework/Player/SCalculatedWay` _value)))))) (not _returnvalue)))
      (`BlueprintMapLibrary.Map_Add` (`local.OutputWays`) (`.Direction_56_4F2B10F847F49B1199F4DC823B142897` (break `/Game/ChessOfModernUnits/GameObjects/Units/Blueprints/SUnitConfig` _unitconfig)) _array_element))
    (bind (_fieldstate_2 _unitconfig_2 _moves) (break `/Game/ChessOfModernUnits/GameFramework/Player/SCalculatedWay` _array_element))
    (bind _moves_2 (`self.GetPossibleMoves` _fieldstate_2 _unitconfig_2))
    (bind _result (`BlueprintSetLibrary.Set_ToArray` _moves_2))
    (for _array_element_2 _result
      (bind (_newfieldstate _newunit _possible) (`self.ComputeOneMove` _fieldstate_2 _array_element_2 _unitconfig_2))
      (if _possible
        (bind _output_get (set `local.Moves` _moves))
        (`KismetArrayLibrary.Array_Add` _output_get _array_element_2)
        (`KismetArrayLibrary.Array_Add` (`local.WaysForCheck`) (make `/Game/ChessOfModernUnits/GameFramework/Player/SCalculatedWay` _newfieldstate _newunit _output_get)))))
  (return (`local.OutputWays`)))

(fn `ComputeMoves`
  (params (UnitCoords :type "/Game/ChessOfModernUnits/GameObjects/Field/Blueprints/SFieldCellCoords Structure") (Moves :type "Array of /Game/ChessOfModernUnits/GameObjects/Units/Blueprints/SUnitMove Structure"))
  (returns (NewFieldState :type "/Game/ChessOfModernUnits/GameObjects/Field/Blueprints/SFieldState Structure") (NewUnitConfig :type "/Game/ChessOfModernUnits/GameObjects/Units/Blueprints/SUnitConfig Structure") (Valid :type Boolean) (Possible :type Boolean))
  (locals (TempUnitConfig :type "/Game/ChessOfModernUnits/GameObjects/Units/Blueprints/SUnitConfig Structure") (TempFieldState :type "/Game/ChessOfModernUnits/GameObjects/Field/Blueprints/SFieldState Structure"))
  (bind _tempunitconfig (`local.TempUnitConfig`))
  (bind _tempfieldstate (`local.TempFieldState`))
  (bind _asbp_player_controller (cast `/Game/ChessOfModernUnits/GameFramework/Player/BP_PlayerController` (`self.GetOwner`)))
  (bind _savedfieldstate (`/Game/ChessOfModernUnits/GameFramework/Player/BP_PlayerController.SavedFieldState` _asbp_player_controller))
  (set `local.TempFieldState` _savedfieldstate)
  (bind (_value _returnvalue) (`BlueprintMapLibrary.Map_Find` (`.Units_31_8194BC274A1D6B758B12AA93D64CC056` (break `/Game/ChessOfModernUnits/GameObjects/Field/Blueprints/SFieldState` _savedfieldstate)) UnitCoords))
  (if _returnvalue
    (set `local.TempUnitConfig` _value)
    (for _array_element Moves
      (bind (_newfieldstate _newunit _possible) (`self.ComputeOneMove` _tempfieldstate _array_element _tempunitconfig))
      (if _possible
        (set `local.TempFieldState` _newfieldstate)
        (set `local.TempUnitConfig` _newunit)
        (else
          (return (struct) (struct) false false))))
    (return _tempfieldstate _tempunitconfig (not (`/Game/ChessOfModernUnits/GameFramework/Player/BPFL_CellsAndUnits.EqualFieldStates` _savedfieldstate (`local.TempFieldState`))) true)
    (else
      (return (struct) (struct) false false))))

(fn `ComputeOneMove`
  (params (FieldState :type "/Game/ChessOfModernUnits/GameObjects/Field/Blueprints/SFieldState Structure") (Move :type "/Game/ChessOfModernUnits/GameObjects/Units/Blueprints/SUnitMove Structure") (Unit :type "/Game/ChessOfModernUnits/GameObjects/Units/Blueprints/SUnitConfig Structure"))
  (returns (NewFieldState :type "/Game/ChessOfModernUnits/GameObjects/Field/Blueprints/SFieldState Structure") (NewUnit :type "/Game/ChessOfModernUnits/GameObjects/Units/Blueprints/SUnitConfig Structure") (Possible :type Boolean))
  (bind ((`Coords_47_E98C47904C4A4C6B43CCA291531B50D8` _coords) (`Alive_50_F54C53F84EFA66D3B0170BB8E9F0CD80` _alive) (`Side_59_393DC6B94AC999E7C6758C8FD57E2723` _side)) (break `/Game/ChessOfModernUnits/GameObjects/Units/Blueprints/SUnitConfig` Unit))
  (bind (_value _returnvalue) (`BlueprintMapLibrary.Map_Find` (`.Units_31_8194BC274A1D6B758B12AA93D64CC056` (break `/Game/ChessOfModernUnits/GameObjects/Field/Blueprints/SFieldState` FieldState)) _coords))
  (bind _asbp_game_state (cast `/Game/ChessOfModernUnits/GameFramework/Singletons/BP_GameState` (`GameplayStatics.GetGameState`)))
  (if (and (`/Game/ChessOfModernUnits/GameFramework/Player/BPFL_CellsAndUnits.EqualUnits` _value Unit) _returnvalue _alive (`|EnumEquality` (`/Game/ChessOfModernUnits/GameFramework/Singletons/BP_GameState.Now Move Side` _asbp_game_state) _side))
    (bind _module (`/Game/ChessOfModernUnits/GameFramework/Player/BPFL_CellsAndUnits.MakeModule` Unit (`.ActiveComponent_20_EA598D07478AB8A33D4C1F99ECAC8CF4` (break `/Game/ChessOfModernUnits/GameObjects/Units/Blueprints/SUnitMove` Move)) (`self.GetOwner`)))
    (bind (_newfieldstate _newunitconfig _possible) (`/Game/ChessOfModernUnits/GameObjects/Units/Blueprints/Modules/BP_BaseUnitModuleComponent.ComputeMove` _module (`local.FieldState`) (`local.Unit`) (`local.Move`)))
    (`self.K2_DestroyComponent` _module)
    (return _newfieldstate _newunitconfig _possible)
    (else
      (return (struct) (struct) false))))

(fn `GetPossibleMoves`
  (params (FieldState :type "/Game/ChessOfModernUnits/GameObjects/Field/Blueprints/SFieldState Structure") (UnitConfig :type "/Game/ChessOfModernUnits/GameObjects/Units/Blueprints/SUnitConfig Structure"))
  (returns (Moves :type "Set of /Game/ChessOfModernUnits/GameObjects/Units/Blueprints/SUnitMove Structure"))
  (locals (PossibleMoves :type "Set of /Game/ChessOfModernUnits/GameObjects/Units/Blueprints/SUnitMove Structure"))
  (if (`.Alive_50_F54C53F84EFA66D3B0170BB8E9F0CD80` (break `/Game/ChessOfModernUnits/GameObjects/Units/Blueprints/SUnitConfig` UnitConfig))
    (`|ExecutionSequence`
      (:`then_0`
        (bind _modules (`/Game/ChessOfModernUnits/GameFramework/Player/BPFL_CellsAndUnits.MakeAllUnitModules` UnitConfig (`self.GetOwner`)))
        (for _array_element _modules
          (bind _possiblemoves (`/Game/ChessOfModernUnits/GameObjects/Units/Blueprints/Modules/BP_BaseUnitModuleComponent.GetPossibleMoves` _array_element (`local.FieldState`) (`local.UnitConfig`)))
          (bind _keys (`BlueprintMapLibrary.Map_Keys` _possiblemoves))
          (`BlueprintSetLibrary.Set_AddItems` (`local.PossibleMoves`) _keys)
          (`self.K2_DestroyComponent` _array_element)))
      (:`then_1`
        (return (`local.PossibleMoves`))))
    (else
      (return))))