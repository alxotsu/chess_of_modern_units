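; BP_Pawn is the player's free camera pawn, with pan, zoom and orbit controls.
; Enhanced Input actions feed MoveCamera, either directly or as mouse drag, adding movement along the root's horizontal forward and right vectors.
; Tick consumes that input and offsets the root by a fixed step per frame, without delta time or sweep.
; Zoom slides the camera along local X within limits, while rotation turns the root with clamped pitch and wrapped yaw.
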(event `self.ReceiveTick`
  (params (DeltaSeconds :type "Float (single-precision)"))
  (bind _returnvalue (`self.ConsumeMovementInputVector`))
  (`SceneComponent.K2_AddWorldOffset` (`self.DefaultSceneRoot`) (* (`KismetMathLibrary.Normal` _returnvalue) 10.0) false false))

(event `EnhancedInput|/Game/ChessOfModernUnits/GameFramework/Player/Input/Actions/CameraControl/IA_ZoomCamera`
  (params (ActionValue :type "Float (double-precision)") (ElapsedSeconds :type "Float (double-precision)") (TriggeredSeconds :type "Float (double-precision)") (InputAction :type "InputAction Object Reference" :default "/Game/ChessOfModernUnits/GameFramework/Player/Input/Actions/CameraControl/IA_ZoomCamera.IA_ZoomCamera"))
  (bind _relativelocation_x (`KismetMathLibrary.BreakVector` (`SceneComponent.RelativeLocation` (`self.Camera`))))
  (:`Triggered`
    (`SceneComponent.K2_SetRelativeLocation` (`self.Camera`) (`KismetMathLibrary.MakeVector` (`KismetMathLibrary.FClamp` (+ (* ActionValue 30.0) _relativelocation_x) -1000.0 -150.0)) false false)))

(event `EnhancedInput|/Game/ChessOfModernUnits/GameFramework/Player/Input/Actions/CameraControl/IA_PlaneCamera`
  (params (ActionValue :type Boolean) (ElapsedSeconds :type "Float (double-precision)") (TriggeredSeconds :type "Float (double-precision)") (InputAction :type "InputAction Object Reference" :default "/Game/ChessOfModernUnits/GameFramework/Player/Input/Actions/CameraControl/IA_PlaneCamera.IA_PlaneCamera"))
  (:`Triggered`
    (`self.MoveCamera` (`KismetMathLibrary.MakeVector2D` (* (`self.GetInputAxisValue`) -0.5) (* (`self.GetInputAxisValue`) -0.5)))))

(event `EnhancedInput|/Game/ChessOfModernUnits/GameFramework/Player/Input/Actions/CameraControl/IA_MoveCamera`
  (params (ActionValue :type "Vector2D Structure") (ElapsedSeconds :type "Float (double-precision)") (TriggeredSeconds :type "Float (double-precision)") (InputAction :type "InputAction Object Reference" :default "/Game/ChessOfModernUnits/GameFramework/Player/Input/Actions/CameraControl/IA_MoveCamera.IA_MoveCamera"))
  (:`Triggered`
    (`self.MoveCamera` ActionValue)))

(event `EnhancedInput|/Game/ChessOfModernUnits/GameFramework/Player/Input/Actions/CameraControl/IA_RotateCamera`
  (params (ActionValue :type Boolean) (ElapsedSeconds :type "Float (double-precision)") (TriggeredSeconds :type "Float (double-precision)") (InputAction :type "InputAction Object Reference" :default "/Game/ChessOfModernUnits/GameFramework/Player/Input/Actions/CameraControl/IA_RotateCamera.IA_RotateCamera"))
  (bind _defaultsceneroot (`self.DefaultSceneRoot`))
  (bind (_returnvalue_roll _returnvalue_pitch _returnvalue_yaw) (`KismetMathLibrary.BreakRotator` (`SceneComponent.K2_GetComponentRotation` _defaultsceneroot)))
  (:`Triggered`
    (`SceneComponent.K2_SetWorldRotation` _defaultsceneroot (`KismetMathLibrary.MakeRotator` 0.0 (`KismetMathLibrary.FClamp` (+ _returnvalue_pitch (* (`self.GetInputAxisValue`) 2.0)) -89.0 -30.0) (`KismetMathLibrary.FMod` (+ _returnvalue_yaw (* (`self.GetInputAxisValue`) 3.0)) 360.0)) false false)))

(fn `MoveCamera`
  (params (Vector :type "Vector2D Structure"))
  (bind (_x _y) (`KismetMathLibrary.BreakVector2D` Vector))
  (bind _defaultsceneroot (`self.DefaultSceneRoot`))
  (`self.AddMovementInput` (+ (* (`KismetMathLibrary.Vector_Normal2D` (`SceneComponent.GetForwardVector` _defaultsceneroot)) _x) (* (`KismetMathLibrary.Vector_Normal2D` (`SceneComponent.GetRightVector` _defaultsceneroot)) _y))))

(fn `UserConstructionScript`)