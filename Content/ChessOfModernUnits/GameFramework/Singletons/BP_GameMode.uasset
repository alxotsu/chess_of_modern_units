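; Game mode for a turn-based, two-sided unit board game, running player setup, turn flow and victory checks.
; Joining players get sides, and controllers receive PreMove on each join or move end.
; VictoryCheck decides win, draw or side switch from surviving units, command-antenna units and their presence on base cells.
; With one player, that player's side follows the active side; PrepareFieldState adds base rows beyond both Y edges.
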(event `self.ReceiveBeginPlay`
  (add `self.onEndMove` (delegate `EndMove`)))

(event `EndMove`
  (`|ExecutionSequence`
    (:`then_0`
      (bind (_newstatename _activeside) (`self.VictoryCheck`))
      (bind _asbp_game_state (cast `/Game/ChessOfModernUnits/GameFramework/Singletons/BP_GameState` (`GameplayStatics.GetGameState`)))
      (bind _output_get (set `/Game/ChessOfModernUnits/GameFramework/Singletons/BP_GameState.StateName` _newstatename _asbp_game_state))
      (set `/Game/ChessOfModernUnits/GameFramework/Singletons/BP_GameState.Now Move Side` _activeside _asbp_game_state)
      (bind _outactors (`GameplayStatics.GetAllActorsOfClass` "/Game/ChessOfModernUnits/GameFramework/Player/BP_PlayerController.BP_PlayerController_C"))
      (for _array_element _outactors
        (`/Game/ChessOfModernUnits/GameFramework/Player/BP_PlayerController.PreMove` _array_element _output_get)))
    (:`then_1`
      (if (== (`self.NumPlayers`) 1)
        (bind _asbp_player_state (cast `/Game/ChessOfModernUnits/GameFramework/Player/BP_PlayerState` (`GameplayStatics.GetPlayerState` 0)))
        (bind _asbp_game_state_2 (cast `/Game/ChessOfModernUnits/GameFramework/Singletons/BP_GameState` (`GameplayStatics.GetGameState`)))
        (set `/Game/ChessOfModernUnits/GameFramework/Player/BP_PlayerState.side` (`/Game/ChessOfModernUnits/GameFramework/Singletons/BP_GameState.Now Move Side` _asbp_game_state_2) _asbp_player_state)))))

(event `self.HandleStartingNewPlayer`
  (params (NewPlayer :type "PlayerController Object Reference"))
  (bind _numplayers (`self.NumPlayers`))
  (`parent.HandleStartingNewPlayer` NewPlayer)
  (cast `/Game/ChessOfModernUnits/GameFramework/Player/BP_PlayerController` NewPlayer)
  (bind _asbp_player_state (cast `/Game/ChessOfModernUnits/GameFramework/Player/BP_PlayerState` (`Controller.PlayerState` NewPlayer)))
  (set `/Game/ChessOfModernUnits/GameFramework/Player/BP_PlayerState.side` (select `int` (`self.NumPlayers`) :`0` "NewEnumerator1" :`1` "NewEnumerator0" :!type "/Game/ChessOfModernUnits/GameFramework/Player/EPlayerSide Enum") _asbp_player_state)
  (`/Engine/EditorBlueprintResources/StandardMacros.IncrementInt` _numplayers
    (:`  `
      (bind _asbp_game_instance (cast `/Game/ChessOfModernUnits/Core/BP_GameInstance` (`GameplayStatics.GetGameInstance`)))
      (bind _asbp_game_state (cast `/Game/ChessOfModernUnits/GameFramework/Singletons/BP_GameState` (`GameplayStatics.GetGameState`)))
      (bind _output_get (set `/Game/ChessOfModernUnits/GameFramework/Singletons/BP_GameState.StateName` (select `bool` (<= (`/Game/ChessOfModernUnits/Core/BP_GameInstance.RequiredPlayers` _asbp_game_instance) _numplayers) :`false` "Preparing" :`true` "ReadyToMove" :!type "Name") _asbp_game_state))
      (bind _outactors (`GameplayStatics.GetAllActorsOfClass` "/Game/ChessOfModernUnits/GameFramework/Player/BP_PlayerController.BP_PlayerController_C"))
      (for _array_element _outactors
        (`/Game/ChessOfModernUnits/GameFramework/Player/BP_PlayerController.PreMove` _array_element _output_get)))))

(fn `GetOwnerOfBaseCell`
  (params (Coords :type "/Game/ChessOfModernUnits/GameObjects/Field/Blueprints/SFieldCellCoords Structure"))
  (returns (Owner :type "/Game/ChessOfModernUnits/GameFramework/Player/EPlayerSide Enum"))
  (return (select `bool` (> Coords_YCoord_12_230624BA45D1462C62A7DA860B56371E 0) :`false` "NewEnumerator1" :`true` "NewEnumerator0" :!type "/Game/ChessOfModernUnits/GameFramework/Player/EPlayerSide Enum")))

(fn `PrepareFieldState`
  (params (FieldState :type "/Game/ChessOfModernUnits/GameObjects/Field/Blueprints/SFieldState Structure"))
  (returns (PreparedFieldState :type "/Game/ChessOfModernUnits/GameObjects/Field/Blueprints/SFieldState Structure"))
  (bind (_sizex _sizey _landscapes _units) (break `/Game/ChessOfModernUnits/GameObjects/Field/Blueprints/SFieldState` FieldState))
  (for _index (range _sizex)
    (`BlueprintMapLibrary.Map_Add` _landscapes (make `/Game/ChessOfModernUnits/GameObjects/Field/Blueprints/SFieldCellCoords` _index -1) "NewEnumerator3")
    (`BlueprintMapLibrary.Map_Add` _landscapes (make `/Game/ChessOfModernUnits/GameObjects/Field/Blueprints/SFieldCellCoords` _index _sizey) "NewEnumerator3"))
  (return (make `/Game/ChessOfModernUnits/GameObjects/Field/Blueprints/SFieldState` _sizex _sizey _landscapes _units)))

(fn `UserConstructionScript`)

(fn `VictoryCheck`
  (returns (NewStateName :type Name) (ActiveSide :type "/Game/ChessOfModernUnits/GameFramework/Player/EPlayerSide Enum"))
  (locals (HasAliveUnits :type "Map of /Game/ChessOfModernUnits/GameFramework/Player/EPlayerSide Enum to Boolean") (HasAliveComUnits :type "Map of /Game/ChessOfModernUnits/GameFramework/Player/EPlayerSide Enum to Boolean") (HasComUnits :type "Map of /Game/ChessOfModernUnits/GameFramework/Player/EPlayerSide Enum to Boolean") (HasComUnitsOnBase :type "Map of /Game/ChessOfModernUnits/GameFramework/Player/EPlayerSide Enum to Boolean"))
  (bind _hasaliveunits (`local.HasAliveUnits`))
  (bind _hasalivecomunits (`local.HasAliveComUnits`))
  (bind _hascomunits (`local.HasComUnits`))
  (bind _hascomunitsonbase (`local.HasComUnitsOnBase`))
  (bind _returnvalue (or (not (`BlueprintMapLibrary.Map_Find` _hasaliveunits "NewEnumerator1")) (and (not (`BlueprintMapLibrary.Map_Find` _hasalivecomunits "NewEnumerator1")) (`BlueprintMapLibrary.Map_Find` _hascomunits "NewEnumerator1")) (`BlueprintMapLibrary.Map_Find` _hascomunitsonbase "NewEnumerator0")))
  (bind _returnvalue_2 (or (not (`BlueprintMapLibrary.Map_Find` _hasaliveunits "NewEnumerator0")) (and (not (`BlueprintMapLibrary.Map_Find` _hasalivecomunits "NewEnumerator0")) (`BlueprintMapLibrary.Map_Find` _hascomunits "NewEnumerator0")) (`BlueprintMapLibrary.Map_Find` _hascomunitsonbase "NewEnumerator1")))
  (`|ExecutionSequence`
    (:`then_0`
      (bind _fieldstate (`/Game/ChessOfModernUnits/GameFramework/Player/BPFL_CellsAndUnits.GetFieldConfigFromWorld`))
      (bind (_sizex _sizey _landscapes _units) (break `/Game/ChessOfModernUnits/GameObjects/Field/Blueprints/SFieldState` _fieldstate))
      (bind _values (`BlueprintMapLibrary.Map_Values` _units))
      (for _array_element _values
        (bind ((`ModuleOnSockets_65_93C0F6A14F5C249A946557A0ACBCDE35` _moduleonsockets) (`Coords_47_E98C47904C4A4C6B43CCA291531B50D8` _coords) (`Alive_50_F54C53F84EFA66D3B0170BB8E9F0CD80` _alive) (`Side_59_393DC6B94AC999E7C6758C8FD57E2723` _side)) (break `/Game/ChessOfModernUnits/GameObjects/Units/Blueprints/SUnitConfig` _array_element))
        (if _alive
          (`BlueprintMapLibrary.Map_Add` (`local.HasAliveUnits`) _side true)
          (bind _values_2 (`BlueprintMapLibrary.Map_Values` _moduleonsockets))
          (if (`KismetArrayLibrary.Array_Contains` _values_2 "ComTankAntenne")
            (`BlueprintMapLibrary.Map_Add` (`local.HasAliveComUnits`) _side true)
            (`BlueprintMapLibrary.Map_Add` (`local.HasComUnits`) _side true :!label _label)
            (if (`|EnumEquality` (`BlueprintMapLibrary.Map_Find` _landscapes _coords) "NewEnumerator3")
              (`BlueprintMapLibrary.Map_Add` (`local.HasComUnitsOnBase`) _side true)))
          (else
            (bind _values_3 (`BlueprintMapLibrary.Map_Values` _moduleonsockets))
            (if (`KismetArrayLibrary.Array_Contains` _values_3 "ComTankAntenne")
              (goto _label))))))
    (:`then_1`
      (if (and _returnvalue_2 _returnvalue)
        (return "Draft" "NewEnumerator1")
        (elif _returnvalue_2
          (return "Win" "NewEnumerator1")
          (elif _returnvalue
            (return "Win" "NewEnumerator0")
            (else
              (bind _asbp_game_state (cast `/Game/ChessOfModernUnits/GameFramework/Singletons/BP_GameState` (`GameplayStatics.GetGameState`)))
              (return "ReadyToMove" (select `/Game/ChessOfModernUnits/GameFramework/Player/EPlayerSide` (`/Game/ChessOfModernUnits/GameFramework/Singletons/BP_GameState.Now Move Side` _asbp_game_state) :`NewEnumerator0` "NewEnumerator1" :`NewEnumerator1` "NewEnumerator0" :!type "/Game/ChessOfModernUnits/GameFramework/Player/EPlayerSide Enum")))))))))