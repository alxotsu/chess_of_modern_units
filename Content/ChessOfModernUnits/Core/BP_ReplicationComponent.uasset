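; BP_ReplicationComponent is a component that passes a unit config struct from authority to remote through a JSON string.
; ReplicateUnitConfig wraps the JsonReplication macro, returning the given config on authority and the decoded value on remote.
; The macro branches on authority: the authority side serializes the struct into SavedJson, while the remote side parses that string and reads a field from it with an empty field name.
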(fn `ReplicateUnitConfig`
  (params (Config :type "/Game/ChessOfModernUnits/GameObjects/Units/Blueprints/SUnitConfig Structure"))
  (returns (ReplConfig :type "/Game/ChessOfModernUnits/GameObjects/Units/Blueprints/SUnitConfig Structure"))
  (bind _value (`self.JsonReplication` Config)
    (:`Authority`
      (return Config))
    (:`Remote`
      (return _value))))