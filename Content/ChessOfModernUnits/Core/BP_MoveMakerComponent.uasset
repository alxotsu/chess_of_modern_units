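; Component that finds, validates and executes unit moves on the chess-style field, delegating rules to one spawned component per unit variant.
; Main-component search expands simulated field states, keeping the move list with most remaining move points per direction and coords; socket components list single-step moves.
; ComputeMoves simulates move sequences on a field copy.
; MakeMoves applies them to the non-hologram unit, then saves field state to all player controllers.
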(event `self.ReceiveBeginPlay`
  (bind _enumvalue (foreach `/Game/ChessOfModernUnits/Units/Components/EUnitComponentVariant` false)
    (:`LoopBody`
      (bind _returnvalue (`|AddComponentByClass` (`self.GetOwner`) (`BlueprintMapLibrary.Map_Find` (`self.UnitComponentsClasses`) _enumvalue) _enumvalue))
      (`BlueprintMapLibrary.Map_Add` (`self.UnitComponents`) (`/Game/ChessOfModernUnits/Units/Components/BP_BaseUnitComponent.Variant` _returnvalue) _returnvalue))))

(event `self.ReceiveEndPlay`
  (params (EndPlayReason :type "EEndPlayReason Enum" :default "Destroyed"))
  (bind _values (`BlueprintMapLibrary.Map_Values` (`self.UnitComponents`)))
  (`self.K2_DestroyComponent` _values))

(event `MakeMoves`
  (params (Coords :type "/Game/ChessOfModernUnits/Placebles/SFieldCellCoords Structure") (Moves :type "Array of /Game/ChessOfModernUnits/Units/SUnitMove Structure (by ref)"))
  (bind _outactors (`GameplayStatics.GetAllActorsOfClass` "/Game/ChessOfModernUnits/Units/BP_Unit.BP_Unit_C"))
  (for _array_element _outactors
    (cast `/Game/ChessOfModernUnits/Units/BP_UnitHologram` _array_element
      (:`CastFailed`
        (if (`/Game/ChessOfModernUnits/Core/BPFL_CustomUtilits.EqualCoords` (`.Coords_7_9C7BED8F4B2205EF8B5C87A1962D4680` (break `/Game/ChessOfModernUnits/Units/SUnitConfig` (`/Game/ChessOfModernUnits/Units/BP_Unit.Config` _array_element))) Coords)
          (`self.MakeMovesF` _array_element Moves)
          (break)))))
  (bind _field (`/Game/ChessOfModernUnits/Core/BPFL_CustomUtilits.GetFieldConfigFromWorld`))
  (bind _outactors_2 (`GameplayStatics.GetAllActorsOfClass` "/Game/ChessOfModernUnits/Controls/OneVsOne/BP_PlayerController.BP_PlayerController_C"))
  (for _array_element_2 _outactors_2
    (set `/Game/ChessOfModernUnits/Controls/OneVsOne/BP_PlayerController.SavedFieldState` _field _array_element_2)))

(fn `ComputeMoves`
  (params (Field :type "/Game/ChessOfModernUnits/Placebles/SFieldConfig Structure") (Coords :type "/Game/ChessOfModernUnits/Placebles/SFieldCellCoords Structure") (Moves :type "Array of /Game/ChessOfModernUnits/Units/SUnitMove Structure"))
  (returns (Possible :type Boolean) (Valid :type Boolean) (FieldOutput :type "/Game/ChessOfModernUnits/Placebles/SFieldConfig Structure") (CoordsOutput :type "/Game/ChessOfModernUnits/Placebles/SFieldCellCoords Structure"))
  (locals (TempField :type "/Game/ChessOfModernUnits/Placebles/SFieldConfig Structure") (TempCoords :type "/Game/ChessOfModernUnits/Placebles/SFieldCellCoords Structure"))
  (bind (_unit _found) (`/Game/ChessOfModernUnits/Core/BPFL_CustomUtilits.GetUnitFromField` Field Coords))
  (set `local.TempField` Field)
  (set `local.TempCoords` Coords)
  (if (and (`.Alive_1_4876116A47F2527D46E553BF84858816` (break `/Game/ChessOfModernUnits/Units/SUnitConfig` _unit)) _found)
    (for _array_element Moves
      (bind (_component _found_2) (`self.GetUnitComponent` (`/Game/ChessOfModernUnits/Core/BPFL_CustomUtilits.GetUnitFromField` (`local.TempField`) (`local.TempCoords`)) (`.ActiveComponent_20_EA598D07478AB8A33D4C1F99ECAC8CF4` (break `/Game/ChessOfModernUnits/Units/SUnitMove` _array_element))))
      (if _found_2
        (bind (_possible _fieldoutput _coordsoutput) (`/Game/ChessOfModernUnits/Units/Components/BP_BaseUnitComponent.ComputeMove` _component (`local.TempField`) (`local.TempCoords`) _array_element))
        (if _possible
          (set `local.TempField` _fieldoutput)
          (set `local.TempCoords` _coordsoutput)
          (else
            (return false false)))
        (else
          (return false false))))
    (return true (`KismetArrayLibrary.Array_IsNotEmpty` (`local.Moves`)) (`local.TempField`) (`local.TempCoords`))
    (else
      (return false false))))

(fn `GetPossibleMovesViaMainComponent`
  (params (Field :type "/Game/ChessOfModernUnits/Placebles/SFieldConfig Structure") (Coords :type "/Game/ChessOfModernUnits/Placebles/SFieldCellCoords Structure"))
  (returns (PossibleMoves :type "Map of /Game/ChessOfModernUnits/Controls/OneVsOne/SDirectonAndCoords Structure to /Game/ChessOfModernUnits/Controls/OneVsOne/SMoveList Structure"))
  (locals (OutputStruct :type "Map of /Game/ChessOfModernUnits/Controls/OneVsOne/SDirectonAndCoords Structure to /Game/ChessOfModernUnits/Controls/OneVsOne/SMoveList Structure") (Metrics :type "Map of /Game/ChessOfModernUnits/Controls/OneVsOne/SDirectonAndCoords Structure to Integer") (Nodes :type "Array of /Game/ChessOfModernUnits/Controls/OneVsOne/SMainComponentMoveMakerNode Structure") (TempMovesArray :type "Array of /Game/ChessOfModernUnits/Units/SUnitMove Structure"))
  (bind _nodes (`local.Nodes`))
  (if (`.Found` (`/Game/ChessOfModernUnits/Core/BPFL_CustomUtilits.GetUnitFromField` Field Coords))
    (`KismetArrayLibrary.Array_Add` _nodes (make `/Game/ChessOfModernUnits/Controls/OneVsOne/SMainComponentMoveMakerNode` Field Coords))
    (for _array_element _nodes
      (bind (_field _coord _moves) (break `/Game/ChessOfModernUnits/Controls/OneVsOne/SMainComponentMoveMakerNode` _array_element))
      (bind _moves_2 (`/Game/ChessOfModernUnits/Units/Components/BP_BaseUnitComponent.GetPossibleMoves` (`self.GetUnitComponent` (`/Game/ChessOfModernUnits/Core/BPFL_CustomUtilits.GetUnitFromField` _field _coord)) "Main" _field _coord))
      (bind _keys (`BlueprintMapLibrary.Map_Keys` _moves_2))
      (for _array_element_2 _keys
        (bind _output_get (set `local.TempMovesArray` _moves))
        (`KismetArrayLibrary.Array_Add` _output_get _array_element_2)
        (bind (_field_2 _coords) (break `/Game/ChessOfModernUnits/Units/Components/SPossibleMoveResult` (`BlueprintMapLibrary.Map_Find` _moves_2 _array_element_2)))
        (`KismetArrayLibrary.Array_Add` (`local.Nodes`) (make `/Game/ChessOfModernUnits/Controls/OneVsOne/SMainComponentMoveMakerNode` _field_2 _coords _output_get))
        (bind ((`MovePoints_5_70E1D9294A119D81C594699875F94696` _movepoints) (`Direction_8_21FECD5E4D1EA9D2C82B07BD2D049BC7` _direction)) (break `/Game/ChessOfModernUnits/Units/Components/SUnitComponentConfig` (`.MainComponent_20_960460F54E1FCEC2EF6C488D79BB28EF` (break `/Game/ChessOfModernUnits/Units/SUnitConfig` (`/Game/ChessOfModernUnits/Core/BPFL_CustomUtilits.GetUnitFromField` _field_2 _coords)))))
        (bind _sdirectonandcoords (make `/Game/ChessOfModernUnits/Controls/OneVsOne/SDirectonAndCoords` _direction _coords))
        (bind (_value _returnvalue) (`BlueprintMapLibrary.Map_Find` (`local.Metrics`) _sdirectonandcoords))
        (if (< (select `bool` _returnvalue :`false` -1 :`true` _value) _movepoints)
          (`BlueprintMapLibrary.Map_Add` (`local.Metrics`) _sdirectonandcoords _movepoints)
          (`BlueprintMapLibrary.Map_Add` (`local.OutputStruct`) _sdirectonandcoords (make `/Game/ChessOfModernUnits/Controls/OneVsOne/SMoveList` (`local.TempMovesArray`))))))
    (return (`local.OutputStruct`))))

(fn `GetPossibleMovesViaSocketComponents`
  (params (Field :type "/Game/ChessOfModernUnits/Placebles/SFieldConfig Structure") (Coords :type "/Game/ChessOfModernUnits/Placebles/SFieldCellCoords Structure"))
  (returns (PossibleMoves :type "Map of Name to /Game/ChessOfModernUnits/Controls/OneVsOne/SMoveList Structure"))
  (locals (OutputStruct :type "Map of Name to /Game/ChessOfModernUnits/Controls/OneVsOne/SMoveList Structure"))
  (bind _value (`BlueprintMapLibrary.Map_Find` (`.Units_32_8194BC274A1D6B758B12AA93D64CC056` (break `/Game/ChessOfModernUnits/Placebles/SFieldConfig` Field)) Coords))
  (bind _keys (`BlueprintMapLibrary.Map_Keys` (`.SocketComponents_19_0467C64B42DB044005745F8E30DB9361` (break `/Game/ChessOfModernUnits/Units/SUnitConfig` _value))))
  (for _array_element _keys
    (bind _moves (`/Game/ChessOfModernUnits/Units/Components/BP_BaseUnitComponent.GetPossibleMoves` (`self.GetUnitComponent` _value _array_element) _array_element (`local.Field`) (`local.Coords`)))
    (bind _keys_2 (`BlueprintMapLibrary.Map_Keys` _moves))
    (`BlueprintMapLibrary.Map_Add` (`local.OutputStruct`) _array_element (make `/Game/ChessOfModernUnits/Controls/OneVsOne/SMoveList` _keys_2)))
  (return (`local.OutputStruct`)))

(fn `GetUnitComponent`
  (params (Unit :type "/Game/ChessOfModernUnits/Units/SUnitConfig Structure (by ref)") (Socket :type Name :default "Main"))
  (returns (Component :type "/Game/ChessOfModernUnits/Units/Components/BP_BaseUnitComponent Object Reference") (Found :type Boolean))
  (bind ((`MainComponent_20_960460F54E1FCEC2EF6C488D79BB28EF` _maincomponent) (`SocketComponents_19_0467C64B42DB044005745F8E30DB9361` _socketcomponents)) (break `/Game/ChessOfModernUnits/Units/SUnitConfig` Unit))
  (bind (_value _returnvalue) (`BlueprintMapLibrary.Map_Find` _socketcomponents Socket))
  (if (== Socket "Main")
    (return (`BlueprintMapLibrary.Map_Find` (`self.UnitComponents`) (`.VariantName_9_C81574FC4C8FC8DF9DA3DD924EEDC407` (break `/Game/ChessOfModernUnits/Units/Components/SUnitComponentConfig` _maincomponent))) true)
    (elif _returnvalue
      (return (`BlueprintMapLibrary.Map_Find` (`self.UnitComponents`) (`.VariantName_9_C81574FC4C8FC8DF9DA3DD924EEDC407` (break `/Game/ChessOfModernUnits/Units/Components/SUnitComponentConfig` _value))) true)
      (else
        (return null false)))))

(fn `MakeMovesF`
  (params (Unit :type "/Game/ChessOfModernUnits/Units/BP_Unit Object Reference") (Moves :type "Array of /Game/ChessOfModernUnits/Units/SUnitMove Structure"))
  (bind _output (`|GetArrayItem` Moves (`KismetArrayLibrary.Array_LastIndex` Moves)))
  (for _index (range (`KismetArrayLibrary.Array_LastIndex` Moves))
    (bind _output_2 (`|GetArrayItem` Moves _index))
    (`/Game/ChessOfModernUnits/Units/Components/BP_BaseUnitComponent.MakeMove` (`self.GetUnitComponent` (`/Game/ChessOfModernUnits/Units/BP_Unit.Config` Unit) (`.ActiveComponent_20_EA598D07478AB8A33D4C1F99ECAC8CF4` (break `/Game/ChessOfModernUnits/Units/SUnitMove` _output_2))) Unit _output_2 (`|GetArrayItem` Moves (+ _index 1)) true))
  (`/Game/ChessOfModernUnits/Units/Components/BP_BaseUnitComponent.MakeMove` :`self` (`self.GetUnitComponent` (`/Game/ChessOfModernUnits/Units/BP_Unit.Config` Unit) (`.ActiveComponent_20_EA598D07478AB8A33D4C1F99ECAC8CF4` (break `/Game/ChessOfModernUnits/Units/SUnitMove` _output))) :`Unit` Unit :`NowMove` _output))