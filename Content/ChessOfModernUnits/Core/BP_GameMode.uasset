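; Game mode for a two-sided, turn-based unit game that assigns joining players White or Black and waits for the required player count.
; On each move end it copies VictoryCheck's result into the game state and calls PreMove on all controllers.
; A lone player's side follows the active side.
; VictoryCheck's win, draw and turn-swap logic, based on surviving units, command units and base capture, is disconnected from its entry and never runs.
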(event `self.ReceiveBeginPlay`
  (add `self.onEndMove` (delegate `EndMove`)))

(event `EndMove`
  (`|ExecutionSequence`
    (:`then_0`
      (bind (_newstatename _activeside) (`self.VictoryCheck`))
      (bind _asbp_game_state (cast `/Game/ChessOfModernUnits/Core/BP_GameState` (`GameplayStatics.GetGameState`)))
      (set `/Game/ChessOfModernUnits/Core/BP_GameState.StateName` _newstatename _asbp_game_state)
      (set `/Game/ChessOfModernUnits/Core/BP_GameState.Now Move Side` _activeside _asbp_game_state)
      (bind _outactors (`GameplayStatics.GetAllActorsOfClass` "/Game/ChessOfModernUnits/Controls/OneVsOne/BP_PlayerController.BP_PlayerController_C"))
      (for _array_element _outactors
        (`/Game/ChessOfModernUnits/Controls/OneVsOne/BP_PlayerController.PreMove` _array_element)))
    (:`then_1`
      (if (== (`self.NumPlayers`) 1)
        (bind _asbp_player_state (cast `/Game/ChessOfModernUnits/Core/BP_PlayerState` (`GameplayStatics.GetPlayerState` 0)))
        (bind _asbp_game_state_2 (cast `/Game/ChessOfModernUnits/Core/BP_GameState` (`GameplayStatics.GetGameState`)))
        (set `/Game/ChessOfModernUnits/Core/BP_PlayerState.side` (`/Game/ChessOfModernUnits/Core/BP_GameState.Now Move Side` _asbp_game_state_2) _asbp_player_state)))))

(event `self.HandleStartingNewPlayer`
  (params (NewPlayer :type "PlayerController Object Reference"))
  (bind _numplayers (`self.NumPlayers`))
  (`parent.HandleStartingNewPlayer` NewPlayer)
  (cast `/Game/ChessOfModernUnits/Controls/OneVsOne/BP_PlayerController` NewPlayer)
  (bind _asbp_player_state (cast `/Game/ChessOfModernUnits/Core/BP_PlayerState` (`Controller.PlayerState` NewPlayer)))
  (set `/Game/ChessOfModernUnits/Core/BP_PlayerState.side` (select `int` (`self.NumPlayers`) :`0` "NewEnumerator1" :`1` "NewEnumerator0" :!type "/Game/ChessOfModernUnits/Core/EPlayerSide Enum") _asbp_player_state)
  (`/Engine/EditorBlueprintResources/StandardMacros.IncrementInt` _numplayers
    (:`  `
      (bind _asbp_game_instance (cast `/Game/ChessOfModernUnits/Core/BP_GameInstance` (`GameplayStatics.GetGameInstance`)))
      (bind _asbp_game_state (cast `/Game/ChessOfModernUnits/Core/BP_GameState` (`GameplayStatics.GetGameState`)))
      (set `/Game/ChessOfModernUnits/Core/BP_GameState.StateName` (select `bool` (<= (`/Game/ChessOfModernUnits/Core/BP_GameInstance.RequiredPlayers` _asbp_game_instance) _numplayers) :`false` "Preparing" :`true` "ReadyToMove" :!type "Name") _asbp_game_state)
      (bind _outactors (`GameplayStatics.GetAllActorsOfClass` "/Game/ChessOfModernUnits/Controls/OneVsOne/BP_PlayerController.BP_PlayerController_C"))
      (for _array_element _outactors
        (`/Game/ChessOfModernUnits/Controls/OneVsOne/BP_PlayerController.PreMove` _array_element)))))

(fn `UserConstructionScript`)

(fn `VictoryCheck`
  (returns (NewStateName :type Name) (ActiveSide :type "/Game/ChessOfModernUnits/Core/EPlayerSide Enum"))
  (locals (HasAliveUnits :type "Map of /Game/ChessOfModernUnits/Core/EPlayerSide Enum to Boolean") (HasAliveComUnits :type "Map of /Game/ChessOfModernUnits/Core/EPlayerSide Enum to Boolean") (HasComUnits :type "Map of /Game/ChessOfModernUnits/Core/EPlayerSide Enum to Boolean") (HasComUnitsOnBase :type "Map of /Game/ChessOfModernUnits/Core/EPlayerSide Enum to Boolean")))