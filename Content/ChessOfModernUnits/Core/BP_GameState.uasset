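; Game state for a chess-style unit game that, on the authority, builds the board from the field config held in the game instance.
; At BeginPlay it passes that config through the replication component, stores and spawns the result, then copies the side to move.
; SpawnFieldActors destroys existing units and cells, then spawns a checkerboard grid with landscape types, extra landscape cells outside the grid, and all configured units.
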(event `self.ReceiveBeginPlay`
  (`/Engine/EditorBlueprintResources/ActorMacros.Switch Has Authority`
    (:`Authority`
      (bind _asbp_game_instance (cast `/Game/ChessOfModernUnits/Core/BP_GameInstance` (`GameplayStatics.GetGameInstance`)))
      (`|ExecutionSequence`
        (:`then_0`
          (bind _replconfig (`/Game/ChessOfModernUnits/Core/BP_ReplicationComponent.ReplicateFieldConfig` (`self.ReplicationComponent`) (`/Game/ChessOfModernUnits/Core/BP_GameInstance.FieldState` _asbp_game_instance)))
          (bind _output_get (set `self.FieldState` _replconfig))
          (`self.SpawnFieldActors` _output_get))
        (:`then_1`
          (set `self.Now Move Side` (`/Game/ChessOfModernUnits/Core/BP_GameInstance.NowMoveSide` _asbp_game_instance)))))))

(fn `SpawnFieldActors`
  (params (SFieldState :type "/Game/ChessOfModernUnits/Placebles/SFieldConfig Structure (by ref)"))
  (locals (MaterialForCell :type "MaterialInstance Object Reference" :default "/Script/Engine.MaterialInstanceConstant'/Game/ChessOfModernUnits/Placebles/Materials/MI_CellLight.MI_CellLight'") (AdditiveCells :type "Array of /Game/ChessOfModernUnits/Placebles/SFieldCellCoords Structure"))
  (bind (_sizex _sizey _landscapes _units) (break `/Game/ChessOfModernUnits/Placebles/SFieldConfig` SFieldState))
  (bind (_sfieldstate_sizex _sfieldstate_sizey _sfieldstate_landscapes) (break `/Game/ChessOfModernUnits/Placebles/SFieldConfig` (`local.SFieldState`)))
  (bind (_sfieldstate_sizex_2 _sfieldstate_sizey_2 _sfieldstate_landscapes_2) (break `/Game/ChessOfModernUnits/Placebles/SFieldConfig` (`local.SFieldState`)))
  (bind _returnvalue (select `bool` (== "/Game/ChessOfModernUnits/Placebles/Materials/MI_CellDark.MI_CellDark" (`local.MaterialForCell`)) :`false` "/Game/ChessOfModernUnits/Placebles/Materials/MI_CellDark.MI_CellDark" :`true` "/Game/ChessOfModernUnits/Placebles/Materials/MI_CellLight.MI_CellLight" :!type "MaterialInstance Object Reference"))
  (`|ExecutionSequence`
    (:`then_0`
      (bind _outactors (`GameplayStatics.GetAllActorsOfClass` "/Game/ChessOfModernUnits/Units/BP_Unit.BP_Unit_C"))
      (for _array_element _outactors
        (`self.K2_DestroyActor` _array_element)))
    (:`then_1`
      (bind _outactors_2 (`GameplayStatics.GetAllActorsOfClass` "/Game/ChessOfModernUnits/Placebles/BP_Cell.BP_Cell_C"))
      (for _array_element_2 _outactors_2
        (`self.K2_DestroyActor` _array_element_2)))
    (:`then_2`
      (bind _keys (`BlueprintMapLibrary.Map_Keys` _landscapes))
      (set `local.AdditiveCells` _keys)
      (set `local.MaterialForCell` (select `bool` (== (mod (+ _sizex _sizey) 2) 0) :`false` "/Game/ChessOfModernUnits/Placebles/Materials/MI_CellDark.MI_CellDark" :`true` "/Game/ChessOfModernUnits/Placebles/Materials/MI_CellLight.MI_CellLight" :!type "MaterialInstance Object Reference"))
      (for _index (range _sizex)
        (if (== (mod _sizey 2) 0)
          (set `local.MaterialForCell` _returnvalue))
        (for _index_2 (range _sizey)
          (bind _output_get (set `local.MaterialForCell` _returnvalue))
          (bind _sfieldcellcoords (make `/Game/ChessOfModernUnits/Placebles/SFieldCellCoords` _index _index_2))
          (bind (_value _returnvalue_2) (`BlueprintMapLibrary.Map_Find` _sfieldstate_landscapes _sfieldcellcoords))
          (`|SpawnActorFromClass` "/Game/ChessOfModernUnits/Placebles/BP_Cell.BP_Cell_C" (`KismetMathLibrary.MakeTransform` (0.0 0.0 0.0)) "Undefined" "MultiplyWithRoot" null _sfieldcellcoords (select `bool` _returnvalue_2 :`false` "NewEnumerator0" :`true` _value) _output_get null)
          (`KismetArrayLibrary.Array_RemoveItem` (`local.AdditiveCells`) _sfieldcellcoords)))
      (for _array_element_3 (`local.AdditiveCells`)
        (`|SpawnActorFromClass` "/Game/ChessOfModernUnits/Placebles/BP_Cell.BP_Cell_C" (`KismetMathLibrary.MakeTransform` (0.0 0.0 0.0)) "Undefined" "MultiplyWithRoot" null _array_element_3 (`BlueprintMapLibrary.Map_Find` _sfieldstate_landscapes_2 _array_element_3) (`local.MaterialForCell`) null)))
    (:`then_3`
      (bind _values (`BlueprintMapLibrary.Map_Values` _units))
      (for _array_element_4 _values
        (`|SpawnActorFromClass` "/Game/ChessOfModernUnits/Units/BP_Unit.BP_Unit_C" (`KismetMathLibrary.MakeTransform` (0.0 0.0 0.0)) "Undefined" "MultiplyWithRoot" null _array_element_4 null)))))

(fn `UserConstructionScript`)