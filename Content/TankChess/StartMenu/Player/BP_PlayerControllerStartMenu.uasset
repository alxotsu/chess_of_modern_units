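; Player controller for the TankChess start menu that creates and shows the menu widget.
; On BeginPlay it adds WBP_StartMenu to the viewport and shows the mouse cursor.
; The TogglePause input switches the widget's panels, returning to the main panel when it is hidden and otherwise activating the end-game panel.
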(event `self.ReceiveBeginPlay`
  (bind _returnvalue (`|GenericCreateObject` "/Game/TankChess/StartMenu/Player/UI/WBP_StartMenu.WBP_StartMenu_C"))
  (`UserWidget.AddToViewport` _returnvalue 0)
  (set `self.bShowMouseCursor` true))

(event `InputAction|TogglePause`
  (params (Key :type "Key Structure"))
  (:`Pressed`
    (if (`|EnumEquality` (`Widget.Visibility` (`/Game/TankChess/StartMenu/Player/UI/WBP_StartMenu.MainPanel` (stale `self.ReceiveBeginPlay` _returnvalue))) "Hidden")
      (`/Game/TankChess/StartMenu/Player/UI/WBP_StartMenu.ActivatePanel` (stale `self.ReceiveBeginPlay` _returnvalue) (`/Game/TankChess/StartMenu/Player/UI/WBP_StartMenu.MainPanel` (stale `self.ReceiveBeginPlay` _returnvalue)))
      (else
        (`/Game/TankChess/StartMenu/Player/UI/WBP_StartMenu.ActivatePanel` (stale `self.ReceiveBeginPlay` _returnvalue) (`/Game/TankChess/StartMenu/Player/UI/WBP_StartMenu.EndGamePanel` (stale `self.ReceiveBeginPlay` _returnvalue)))))))

(fn `UserConstructionScript`)