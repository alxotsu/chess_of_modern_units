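; Game state Blueprint for TankChess that holds the board and the side whose turn it is.
; Setting a state struct spawns a BP_Field at the origin if none exists, pushes the state into it, and stores the move side.
; Reading the state rebuilds the struct from the field's size, landscapes and tanks plus the stored side.
; It also exposes cell lookup by coordinates and a getter and setter for the moving side.
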(event `/Game/TankChess/Game/BPI_GsmeStateMain.SetGameState`
  (params (GameState :type "/Game/TankChess/Core/S_GameState Structure"))
  (`/Engine/EditorBlueprintResources/StandardMacros.IsValid` (`self.Field`)
    (:`Is Valid`
      _)
    (:`Is Not Valid`
      (bind _returnvalue (`|SpawnActorFromClass` "/Game/TankChess/Game/Field/Blueprints/BP_Field.BP_Field_C" (`KismetMathLibrary.MakeTransform` (0.0 0.0 0.0)) "Undefined" "MultiplyWithRoot" null null))
      (set `self.Field` _returnvalue)))
  (`/Game/TankChess/Game/Field/Blueprints/BP_Field.SetFieldState` (`self.Field`) GameState)
  (`self.SetPlayerSide` (`.MoveSide_28_7C4C6FBA485726C6C95D1795E9C3FBD2` (break `/Game/TankChess/Core/S_GameState` GameState))))

(fn `GetCell`
  (params (Coords :type "/Game/TankChess/Game/Field/Blueprints/SFieldCellCoords Structure"))
  (returns (Cell :type "/Game/TankChess/Game/Field/Blueprints/BP_Cell Object Reference") (Find :type Boolean))
  (bind (_value _returnvalue) (`BlueprintMapLibrary.Map_Find` (`/Game/TankChess/Game/Field/Blueprints/BP_Field.Cells` (`self.Field`)) Coords))
  (return _value _returnvalue))

(fn `GetGameStateStruct`
  (returns (GameState :type "/Game/TankChess/Core/S_GameState Structure"))
  (bind (_fieldsizex _fieldsizey _fieldlandscapes _fieldtanks) (break `/Game/TankChess/Core/S_GameState` (`/Game/TankChess/Game/Field/Blueprints/BP_Field.GetFieldState` (`self.Field`))))
  (return (make `/Game/TankChess/Core/S_GameState` _fieldsizex _fieldsizey _fieldlandscapes _fieldtanks (`self.NowMoveSide`))))

(fn `GetGameStateStructni`
  (returns (State :type "/Game/TankChess/Core/S_GameState Structure"))
  (locals (landscapes :type "Map of /Game/TankChess/Game/Field/Blueprints/SFieldCellCoords Structure to /Game/TankChess/Game/Field/Blueprints/ELandscapeType Enum") (TankConfigs :type "Array of /Game/TankChess/Game/Units/Tanks/Blueprints/STankConfig Structure"))
  (bind (_fieldsizex _fieldsizey _fieldlandscapes _fieldtanks) (break `/Game/TankChess/Core/S_GameState` (`/Game/TankChess/Game/Field/Blueprints/BP_Field.GetFieldState` (`self.Field`))))
  (return (make `/Game/TankChess/Core/S_GameState` _fieldsizex _fieldsizey _fieldlandscapes _fieldtanks (`self.NowMoveSide`))))

(fn `GetPlayerSide`
  (returns (PlayerSide :type "/Game/TankChess/Game/Player/EPlayerSide Enum"))
  (return (`self.NowMoveSide`)))

(fn `SetGameStateni`
  (params (GameState :type "/Game/TankChess/Core/S_GameState Structure"))
  (locals (MaterialForCell :type "MaterialInstance Object Reference"))
  (`/Engine/EditorBlueprintResources/StandardMacros.IsValid` (`self.Field`)
    (:`Is Valid`
      _)
    (:`Is Not Valid`
      (bind _returnvalue (`|SpawnActorFromClass` "/Game/TankChess/Game/Field/Blueprints/BP_Field.BP_Field_C" (`KismetMathLibrary.MakeTransform` (0.0 0.0 0.0)) "Undefined" "MultiplyWithRoot" null null))
      (set `self.Field` _returnvalue)))
  (`/Game/TankChess/Game/Field/Blueprints/BP_Field.SetFieldState` (`self.Field`) GameState)
  (set `self.NowMoveSide` (`.MoveSide_28_7C4C6FBA485726C6C95D1795E9C3FBD2` (break `/Game/TankChess/Core/S_GameState` GameState))))

(fn `SetPlayerSide`
  (params (PlayerSide :type "/Game/TankChess/Game/Player/EPlayerSide Enum" :default "NewEnumerator0"))
  (returns (Output :type "/Game/TankChess/Game/Player/EPlayerSide Enum"))
  (bind _output_get (set `self.NowMoveSide` PlayerSide))
  (return _output_get))

(fn `UserConstructionScript`)