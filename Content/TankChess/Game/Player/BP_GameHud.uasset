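; Player HUD for the tank chess game that previews moves and shots with colored hologram tanks and drives the tank control widget.
; VisualizeHolograms rebuilds holograms for the selected tank, other tanks and Tower weapon targets, tinted by side or shot result.
; MakeHologram reuses any hologram at the same coordinates, and GetControlWidget creates the widget on demand.
; OpenWayCalculator sends paths from the selected hologram's movement component to that widget.
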(event `/Game/TankChess/Game/Player/BPI_GameHud.OpenWayCalculator`
  (params (DestinationCoords :type "/Game/TankChess/Game/Field/Blueprints/SFieldCellCoords Structure"))
  (bind _asbp_base_movement_component (cast `/Game/TankChess/Game/Units/UnitComponents/Blueprints/MovementComponents/BP_BaseMovementComponent` (`/Game/TankChess/Game/Units/Tanks/Blueprints/BP_UnitComponentManagerComponent.GetComponentBySocket` (`/Game/TankChess/Game/Units/Tanks/Blueprints/BP_BaseTank.ComponentManager` (`self.SelectedTankHologram`)) "None")))
  (bind _ways (`/Game/TankChess/Game/Units/UnitComponents/Blueprints/MovementComponents/BP_BaseMovementComponent.CalculateWaysForCoord` _asbp_base_movement_component DestinationCoords (`self.SelectedConfig`) (`self.OtherConfigs`)))
  (bind _foundwidgets (`WidgetBlueprintLibrary.GetAllWidgetsOfClass` "/Game/TankChess/Game/Player/UI/WBP_TankControl.WBP_TankControl_C"))
  (`/Game/TankChess/Game/Player/UI/WBP_TankControl.OpenMoveCalculator` (`|GetArrayItem` _foundwidgets) _ways false))

(event `/Game/TankChess/Game/Player/BPI_GameHud.VisualizeHolograms`
  (params (Moves :type "Array of /Game/TankChess/Game/Units/Tanks/Blueprints/STankMove Structure (by ref)") (SelectedTankConfigs :type "Array of /Game/TankChess/Game/Units/Tanks/Blueprints/STankConfig Structure (by ref)") (OtherTanksConfigs :type "Map of /Game/TankChess/Game/Units/Tanks/Blueprints/BP_BaseTank Object Reference to /Game/TankChess/Game/Units/Tanks/Blueprints/STankConfig Structure") (Valid :type Boolean))
  (`|ExecutionSequence`
    (:`then_0`
      (bind _result (`BlueprintSetLibrary.Set_ToArray` (`self.Holograms`)))
      (for _array_element _result
        (`self.K2_DestroyActor` _array_element))
      (`BlueprintSetLibrary.Set_Clear` (`self.Holograms`)))
    (:`then_1`
      (bind _output_get (set `self.SelectedConfig` (`|GetArrayItem` SelectedTankConfigs (- (`KismetArrayLibrary.Array_Length` SelectedTankConfigs) 1))))
      (bind _hologram (`self.MakeHologram` _output_get (struct :`G` 1.0 :`A` 0.8)))
      (set `self.SelectedTankHologram` _hologram))
    (:`then_2`
      (bind _controlwidget (`self.getControlWidget`))
      (`/Game/TankChess/Game/Player/UI/WBP_TankControl.SetupWidget` _controlwidget (`self.SelectedConfig`) Valid (`KismetArrayLibrary.Array_IsNotEmpty` Moves)))
    (:`then_3`
      (bind _output_get_2 (set `self.OtherConfigs` OtherTanksConfigs))
      (bind _values (`BlueprintMapLibrary.Map_Values` _output_get_2))
      (for _array_element_2 _values
        (`self.MakeHologram` _array_element_2 (select `bool` (`|EnumEquality` (`.Side_8_19DF35D449730F8EA57E838ADEFA2C2E` (break `/Game/TankChess/Game/Units/Tanks/Blueprints/STankConfig` _array_element_2)) (`.Side_8_19DF35D449730F8EA57E838ADEFA2C2E` (break `/Game/TankChess/Game/Units/Tanks/Blueprints/STankConfig` (`self.SelectedConfig`)))) :`false` (struct :`R` 1.0 :`A` 0.8) :`true` (struct :`G` 1.0 :`A` 0.8) :!type "LinearColor Structure") true)))
    (:`then_4`
      (bind _socket (`self.GetSelectedComponent`))
      (if (`BlueprintMapLibrary.Map_Find` (`.CanUse_23_BE99ED37467B2319636ED0A69AB3D10F` (break `/Game/TankChess/Game/Units/Tanks/Blueprints/STankTempState` (`.TempState_34_C934DA7A4C1FCB64CCCC299CC61576E1` (break `/Game/TankChess/Game/Units/Tanks/Blueprints/STankConfig` (`self.SelectedConfig`))))) _socket)
        (bind _asbp_base_weapon_component (cast `/Game/TankChess/Game/Units/UnitComponents/Blueprints/WeaponComponents/BP_BaseWeaponComponent` (`/Game/TankChess/Game/Units/Tanks/Blueprints/BP_UnitComponentManagerComponent.GetComponentBySocket` (`/Game/TankChess/Game/Units/Tanks/Blueprints/BP_BaseTank.ComponentManager` (`self.SelectedTankHologram`)) _socket)))
        (bind (_targets _yourconfigaftershot) (`/Game/TankChess/Game/Units/UnitComponents/Blueprints/WeaponComponents/BP_BaseWeaponComponent.GetTargetsList` _asbp_base_weapon_component (`/Game/TankChess/Game/Units/Tanks/Blueprints/BP_BaseTank.GetConfig` (`self.SelectedTankHologram`)) OtherTanksConfigs))
        (bind _asbp_main_player_controller (cast `/Game/TankChess/Game/Player/BP_MainPlayerController` (`self.GetOwningPlayerController` self)))
        (bind _keys (`BlueprintMapLibrary.Map_Keys` _targets))
        (for _array_element_3 _keys
          (bind _value (`BlueprintMapLibrary.Map_Find` _targets _array_element_3))
          (`self.MakeHologram` _value (select `bool` (`.ReturnValue` (`BlueprintMapLibrary.Map_Find` _yourconfigaftershot _array_element_3)) :`false` (struct :`R` 1.0 :`G` 1.0 :`A` 0.8) :`true` (select `bool` (`|EnumEquality` (`.Side_8_19DF35D449730F8EA57E838ADEFA2C2E` (break `/Game/TankChess/Game/Units/Tanks/Blueprints/STankConfig` _value)) (`/Game/TankChess/Game/Player/BP_MainPlayerController.Side` _asbp_main_player_controller)) :`false` (struct :`R` 1.0 :`A` 0.8) :`true` (struct :`G` 1.0 :`A` 0.8) :!type "LinearColor Structure"))))))))

(event `/Game/TankChess/Game/Player/BPI_GameHud.ClearAllHolograms`
  (bind _result (`BlueprintSetLibrary.Set_ToArray` (`self.Holograms`)))
  (for _array_element _result
    (`self.K2_DestroyActor` _array_element))
  (`BlueprintSetLibrary.Set_Clear` (`self.Holograms`))
  (bind _controlwidget (`self.getControlWidget`))
  (`Widget.RemoveFromParent` _controlwidget))

(fn `getControlWidget`
  (returns (controlWidget :type "/Game/TankChess/Game/Player/UI/WBP_TankControl Object Reference"))
  (bind _foundwidgets (`WidgetBlueprintLibrary.GetAllWidgetsOfClass` "/Game/TankChess/Game/Player/UI/WBP_TankControl.WBP_TankControl_C"))
  (if (`KismetArrayLibrary.Array_IsEmpty` _foundwidgets)
    (bind _returnvalue (`|CreateWidget` "/Game/TankChess/Game/Player/UI/WBP_TankControl.WBP_TankControl_C"))
    (`UserWidget.AddToViewport` _returnvalue 0)
    (return _returnvalue)
    (else
      (return (`|GetArrayItem` _foundwidgets)))))

(fn `GetSelectedComponent`
  (returns (Socket :type Name))
  (return "Tower"))

(fn `MakeHologram`
  (params (Config :type "/Game/TankChess/Game/Units/Tanks/Blueprints/STankConfig Structure") (Color :type "LinearColor Structure") (Light :type Boolean))
  (returns (Hologram :type "/Game/TankChess/Game/Units/Tanks/Blueprints/BP_HologramTank Object Reference"))
  (bind _result (`BlueprintSetLibrary.Set_ToArray` (`self.Holograms`)))
  (for _array_element _result
    (if (`/Game/TankChess/Game/Units/Tanks/Blueprints/BPFL_TankDataMaps.EqualCoords` (`.Coords_11_E825CE4C49EDC82B0C70A68D3435969C` (break `/Game/TankChess/Game/Units/Tanks/Blueprints/STankConfig` Config)) (`/Game/TankChess/Game/Units/Tanks/Blueprints/BP_BaseTank.coords` _array_element))
      (`/Game/TankChess/Game/Units/Tanks/Blueprints/BP_HologramTank.SetHologramMaterial` _array_element Color Light)
      (return _array_element)))
  (bind _returnvalue (`|SpawnActorFromClass` "/Game/TankChess/Game/Units/Tanks/Blueprints/BP_HologramTank.BP_HologramTank_C" (`KismetMathLibrary.MakeTransform` (0.0 0.0 0.0)) "Undefined" "MultiplyWithRoot" null null))
  (`/Game/TankChess/Game/Units/Tanks/Blueprints/BP_BaseTank.SetConfig` _returnvalue Config)
  (`/Game/TankChess/Game/Units/Tanks/Blueprints/BP_HologramTank.SetHologramMaterial` _returnvalue Color Light)
  (`BlueprintSetLibrary.Set_Add` (`self.Holograms`) _returnvalue)
  (return _returnvalue))

(fn `UserConstructionScript`)