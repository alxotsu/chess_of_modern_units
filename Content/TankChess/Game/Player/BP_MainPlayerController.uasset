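; Player controller for TankChess that handles camera movement, tank selection and turn-based move planning.
; Camera input rotates and pans the pawn, with zoom coupling height to pitch.
; A cursor trace selects tanks of the side to move, which refreshes whenever the game mode ends a move.
; Queued steps are dry-run through the tank's MakeMove and shown as HUD holograms, dropping impossible ones, until confirmed, undone or cancelled.
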(event `InputAxis|Zoom`
  (params (AxisValue :type "Float (single-precision)"))
  (bind _returnvalue (`self.K2_GetPawn`))
  (bind _output_get (set `self.ZoomValue` (`KismetMathLibrary.FClamp` (+ (* AxisValue -0.05) (`self.ZoomValue`)))))
  (`SceneComponent.K2_SetWorldTransform` (`Actor.RootComponent` _returnvalue) (`KismetMathLibrary.MakeTransform` (`KismetMathLibrary.MakeVector` (.x (.location (`self.GetTransform` _returnvalue))) (.y (.location (`self.GetTransform` _returnvalue))) (+ (* _output_get 800.0) 100.0)) (`KismetMathLibrary.MakeRotator` (.roll (.rotation (`self.GetTransform` _returnvalue))) (+ (* _output_get -70.0) -10.0) (.yaw (.rotation (`self.GetTransform` _returnvalue))))) false false))

(event `InputAxis|MouseY`
  (params (AxisValue :type "Float (single-precision)"))
  (if (or (`self.MoveCamera`) (`self.MoveCameraPlane`))
    (`self.MovePawn` (* AxisValue -10.0))))

(event `EnhancedInput|/Game/TankChess/Game/Player/Input/Actions/CameraControl/IA_EnablePlaneCameraMove`
  (params (ActionValue :type Boolean) (ElapsedSeconds :type "Float (double-precision)") (TriggeredSeconds :type "Float (double-precision)") (InputAction :type "InputAction Object Reference" :default "/Game/TankChess/Game/Player/Input/Actions/CameraControl/IA_EnablePlaneCameraMove.IA_EnablePlaneCameraMove"))
  (:`Triggered`
    (set `self.MoveCameraPlane` true))
  (:`Completed`
    (set `self.MoveCameraPlane` false)))

(event `InputAxis|MouseX`
  (params (AxisValue :type "Float (single-precision)"))
  (if (`self.MoveCamera`)
    (`self.MovePawn` 0.0 0.0 AxisValue)
    (elif (`self.MoveCameraPlane`)
      (`self.MovePawn` 0.0 (* AxisValue -10.0)))))

(event `EnhancedInput|/Game/TankChess/Game/Player/Input/Actions/CameraControl/IA_EnableCamera`
  (params (ActionValue :type Boolean) (ElapsedSeconds :type "Float (double-precision)") (TriggeredSeconds :type "Float (double-precision)") (InputAction :type "InputAction Object Reference" :default "/Game/TankChess/Game/Player/Input/Actions/CameraControl/IA_EnableCamera.IA_EnableCamera"))
  (:`Triggered`
    (set `self.MoveCamera` true))
  (:`Completed`
    (set `self.MoveCamera` false)))

(event `MovePawn`
  (params (Forward :type "Float (double-precision)") (Side :type "Float (double-precision)") (Rotate :type "Float (double-precision)"))
  (bind _returnvalue (`self.K2_GetPawn`))
  (bind _yaw (.yaw (.rotation (`self.GetTransform` _returnvalue))))
  (bind _returnvalue_2 (+ _yaw 90.0))
  (`SceneComponent.K2_SetWorldTransform` (`Actor.RootComponent` _returnvalue) (`KismetMathLibrary.MakeTransform` (`KismetMathLibrary.MakeVector` (+ (.x (.location (`self.GetTransform` _returnvalue))) (* Forward (`KismetMathLibrary.DegCos` _yaw)) (* Side (`KismetMathLibrary.DegCos` _returnvalue_2))) (+ (.y (.location (`self.GetTransform` _returnvalue))) (* Forward (`KismetMathLibrary.DegSin` _yaw)) (* Side (`KismetMathLibrary.DegSin` _returnvalue_2))) (.z (.location (`self.GetTransform` _returnvalue)))) (`KismetMathLibrary.MakeRotator` (.roll (.rotation (`self.GetTransform` _returnvalue))) (.pitch (.rotation (`self.GetTransform` _returnvalue))) (+ _yaw Rotate 0.0))) false false))

(event `self.ReceiveBeginPlay`
  (bind _returnvalue (subsystem `EnhancedInputLocalPlayerSubsystem`))
  (`|ExecutionSequence`
    (:`then_0`
      (`/Engine/EditorBlueprintResources/StandardMacros.IsValid` _returnvalue
        (:`Is Valid`
          (`EnhancedInputSubsystemInterface.AddMappingContext` _returnvalue "/Game/TankChess/Game/Player/Input/IMC_MainGameActions.IMC_MainGameActions" 0 (struct))
          (set `self.bShowMouseCursor` true))))
    (:`then_1`
      (bind _asbp_game_mode_main (cast `/Game/TankChess/Game/BP_GameModeMain` (`GameplayStatics.GetGameMode`)))
      (add `/Game/TankChess/Game/BP_GameModeMain.OnEndMove` _asbp_game_mode_main (delegate `UpdateSide`)))
    (:`then_2`
      (`self.UpdateSide`))))

(event `DefaultCameraPosition`
  (bind _asbp_main_pawn (cast `/Game/TankChess/Game/Player/BP_MainPawn` (`self.K2_GetPawn`) :!label _label))
  (`/Game/TankChess/Game/Player/BP_MainPawn.UpdatePosition` _asbp_main_pawn))

(event `UpdateSide`
  (bind _gamestate (message `/Game/TankChess/Game/BPI_GameStateMain.GetGameState` (`GameplayStatics.GetGameState`)))
  (set `self.Side` (`.NowMove_35_2D1A271D48DF300CB4A9C28CFB476DAF` (break `/Game/TankChess/Core/S_GameState` _gamestate)))
  (bind _asbp_main_pawn (cast `/Game/TankChess/Game/Player/BP_MainPawn` (`self.K2_GetPawn`)))
  (`/Game/TankChess/Game/Player/BP_MainPawn.UpdatePosition` _asbp_main_pawn))

(event `EnhancedInput|/Game/TankChess/Game/Player/Input/Actions/CameraControl/IA_SetDefaultPosition`
  (params (ActionValue :type Boolean) (ElapsedSeconds :type "Float (double-precision)") (TriggeredSeconds :type "Float (double-precision)") (InputAction :type "InputAction Object Reference" :default "/Game/TankChess/Game/Player/Input/Actions/CameraControl/IA_SetDefaultPosition.IA_SetDefaultPosition"))
  (:`Completed`
    (goto _label)))

(event `EnhancedInput|/Game/TankChess/Game/Player/Input/Actions/TankControl/IA_MoveUnit_Forward`
  (params (ActionValue :type Boolean) (ElapsedSeconds :type "Float (double-precision)") (TriggeredSeconds :type "Float (double-precision)") (InputAction :type "InputAction Object Reference" :default "/Game/TankChess/Game/Player/Input/Actions/TankControl/IA_MoveUnit_Forward.IA_MoveUnit_Forward"))
  (:`Completed`
    (`self.AddOneMovement` "NewEnumerator0")))

(event `EnhancedInput|/Game/TankChess/Game/Player/Input/Actions/TankControl/IA_MoveUnit_Back`
  (params (ActionValue :type Boolean) (ElapsedSeconds :type "Float (double-precision)") (TriggeredSeconds :type "Float (double-precision)") (InputAction :type "InputAction Object Reference" :default "/Game/TankChess/Game/Player/Input/Actions/TankControl/IA_MoveUnit_Back.IA_MoveUnit_Back"))
  (:`Completed`
    (`self.AddOneMovement` "NewEnumerator1")))

(event `EnhancedInput|/Game/TankChess/Game/Player/Input/Actions/TankControl/IA_SelectUnit_Click`
  (params (ActionValue :type Boolean) (ElapsedSeconds :type "Float (double-precision)") (TriggeredSeconds :type "Float (double-precision)") (InputAction :type "InputAction Object Reference" :default "/Game/TankChess/Game/Player/Input/Actions/TankControl/IA_SelectUnit_Click.IA_SelectUnit_Click"))
  (bind (_unit _coords _valid) (`self.SelectCell`))
  (:`Completed`
    (if (and (`self.EnabledControl`) _valid)
      (`/Engine/EditorBlueprintResources/StandardMacros.IsValid` _unit
        (:`Is Valid`
          (if (`|EnumEquality` (`/Game/TankChess/Game/Units/Tanks/Blueprints/BP_BaseTank.Side` _unit) (`self.Side`))
            (bind _output_get (set `self.SelectedTank` _unit))
            (`KismetArrayLibrary.Array_Clear` (`self.Moves`))
            (bind (_valid_2 _possible _configsofselectedtank _othertankconfigs) (`/Game/TankChess/Game/Units/Tanks/Blueprints/BP_BaseTank.MakeMove` :`self` _output_get))
            (message `/Game/TankChess/Game/Player/BPI_GameHud.VisualizeHolograms` (`self.GetHUD`) (`self.Moves`) _configsofselectedtank _othertankconfigs _valid_2)
            (else
              (`/Engine/EditorBlueprintResources/StandardMacros.IsValid` (`self.SelectedTank`)
                (:`Is Valid`
                  (bind _socket (message `/Game/TankChess/Game/Player/BPI_GameHud.GetSelectedComponent` (`self.GetHUD`)))
                  (`self.AddMove` (make `/Game/TankChess/Game/Units/Tanks/Blueprints/STankMove` _socket _coords)))))))
        (:`Is Not Valid`
          (`/Engine/EditorBlueprintResources/StandardMacros.IsValid` (`self.SelectedTank`)
            (:`Is Valid`
              (message `/Game/TankChess/Game/Player/BPI_GameHud.OpenWayCalculator` (`self.GetHUD`) _coords))))))))

(event `EnhancedInput|/Game/TankChess/Game/Player/Input/Actions/TankControl/IA_MoveUnit_Right`
  (params (ActionValue :type Boolean) (ElapsedSeconds :type "Float (double-precision)") (TriggeredSeconds :type "Float (double-precision)") (InputAction :type "InputAction Object Reference" :default "/Game/TankChess/Game/Player/Input/Actions/TankControl/IA_MoveUnit_Right.IA_MoveUnit_Right"))
  (:`Completed`
    (`self.AddOneMovement` "NewEnumerator3")))

(event `EnhancedInput|/Game/TankChess/Game/Player/Input/Actions/TankControl/IA_MoveUnit_Left`
  (params (ActionValue :type Boolean) (ElapsedSeconds :type "Float (double-precision)") (TriggeredSeconds :type "Float (double-precision)") (InputAction :type "InputAction Object Reference" :default "/Game/TankChess/Game/Player/Input/Actions/TankControl/IA_MoveUnit_Left.IA_MoveUnit_Left"))
  (:`Completed`
    (`self.AddOneMovement` "NewEnumerator2")))

(event `MakeMove`
  (bind _valid (`/Game/TankChess/Game/Units/Tanks/Blueprints/BP_BaseTank.MakeMove` (`self.SelectedTank`) (`self.Moves`) true :!label _label_2))
  (if _valid
    (`self.ResetMove`)))

(event `EnhancedInput|/Game/TankChess/Game/Player/Input/Actions/TankControl/IA_ConfirmMove`
  (params (ActionValue :type Boolean) (ElapsedSeconds :type "Float (double-precision)") (TriggeredSeconds :type "Float (double-precision)") (InputAction :type "InputAction Object Reference" :default "/Game/TankChess/Game/Player/Input/Actions/TankControl/IA_ConfirmMove.IA_ConfirmMove"))
  (:`Completed`
    (goto _label_2)))

(event `ResetMove`
  (message `/Game/TankChess/Game/Player/BPI_GameHud.ClearAllHolograms` (`self.GetHUD`) :!label _label_3)
  (set `self.SelectedTank` null)
  (`KismetArrayLibrary.Array_Clear` (`self.Moves`)))

(event `EnhancedInput|/Game/TankChess/Game/Player/Input/Actions/TankControl/IA_CancelMove`
  (params (ActionValue :type Boolean) (ElapsedSeconds :type "Float (double-precision)") (TriggeredSeconds :type "Float (double-precision)") (InputAction :type "InputAction Object Reference" :default "/Game/TankChess/Game/Player/Input/Actions/TankControl/IA_CancelMove.IA_CancelMove"))
  (:`Completed`
    (goto _label_3)))

(event `UndoMovement`
  (bind _moves (`self.Moves`))
  (bind _moves_2 (`self.Moves`))
  (if (`KismetArrayLibrary.Array_IsNotEmpty` _moves) :!label _label_4
    (`KismetArrayLibrary.Array_Remove` _moves_2 (- (`KismetArrayLibrary.Array_Length` _moves) 1))
    (bind (_valid _possible _configsofselectedtank _othertankconfigs) (`/Game/TankChess/Game/Units/Tanks/Blueprints/BP_BaseTank.MakeMove` (`self.SelectedTank`) _moves_2 false))
    (message `/Game/TankChess/Game/Player/BPI_GameHud.VisualizeHolograms` (`self.GetHUD`) (`self.Moves`) _configsofselectedtank _othertankconfigs _valid)))

(event `EnhancedInput|/Game/TankChess/Game/Player/Input/Actions/TankControl/IA_UndoMovement`
  (params (ActionValue :type Boolean) (ElapsedSeconds :type "Float (double-precision)") (TriggeredSeconds :type "Float (double-precision)") (InputAction :type "InputAction Object Reference" :default "/Game/TankChess/Game/Player/Input/Actions/TankControl/IA_UndoMovement.IA_UndoMovement"))
  (:`Completed`
    (goto _label_4)))

(fn `AddMove`
  (params (Move :type "/Game/TankChess/Game/Units/Tanks/Blueprints/STankMove Structure"))
  (returns (Possible :type Boolean))
  (bind _moves (`self.Moves`))
  (bind _moves_2 (`self.Moves`))
  (`KismetArrayLibrary.Array_Add` _moves_2 Move)
  (bind (_valid _possible _configsofselectedtank _othertankconfigs) (`/Game/TankChess/Game/Units/Tanks/Blueprints/BP_BaseTank.MakeMove` (`self.SelectedTank`) _moves_2 false))
  (if _possible
    (message `/Game/TankChess/Game/Player/BPI_GameHud.VisualizeHolograms` (`self.GetHUD`) _moves _configsofselectedtank _othertankconfigs _valid)
    (else
      (`KismetArrayLibrary.Array_Remove` _moves (- (`KismetArrayLibrary.Array_Length` _moves) 1))))
  (return _possible))

(fn `AddOneMovement`
  (params (Movement :type "/Game/TankChess/Game/Units/UnitComponents/Blueprints/MovementComponents/EMovement Enum" :default "NewEnumerator0"))
  (returns (Valid :type Boolean))
  (if (and (`self.EnabledControl`) (`KismetSystemLibrary.IsValid` (`self.SelectedTank`)))
    (bind _possible (`self.AddMove` (make `/Game/TankChess/Game/Units/Tanks/Blueprints/STankMove` "None" (struct) Movement)))
    (return _possible)))

(fn `EnabledControl`
  (returns (Enabled :type Boolean))
  (bind _gamestate (message `/Game/TankChess/Game/BPI_GameStateMain.GetGameState` (`GameplayStatics.GetGameState`)))
  (return (`|EnumEquality` (break `/Game/TankChess/Core/S_GameState` _gamestate) (`self.Side`))))

(fn `SelectCell`
  (returns (Unit :type "/Game/TankChess/Game/Units/Tanks/Blueprints/BP_BaseTank Object Reference") (Coords :type "/Game/TankChess/Game/Field/Blueprints/SFieldCellCoords Structure") (Valid :type Boolean))
  (bind _map (`|MakeMap` null :!type "/Game/TankChess/Game/Units/Tanks/Blueprints/BP_BaseTank Object Reference" :!valuetype "/Game/TankChess/Game/Units/Tanks/Blueprints/STankConfig Structure"))
  (bind (_bblockinghit _binitialoverlap _time _distance _location _impactpoint _normal _impactnormal _physmat _hitactor) (`GameplayStatics.BreakHitResult` (`self.GetHitResultUnderCursorByChannel` "TraceTypeQuery1")))
  (bind _asbp_cell (cast `/Game/TankChess/Game/Field/Blueprints/BP_Cell` _hitactor)
    (:`then`
      (bind _coords (`/Game/TankChess/Game/Field/Blueprints/BP_Cell.Coords` _asbp_cell))
      (bind _tank (message `/Game/TankChess/Game/BPI_GameStateMain.GetCell` (`GameplayStatics.GetGameState`) _coords _map))
      (return _tank _coords true))
    (:`CastFailed`
      (bind _asbp_base_tank (cast `/Game/TankChess/Game/Units/Tanks/Blueprints/BP_BaseTank` _hitactor)
        (:`then`
          (bind _coords_2 (`/Game/TankChess/Game/Units/Tanks/Blueprints/BP_BaseTank.coords` _asbp_base_tank))
          (bind _tank_2 (message `/Game/TankChess/Game/BPI_GameStateMain.GetCell` (`GameplayStatics.GetGameState`) _coords_2 _map))
          (return _tank_2 _coords_2 true))
        (:`CastFailed`
          (return null (struct) false))))))

(fn `UserConstructionScript`)