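; BP_MainPawn is the player pawn for TankChess, providing a raised, downward-angled viewpoint at the player's side of the field.
; UpdatePosition derives offsets from the field dimensions in the game state's field-state message.
; It then reads the local player controller's Side and moves the root component beyond the matching end along Y, with Black and White facing opposite directions.
; The event graph and construction script are empty.
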(fn `UpdatePosition`
  (locals (YOffset :type "Float (double-precision)") (XOffset :type "Float (double-precision)" :default 0.0))
  (`|ExecutionSequence`
    (:`then_0`
      (bind _state (message `/Game/TankChess/Game/BPI_GameStateMain.GetFieldState` (`GameplayStatics.GetGameState`)))
      (bind (_sizex _sizey) (break `/Game/TankChess/Game/Field/Blueprints/SFieldState` _state))
      (set `local.YOffset` (`KismetMathLibrary.Conv_IntToDouble` (* _sizey 50)))
      (set `local.XOffset` (`KismetMathLibrary.Conv_IntToDouble` (* (- _sizey 1) 50))))
    (:`then_1`
      (bind _asbp_main_player_controller (cast `/Game/TankChess/Game/Player/BP_MainPlayerController` (`self.GetLocalViewingPlayerController`)))
      (switch `/Game/TankChess/Game/Player/EPlayerSide` (`/Game/TankChess/Game/Player/BP_MainPlayerController.Side` _asbp_main_player_controller)
        (:`NewEnumerator0`
          (`SceneComponent.K2_SetWorldLocationAndRotation` (`self.DefaultSceneRoot`) (`KismetMathLibrary.MakeVector` (`local.XOffset`) (+ (- (* _sizex 100) 50) (`local.YOffset`)) 400.0) (struct :`Pitch` -30.0 :`Yaw` -90.0) false false))
        (:`NewEnumerator1`
          (`SceneComponent.K2_SetWorldLocationAndRotation` (`self.DefaultSceneRoot`) (`KismetMathLibrary.MakeVector` (`local.XOffset`) (* (+ (`local.YOffset`) 50.0) -1.0) 400.0) (struct :`Pitch` -30.0 :`Yaw` 90.0) false false))))))

(fn `UserConstructionScript`)