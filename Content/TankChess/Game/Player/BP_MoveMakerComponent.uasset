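; Player component for TankChess that enumerates, simulates and validates unit moves on field states.
; Unit modules supply the rules: each behavior class from DT_UnitModules is spawned as a temporary component, queried, then destroyed.
; ComputeOneMove checks unit and turn, and ComputeMoves chains it from the GameState field, failing on any impossible step.
; CalculateWays exhaustively expands possible moves, keeping the route to a target with most move points left per final facing.
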(fn `CalculateWays`
  (params (FieldState :type "/Game/TankChess/Game/Field/Blueprints/SFieldState Structure") (UnitConfig :type "/Game/TankChess/Game/Units/Blueprints/SUnitConfig Structure") (TargetCoords :type "/Game/TankChess/Game/Field/Blueprints/SFieldCellCoords Structure"))
  (returns (Ways :type "Map of /Game/TankChess/Game/Units/Blueprints/EDirection Enum to /Game/TankChess/Game/Player/SCalculatedWay Structure"))
  (locals (WaysForCheck :type "Array of /Game/TankChess/Game/Player/SCalculatedWay Structure") (OutputWays :type "Map of /Game/TankChess/Game/Units/Blueprints/EDirection Enum to /Game/TankChess/Game/Player/SCalculatedWay Structure") (Sockets :type "Array of Name") (Moves :type "Array of /Game/TankChess/Game/Units/Blueprints/SUnitMove Structure"))
  (`KismetArrayLibrary.Array_Add` (`local.WaysForCheck`) (make `/Game/TankChess/Game/Player/SCalculatedWay` FieldState UnitConfig))
  (for _array_element (`local.WaysForCheck`)
    (bind (_fieldstate _unitconfig) (break `/Game/TankChess/Game/Player/SCalculatedWay` _array_element))
    (bind (_value _returnvalue) (`BlueprintMapLibrary.Map_Find` (`local.OutputWays`) (`.Direction_56_4F2B10F847F49B1199F4DC823B142897` (break `/Game/TankChess/Game/Units/Blueprints/SUnitConfig` _unitconfig))))
    (if (and (`/Game/TankChess/Game/Units/Blueprints/BPFL_CoordsAndDirectionTransforms.EqualCoords` (`.Coords_47_E98C47904C4A4C6B43CCA291531B50D8` (break `/Game/TankChess/Game/Units/Blueprints/SUnitConfig` _unitconfig)) (`local.TargetCoords`)) (or (> (break `/Game/TankChess/Game/Units/Blueprints/SUnitTempState` (`.TempState_62_5ABFF3A34B4DD39392594A92040E2E81` (break `/Game/TankChess/Game/Units/Blueprints/SUnitConfig` _unitconfig))) (break `/Game/TankChess/Game/Units/Blueprints/SUnitTempState` (`.TempState_62_5ABFF3A34B4DD39392594A92040E2E81` (break `/Game/TankChess/Game/Units/Blueprints/SUnitConfig` (`.UnitConfig_2_EAC4962249C2BC1D6D65DDB63682F041` (break `/Game/TankChess/Game/Player/SCalculatedWay` _value)))))) (not _returnvalue)))
      (`BlueprintMapLibrary.Map_Add` (`local.OutputWays`) (`.Direction_56_4F2B10F847F49B1199F4DC823B142897` (break `/Game/TankChess/Game/Units/Blueprints/SUnitConfig` _unitconfig)) _array_element))
    (bind (_fieldstate_2 _unitconfig_2 _moves) (break `/Game/TankChess/Game/Player/SCalculatedWay` _array_element))
    (bind _moves_2 (`self.GetPossibleMoves` _fieldstate_2 _unitconfig_2))
    (bind _result (`BlueprintSetLibrary.Set_ToArray` _moves_2))
    (for _array_element_2 _result
      (bind (_newfieldstate _newunit _possible) (`self.ComputeOneMove` _fieldstate_2 _array_element_2 _unitconfig_2))
      (if _possible
        (bind _output_get (set `local.Moves` _moves))
        (`KismetArrayLibrary.Array_Add` _output_get _array_element_2)
        (`KismetArrayLibrary.Array_Add` (`local.WaysForCheck`) (make `/Game/TankChess/Game/Player/SCalculatedWay` _newfieldstate _newunit _output_get)))))
  (return (`local.OutputWays`)))

(fn `ComputeMoves`
  (params (UnitCoords :type "/Game/TankChess/Game/Field/Blueprints/SFieldCellCoords Structure") (Moves :type "Array of /Game/TankChess/Game/Units/Blueprints/SUnitMove Structure"))
  (returns (NewFieldState :type "/Game/TankChess/Game/Field/Blueprints/SFieldState Structure") (NewUnitConfig :type "/Game/TankChess/Game/Units/Blueprints/SUnitConfig Structure") (Valid :type Boolean) (Possible :type Boolean))
  (locals (TempUnitConfig :type "/Game/TankChess/Game/Units/Blueprints/SUnitConfig Structure") (TempFieldState :type "/Game/TankChess/Game/Field/Blueprints/SFieldState Structure"))
  (bind _tempunitconfig (`local.TempUnitConfig`))
  (bind _tempfieldstate (`local.TempFieldState`))
  (bind _state (message `/Game/TankChess/Game/BPI_GameStateMain.GetFieldState` (`GameplayStatics.GetGameState`)))
  (set `local.TempFieldState` _state)
  (bind (_value _returnvalue) (`BlueprintMapLibrary.Map_Find` (`.Units_31_8194BC274A1D6B758B12AA93D64CC056` (break `/Game/TankChess/Game/Field/Blueprints/SFieldState` _state)) UnitCoords))
  (if _returnvalue
    (set `local.TempUnitConfig` _value)
    (for _array_element Moves
      (bind (_newfieldstate _newunit _possible) (`self.ComputeOneMove` _tempfieldstate _array_element _tempunitconfig))
      (if _possible
        (set `local.TempFieldState` _newfieldstate)
        (set `local.TempUnitConfig` _newunit)
        (else
          (return (struct) (struct) false false))))
    (return _tempfieldstate _tempunitconfig (not (`/Game/TankChess/Game/BPFL_CellsAndUnits.EqualFieldStates` _state (`local.TempFieldState`))) true)
    (else
      (return (struct) (struct) false false))))

(fn `ComputeOneMove`
  (params (FieldState :type "/Game/TankChess/Game/Field/Blueprints/SFieldState Structure") (Move :type "/Game/TankChess/Game/Units/Blueprints/SUnitMove Structure") (Unit :type "/Game/TankChess/Game/Units/Blueprints/SUnitConfig Structure"))
  (returns (NewFieldState :type "/Game/TankChess/Game/Field/Blueprints/SFieldState Structure") (NewUnit :type "/Game/TankChess/Game/Units/Blueprints/SUnitConfig Structure") (Possible :type Boolean))
  (locals (ModuleClass :type "/Game/TankChess/Game/Units/Blueprints/Modules/BP_BaseUnitModuleComponent Class Reference"))
  (bind (_mainmodule _moduleonsockets) (break `/Game/TankChess/Game/Units/Blueprints/SUnitConfig` Unit))
  (bind (_mainmodule_2 _moduleonsockets_2 _coords _direction _alive _side) (break `/Game/TankChess/Game/Units/Blueprints/SUnitConfig` Unit))
  (bind _activecomponent (break `/Game/TankChess/Game/Units/Blueprints/SUnitMove` Move))
  (bind (_value _returnvalue) (`BlueprintMapLibrary.Map_Find` (`.Units_31_8194BC274A1D6B758B12AA93D64CC056` (break `/Game/TankChess/Game/Field/Blueprints/SFieldState` FieldState)) _coords))
  (bind _gamestate (message `/Game/TankChess/Game/BPI_GameStateMain.GetGameState` (`GameplayStatics.GetGameState`)))
  (if (and (`/Game/TankChess/Game/BPFL_CellsAndUnits.EqualUnits` _value Unit) _returnvalue _alive (`|EnumEquality` (break `/Game/TankChess/Core/SGameState` _gamestate) _side))
    (if (== _activecomponent "Main")
      (bind _returnvalue_2 (`|GetDataTableRow` "/Game/TankChess/Game/Units/Blueprints/Modules/DT_UnitModules.DT_UnitModules" _mainmodule)
        (:`then`
          (set `local.ModuleClass` (break `/Game/TankChess/Game/Units/Blueprints/Modules/TableStructures/SModuleDescription` _returnvalue_2))
          (bind _returnvalue_3 (`|AddComponentByClass` (`self.GetOwner`) (`local.ModuleClass`) _activecomponent :!label _label))
          (bind (_newfieldstate _newunitconfig _possible) (`/Game/TankChess/Game/Units/Blueprints/Modules/BP_BaseUnitModuleComponent.ComputeMove` _returnvalue_3 (`local.FieldState`) (`local.Unit`) (`local.Move`)))
          (`self.K2_DestroyComponent` _returnvalue_3)
          (return _newfieldstate _newunitconfig _possible))
        (:`RowNotFound`
          _))
      (else
        (bind _returnvalue_4 (`|GetDataTableRow` "/Game/TankChess/Game/Units/Blueprints/Modules/DT_UnitModules.DT_UnitModules" (`BlueprintMapLibrary.Map_Find` _moduleonsockets _activecomponent))
          (:`then`
            (set `local.ModuleClass` (break `/Game/TankChess/Game/Units/Blueprints/Modules/TableStructures/SModuleDescription` _returnvalue_4))
            (goto _label))
          (:`RowNotFound`
            _))))
    (return (struct) (struct) false)
    (else
      (return (struct) (struct) false))))

(fn `GetPossibleMoves`
  (params (FieldState :type "/Game/TankChess/Game/Field/Blueprints/SFieldState Structure") (UnitConfig :type "/Game/TankChess/Game/Units/Blueprints/SUnitConfig Structure"))
  (returns (Moves :type "Set of /Game/TankChess/Game/Units/Blueprints/SUnitMove Structure"))
  (locals (PossibleMoves :type "Set of /Game/TankChess/Game/Units/Blueprints/SUnitMove Structure") (Module :type "/Game/TankChess/Game/Units/Blueprints/Modules/BP_BaseUnitModuleComponent Object Reference"))
  (bind (_mainmodule _moduleonsockets _coords _direction _alive) (break `/Game/TankChess/Game/Units/Blueprints/SUnitConfig` UnitConfig))
  (if _alive
    (`|ExecutionSequence`
      (:`then_0`
        (bind _keys (`BlueprintMapLibrary.Map_Keys` _moduleonsockets))
        (for _array_element _keys
          (bind _returnvalue (`|GetDataTableRow` "/Game/TankChess/Game/Units/Blueprints/Modules/DT_UnitModules.DT_UnitModules" (`BlueprintMapLibrary.Map_Find` _moduleonsockets _array_element))
            (:`then`
              (bind _returnvalue_2 (`|AddComponentByClass` (`self.GetOwner`) (break `/Game/TankChess/Game/Units/Blueprints/Modules/TableStructures/SModuleDescription` _returnvalue) _array_element))
              (set `local.Module` _returnvalue_2)
              (bind _possiblemoves (`/Game/TankChess/Game/Units/Blueprints/Modules/BP_BaseUnitModuleComponent.GetPossibleMoves` (`local.Module`) (`local.FieldState`) (`local.UnitConfig`) :!label _label))
              (bind _result (`BlueprintSetLibrary.Set_ToArray` _possiblemoves))
              (`BlueprintSetLibrary.Set_AddItems` (`local.PossibleMoves`) _result)
              (`self.K2_DestroyComponent` (`local.Module`))))))
      (:`then_1`
        (bind _returnvalue_3 (`|GetDataTableRow` "/Game/TankChess/Game/Units/Blueprints/Modules/DT_UnitModules.DT_UnitModules" _mainmodule)
          (:`then`
            (bind _returnvalue_4 (`|AddComponentByClass` (`self.GetOwner`) (break `/Game/TankChess/Game/Units/Blueprints/Modules/TableStructures/SModuleDescription` _returnvalue_3) "Main"))
            (set `local.Module` _returnvalue_4)
            (goto _label))))
      (:`then_2`
        (return (`local.PossibleMoves`))))
    (else
      (return))))