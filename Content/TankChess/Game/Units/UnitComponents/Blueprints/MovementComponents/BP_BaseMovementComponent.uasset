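; Base movement component for Tank Chess units, with placeholder movement and damage logic that appears meant for child classes to override.
; MakeMove delegates to CalculateMovement, while ApplyDamage always reports invalid.
; CalculateWaysForCoord expands BP_RecursiveMovementNode children breadth-first by appending to the list it iterates.
; For each facing direction at the target coordinate, it keeps the path leaving the most move points.
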(fn `ApplyDamage`
  (params (Direction :type "/Game/TankChess/Game/Units/Tanks/Blueprints/EDirection Enum" :default "NewEnumerator0") (GunPower :type Integer) (Config :type "/Game/TankChess/Game/Units/Tanks/Blueprints/STankConfig Structure"))
  (returns (Valid :type Boolean) (NewConfig :type "/Game/TankChess/Game/Units/Tanks/Blueprints/STankConfig Structure"))
  (return false))

(fn `CalculateMovement`
  (params (Config :type "/Game/TankChess/Game/Units/Tanks/Blueprints/STankConfig Structure") (Movement :type "/Game/TankChess/Game/Units/UnitComponents/Blueprints/MovementComponents/EMovement Enum" :default "NewEnumerator0") (OtherConfigs :type "Map of /Game/TankChess/Game/Units/Tanks/Blueprints/BP_BaseTank Object Reference to /Game/TankChess/Game/Units/Tanks/Blueprints/STankConfig Structure"))
  (returns (NewConfig :type "/Game/TankChess/Game/Units/Tanks/Blueprints/STankConfig Structure") (Possible :type Boolean) (OutputConfigs :type "Map of /Game/TankChess/Game/Units/Tanks/Blueprints/BP_BaseTank Object Reference to /Game/TankChess/Game/Units/Tanks/Blueprints/STankConfig Structure"))
  (locals (Delta :type "/Game/TankChess/Game/Field/Blueprints/SFieldCellCoords Structure") (OutputConfig :type "/Game/TankChess/Game/Units/Tanks/Blueprints/STankConfig Structure"))
  (return (struct) true))

(fn `CalculateWaysForCoord`
  (params (TargetCoords :type "/Game/TankChess/Game/Field/Blueprints/SFieldCellCoords Structure") (Config :type "/Game/TankChess/Game/Units/Tanks/Blueprints/STankConfig Structure") (OtherConfigs :type "Map of /Game/TankChess/Game/Units/Tanks/Blueprints/BP_BaseTank Object Reference to /Game/TankChess/Game/Units/Tanks/Blueprints/STankConfig Structure"))
  (returns (Ways :type "Map of /Game/TankChess/Game/Units/Tanks/Blueprints/EDirection Enum to /Game/TankChess/Game/Units/UnitComponents/Blueprints/MovementComponents/SCalculatedWay Structure"))
  (locals (NodesForCheck :type "Array of /Game/TankChess/Game/Units/UnitComponents/Blueprints/MovementComponents/BP_RecursiveMovementNode Object Reference") (OutputWays :type "Map of /Game/TankChess/Game/Units/Tanks/Blueprints/EDirection Enum to /Game/TankChess/Game/Units/UnitComponents/Blueprints/MovementComponents/SCalculatedWay Structure") (MaxMovePoints :type "Map of /Game/TankChess/Game/Units/Tanks/Blueprints/EDirection Enum to Object Object Reference"))
  ;[1 1 1] Dont work simple default value
  ; (I do not fucking know why)
  (set `local.MaxMovePoints` (`|MakeMap` "NewEnumerator0" -1 "NewEnumerator1" -1 "NewEnumerator2" -1 "NewEnumerator3" -1 "NewEnumerator4" -1 "NewEnumerator5" -1 "NewEnumerator6" -1 "NewEnumerator7" -1 :!type "/Game/TankChess/Game/Units/Tanks/Blueprints/EDirection Enum"))
  (bind _returnvalue (`|GenericCreateObject` "/Game/TankChess/Game/Units/UnitComponents/Blueprints/MovementComponents/BP_RecursiveMovementNode.BP_RecursiveMovementNode_C"))
  (set `/Game/TankChess/Game/Units/UnitComponents/Blueprints/MovementComponents/BP_RecursiveMovementNode.TempConfig` Config _returnvalue)
  (bind _children (`/Game/TankChess/Game/Units/UnitComponents/Blueprints/MovementComponents/BP_RecursiveMovementNode.MakeChildren` _returnvalue self (`local.OtherConfigs`)))
  (bind _output_get (set `local.NodesForCheck` _children))
  (for _array_element _output_get
    (bind (_maincomponentclass _coords _direction _alive _side _components _tempstate) (break `/Game/TankChess/Game/Units/Tanks/Blueprints/STankConfig` (`/Game/TankChess/Game/Units/UnitComponents/Blueprints/MovementComponents/BP_RecursiveMovementNode.TempConfig` _array_element)))
    (bind _movepoints (break `/Game/TankChess/Game/Units/Tanks/Blueprints/STankTempState` _tempstate))
    (if (and (`/Game/TankChess/Game/Units/Tanks/Blueprints/BPFL_TankDataMaps.EqualCoords` (`local.TargetCoords`) _coords) (> _movepoints (`BlueprintMapLibrary.Map_Find` (`local.MaxMovePoints`) _direction)))
      (`BlueprintMapLibrary.Map_Add` (`local.MaxMovePoints`) _direction _movepoints)
      (bind _way (`/Game/TankChess/Game/Units/UnitComponents/Blueprints/MovementComponents/BP_RecursiveMovementNode.GetCalculatedWay` _array_element))
      (`BlueprintMapLibrary.Map_Add` (`local.OutputWays`) _direction _way))
    (bind _children_2 (`/Game/TankChess/Game/Units/UnitComponents/Blueprints/MovementComponents/BP_RecursiveMovementNode.MakeChildren` _array_element self (`local.OtherConfigs`)))
    (`KismetArrayLibrary.Array_Append` (`local.NodesForCheck`) _children_2))
  (return (`local.OutputWays`)))

(fn `MakeMove`
  (params (Move :type "/Game/TankChess/Game/Units/Tanks/Blueprints/STankMove Structure") (Config :type "/Game/TankChess/Game/Units/Tanks/Blueprints/STankConfig Structure") (OtherConfigs :type "Map of /Game/TankChess/Game/Units/Tanks/Blueprints/BP_BaseTank Object Reference to /Game/TankChess/Game/Units/Tanks/Blueprints/STankConfig Structure"))
  (returns (NewConfig :type "/Game/TankChess/Game/Units/Tanks/Blueprints/STankConfig Structure") (Possible :type Boolean) (OtherConfigsOut :type "Map of /Game/TankChess/Game/Units/Tanks/Blueprints/BP_BaseTank Object Reference to /Game/TankChess/Game/Units/Tanks/Blueprints/STankConfig Structure"))
  (locals (Tank :type "/Game/TankChess/Game/Units/Tanks/Blueprints/BP_BaseTank Object Reference") (TempTankState :type "/Game/TankChess/Game/Units/Tanks/Blueprints/STankTempState Structure"))
  (bind (_newconfig _possible _outputconfigs) (`self.CalculateMovement` Config (`.Movement_15_9D0598D440526568FDBB37AF3C3EF979` (break `/Game/TankChess/Game/Units/Tanks/Blueprints/STankMove` Move)) OtherConfigs))
  (return _newconfig _possible _outputconfigs))