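; Light tank movement component for TankChess that resolves grid moves and armor hits on tank configs.
; CalculateMovement steps or rotates for one move point, though reversing spends all remaining points; steps require an existing, unoccupied cell with allowed landscape.
; ApplyDamage compares gun power to armor on the struck relative side, killing the tank if power is higher.
; Both return rebuilt config structs, and movement checks cells against supplied edited configs.
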(fn `ApplyDamage`
  (params (Direction :type "/Game/TankChess/Game/Units/Tanks/Blueprints/EDirection Enum" :default "NewEnumerator0") (GunPower :type Integer) (Config :type "/Game/TankChess/Game/Units/Tanks/Blueprints/STankConfig Structure"))
  (returns (Valid :type Boolean) (NewConfig :type "/Game/TankChess/Game/Units/Tanks/Blueprints/STankConfig Structure"))
  (bind (_maincomponentclass _coords _direction _alive) (break `/Game/TankChess/Game/Units/Tanks/Blueprints/STankConfig` Config))
  (bind (_maincomponentclass_2 _coords_2 _direction_2 _alive_2 _side _components _tempstate) (break `/Game/TankChess/Game/Units/Tanks/Blueprints/STankConfig` Config))
  (if _alive
    (bind _diametral (`/Game/TankChess/Game/Units/Tanks/Blueprints/BPFL_TankDataMaps.GetDiametralDirection` Direction))
    (bind _relativedirection (`/Game/TankChess/Game/Units/Tanks/Blueprints/BPFL_TankDataMaps.GetRelativeDirection` _diametral _direction))
    (bind _returnvalue (>= (`BlueprintMapLibrary.Map_Find` (`self.Armor`) _relativedirection) GunPower))
    (return (not _returnvalue) (make `/Game/TankChess/Game/Units/Tanks/Blueprints/STankConfig` _maincomponentclass_2 _coords_2 _direction_2 _returnvalue _side _components _tempstate))
    (else
      (return false Config))))

(fn `CalculateMovement`
  (params (Config :type "/Game/TankChess/Game/Units/Tanks/Blueprints/STankConfig Structure") (Movement :type "/Game/TankChess/Game/Units/UnitComponents/Blueprints/MovementComponents/EMovement Enum" :default "NewEnumerator0") (OtherConfigs :type "Map of /Game/TankChess/Game/Units/Tanks/Blueprints/BP_BaseTank Object Reference to /Game/TankChess/Game/Units/Tanks/Blueprints/STankConfig Structure"))
  (returns (NewConfig :type "/Game/TankChess/Game/Units/Tanks/Blueprints/STankConfig Structure") (Possible :type Boolean) (OutputConfigs :type "Map of /Game/TankChess/Game/Units/Tanks/Blueprints/BP_BaseTank Object Reference to /Game/TankChess/Game/Units/Tanks/Blueprints/STankConfig Structure"))
  (locals (Delta :type "/Game/TankChess/Game/Field/Blueprints/SFieldCellCoords Structure"))
  (bind (_maincomponentclass _coords _direction _alive _side _components _tempstate) (break `/Game/TankChess/Game/Units/Tanks/Blueprints/STankConfig` Config))
  (bind (_maincomponentclass_2 _coords_2 _direction_2 _alive_2 _side_2 _components_2 _tempstate_2) (break `/Game/TankChess/Game/Units/Tanks/Blueprints/STankConfig` (`local.Config`)))
  (bind (_maincomponentclass_3 _coords_3 _direction_3 _alive_3 _side_3 _components_3 _tempstate_3) (break `/Game/TankChess/Game/Units/Tanks/Blueprints/STankConfig` (`local.Config`)))
  (if (> (break `/Game/TankChess/Game/Units/Tanks/Blueprints/STankTempState` _tempstate) 0)
    (switch `/Game/TankChess/Game/Units/UnitComponents/Blueprints/MovementComponents/EMovement` (`local.Movement`)
      (:`NewEnumerator0`
        (bind _delta (`/Game/TankChess/Game/Units/Tanks/Blueprints/BPFL_TankDataMaps.GetDeltaCoordsByDirection` _direction))
        (set `local.Delta` _delta))
      (:`NewEnumerator1`
        (bind _delta_2 (`/Game/TankChess/Game/Units/Tanks/Blueprints/BPFL_TankDataMaps.GetDeltaCoordsByDirection` _direction))
        (set `local.Delta` (`/Game/TankChess/Game/Units/Tanks/Blueprints/BPFL_TankDataMaps.MultiplyCoords` _delta_2 -1)))
      (:`NewEnumerator2`
        (bind _newdirection (`/Game/TankChess/Game/Units/Tanks/Blueprints/BPFL_TankDataMaps.GetDirectionAfterRotate` (`local.Movement`) _direction_2 :!label _label))
        (return (make `/Game/TankChess/Game/Units/Tanks/Blueprints/STankConfig` _maincomponentclass_2 _coords_2 _newdirection _alive_2 _side_2 _components_2 (make `/Game/TankChess/Game/Units/Tanks/Blueprints/STankTempState` (- (break `/Game/TankChess/Game/Units/Tanks/Blueprints/STankTempState` _tempstate_2) 1) (`.CanUse_23_BE99ED37467B2319636ED0A69AB3D10F` (break `/Game/TankChess/Game/Units/Tanks/Blueprints/STankTempState` _tempstate_2)))) true (`local.OtherConfigs`)))
      (:`NewEnumerator3`
        (goto _label)))
    (bind (_tank _landscape _find) (message `/Game/TankChess/Game/BPI_GameStateMain.GetCell` (`GameplayStatics.GetGameState`) (`/Game/TankChess/Game/Units/Tanks/Blueprints/BPFL_TankDataMaps.AddCoords` (`.Coords_11_E825CE4C49EDC82B0C70A68D3435969C` (break `/Game/TankChess/Game/Units/Tanks/Blueprints/STankConfig` (`local.Config`))) (`local.Delta`)) (`local.OtherConfigs`)))
    (if _find
      (if (and (not (`KismetSystemLibrary.IsValid` _tank)) (`KismetArrayLibrary.Array_Contains` (`self.PossibleLandscapes`) _landscape))
        (return (make `/Game/TankChess/Game/Units/Tanks/Blueprints/STankConfig` _maincomponentclass_3 (`/Game/TankChess/Game/Units/Tanks/Blueprints/BPFL_TankDataMaps.AddCoords` _coords_3 (`local.Delta`)) _direction_3 _alive_3 _side_3 _components_3 (make `/Game/TankChess/Game/Units/Tanks/Blueprints/STankTempState` (select `bool` (`|EnumEquality` (`local.Movement`) "NewEnumerator1") :`false` (- (break `/Game/TankChess/Game/Units/Tanks/Blueprints/STankTempState` _tempstate_3) 1)) (`.CanUse_23_BE99ED37467B2319636ED0A69AB3D10F` (break `/Game/TankChess/Game/Units/Tanks/Blueprints/STankTempState` _tempstate_3)))) true (`local.OtherConfigs`))
        (else
          _)))
    (return (struct) false (`local.OtherConfigs`))
    (else
      (return (struct) false (`local.OtherConfigs`)))))