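; BP_RecursiveMovementNode is a search-tree node for computing movement paths of tank units in TankChess.
; Each node stores a movement, the resulting tank configuration and a link to its predecessor.
; MakeChildren tests every EMovement value through the movement component, given other configs, and creates child nodes for the possible ones.
; GetCalculatedWay walks back through predecessors to return the ordered movement list and final tank state.
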(fn `GetCalculatedWay`
  (returns (Way :type "/Game/TankChess/Game/Units/UnitComponents/Blueprints/MovementComponents/SCalculatedWay Structure"))
  (locals (TempNode :type "/Game/TankChess/Game/Units/UnitComponents/Blueprints/MovementComponents/BP_RecursiveMovementNode Object Reference") (Movements :type "Array of /Game/TankChess/Game/Units/UnitComponents/Blueprints/MovementComponents/EMovement Enum"))
  (bind _tempnode (`local.TempNode`))
  (bind _output_get (set `local.TempNode` self))
  (while (`KismetSystemLibrary.IsValid` (`/Game/TankChess/Game/Units/UnitComponents/Blueprints/MovementComponents/BP_RecursiveMovementNode.Prev` _output_get))
    (`KismetArrayLibrary.Array_Insert` (`local.Movements`) (`/Game/TankChess/Game/Units/UnitComponents/Blueprints/MovementComponents/BP_RecursiveMovementNode.Movement` _tempnode))
    (set `local.TempNode` (`/Game/TankChess/Game/Units/UnitComponents/Blueprints/MovementComponents/BP_RecursiveMovementNode.Prev` _tempnode)))
  (return (make `/Game/TankChess/Game/Units/UnitComponents/Blueprints/MovementComponents/SCalculatedWay` (`local.Movements`) (`self.TempConfig`))))

(fn `MakeChildren`
  (params (MoveComponent :type "/Game/TankChess/Game/Units/UnitComponents/Blueprints/MovementComponents/BP_BaseMovementComponent Object Reference") (OtherConfigs :type "Map of /Game/TankChess/Game/Units/Tanks/Blueprints/BP_BaseTank Object Reference to /Game/TankChess/Game/Units/Tanks/Blueprints/STankConfig Structure"))
  (returns (Children :type "Array of /Game/TankChess/Game/Units/UnitComponents/Blueprints/MovementComponents/BP_RecursiveMovementNode Object Reference"))
  (locals (ChildrenArray :type "Array of /Game/TankChess/Game/Units/UnitComponents/Blueprints/MovementComponents/BP_RecursiveMovementNode Object Reference"))
  (bind _enumvalue (foreach `/Game/TankChess/Game/Units/UnitComponents/Blueprints/MovementComponents/EMovement` false)
    (:`LoopBody`
      (bind (_newconfig _possible) (`/Game/TankChess/Game/Units/UnitComponents/Blueprints/MovementComponents/BP_BaseMovementComponent.CalculateMovement` MoveComponent (`self.TempConfig`) _enumvalue OtherConfigs))
      (if _possible
        (bind _returnvalue (`|GenericCreateObject` "BP_RecursiveMovementNode_C"))
        (set `/Game/TankChess/Game/Units/UnitComponents/Blueprints/MovementComponents/BP_RecursiveMovementNode.Movement` _enumvalue _returnvalue)
        (set `/Game/TankChess/Game/Units/UnitComponents/Blueprints/MovementComponents/BP_RecursiveMovementNode.TempConfig` _newconfig _returnvalue)
        (set `/Game/TankChess/Game/Units/UnitComponents/Blueprints/MovementComponents/BP_RecursiveMovementNode.Prev` self _returnvalue)
        (`KismetArrayLibrary.Array_Add` (`local.ChildrenArray`) _returnvalue)))
    (:`then`
      (return (`local.ChildrenArray`)))))