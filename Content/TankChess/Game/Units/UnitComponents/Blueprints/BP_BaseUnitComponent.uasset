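; Base component for units in TankChess, defining the shared interface for validating and making moves.
; ValidateMove rejects actions outside PossibleActions, and moves naming an active component class that this component's class does not derive from.
; Accepted moves pass to ValidateMoveInternal with a temp state, a template-method hook that returns invalid by default.
; MakeMove, AddOwner and RemoveOwner are empty stubs.
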(fn `AddOwner`
  (params (Owner :type "/Game/TankChess/Game/Units/Tanks/Blueprints/BP_BaseTank Object Reference")))

(fn `MakeMove`
  (params (Move :type "/Game/TankChess/Game/Units/Tanks/Blueprints/STankMove Structure") (TempState :type "/Game/TankChess/Game/Units/Tanks/Blueprints/STankTempState Structure"))
  (returns (NewTempState :type "/Game/TankChess/Game/Units/Tanks/Blueprints/STankTempState Structure"))
  (return))

(fn `RemoveOwner`
  (params (Owner :type "/Game/TankChess/Game/Units/Tanks/Blueprints/BP_BaseTank Object Reference")))

(fn `ValidateMove`
  (params (Move :type "/Game/TankChess/Game/Units/Tanks/Blueprints/STankMove Structure") (TempState :type "/Game/TankChess/Game/Units/Tanks/Blueprints/STankTempState Structure"))
  (returns (IsValid :type Boolean) (NewTempState :type "/Game/TankChess/Game/Units/Tanks/Blueprints/STankTempState Structure"))
  (bind (_action _activecomponent) (break `/Game/TankChess/Game/Units/Tanks/Blueprints/STankMove` Move))
  (if (or (not (`KismetArrayLibrary.Array_Contains` (`self.PossibleActions`) _action)) (and (`KismetSystemLibrary.IsValidClass` _activecomponent) (not (`KismetMathLibrary.ClassIsChildOf` (`GameplayStatics.GetObjectClass` self) _activecomponent))))
    (return false)
    (else
      (bind (_isvalid _newtempstate) (`self.ValidateMove_internal` Move TempState))
      (return _isvalid _newtempstate))))

(fn `ValidateMove_internal`
  (params (Move :type "/Game/TankChess/Game/Units/Tanks/Blueprints/STankMove Structure") (TempState :type "/Game/TankChess/Game/Units/Tanks/Blueprints/STankTempState Structure"))
  (returns (IsValid :type Boolean) (NewTempState :type "/Game/TankChess/Game/Units/Tanks/Blueprints/STankTempState Structure"))
  (return false))