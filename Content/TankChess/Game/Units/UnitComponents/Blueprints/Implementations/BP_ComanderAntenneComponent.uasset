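; BP_ComanderAntenneComponent is a TankChess unit component that gives its owning unit a commander antenna and access to one more landscape type.
; AddOwner shows the owner's CommanderAntenne, gets the movement component through the ItemManager and adds the landscape to its PossibleLandscapes.
; RemoveOwner reverses both changes, hiding the antenna and removing that landscape.
; Both overrides call their parent first.
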(fn `AddOwner`
  (params (Owner :type "/Game/TankChess/Game/Units/Tanks/Blueprints/BP_BaseTank Object Reference"))
  (`parent.AddOwner` Owner)
  (`SceneComponent.SetVisibility` (`/Game/TankChess/Game/Units/Tanks/Blueprints/BP_BaseTank.CommanderAntenne` Owner) true false)
  (bind _component (`/Game/TankChess/Game/Units/UnitComponents/Blueprints/BP_UnitComponentManagerComponent.GetComponent` (`/Game/TankChess/Game/Units/Tanks/Blueprints/BP_BaseTank.ItemManager` (`local.Owner`)) (make `/Game/TankChess/Game/Units/Tanks/Blueprints/STankMove` "NewEnumerator4" "/Game/TankChess/Game/Units/UnitComponents/Blueprints/Implementations/MovementComponents/BP_BaseMovementComponent.BP_BaseMovementComponent_C" (struct :`Coords` (struct) :`Direction` "NewEnumerator0"))))
  (bind _asbp_base_movement_component (cast `/Game/TankChess/Game/Units/UnitComponents/Blueprints/Implementations/MovementComponents/BP_BaseMovementComponent` _component))
  (`KismetArrayLibrary.Array_AddUnique` (`/Game/TankChess/Game/Units/UnitComponents/Blueprints/Implementations/MovementComponents/BP_BaseMovementComponent.PossibleLandscapes` _asbp_base_movement_component) "NewEnumerator3"))

(fn `RemoveOwner`
  (params (Owner :type "/Game/TankChess/Game/Units/Tanks/Blueprints/BP_BaseTank Object Reference"))
  (`parent.RemoveOwner` Owner)
  (`SceneComponent.SetVisibility` (`/Game/TankChess/Game/Units/Tanks/Blueprints/BP_BaseTank.CommanderAntenne` Owner) false false)
  (bind _component (`/Game/TankChess/Game/Units/UnitComponents/Blueprints/BP_UnitComponentManagerComponent.GetComponent` (`/Game/TankChess/Game/Units/Tanks/Blueprints/BP_BaseTank.ItemManager` Owner) (make `/Game/TankChess/Game/Units/Tanks/Blueprints/STankMove` "NewEnumerator4" "/Game/TankChess/Game/Units/UnitComponents/Blueprints/Implementations/MovementComponents/BP_BaseMovementComponent.BP_BaseMovementComponent_C" (struct :`Coords` (struct) :`Direction` "NewEnumerator0"))))
  (bind _asbp_base_movement_component (cast `/Game/TankChess/Game/Units/UnitComponents/Blueprints/Implementations/MovementComponents/BP_BaseMovementComponent` _component))
  (`KismetArrayLibrary.Array_RemoveItem` (`/Game/TankChess/Game/Units/UnitComponents/Blueprints/Implementations/MovementComponents/BP_BaseMovementComponent.PossibleLandscapes` _asbp_base_movement_component) "NewEnumerator3"))