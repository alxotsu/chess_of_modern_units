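; Main tank movement component that validates grid moves and finds ways to a target cell for each final facing.
; CalculateWays expands recursive movement nodes breadth-first through a growing array, keeping the way with the most remaining move points per direction.
; CalculateMovement simulates one step, blocking disallowed landscapes, occupied cells and same-side base cells.
; Forward steps and turns cost one point, while reversing spends all remaining points.
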(fn `CalculateMovement`
  (params (TempState :type "/Game/TankChess/Game/Units/Tanks/Blueprints/STankTempState Structure") (Movement :type "/Game/TankChess/Game/Units/UnitComponents/Blueprints/Implementations/MovementComponents/EMovement Enum" :default "NewEnumerator0"))
  (returns (NewTempState :type "/Game/TankChess/Game/Units/Tanks/Blueprints/STankTempState Structure") (IsPossible :type Boolean))
  (locals (Delta :type "/Game/TankChess/Game/Field/Blueprints/SFieldCellCoords Structure") (OutputState :type "/Game/TankChess/Game/Units/Tanks/Blueprints/STankTempState Structure"))
  (bind (_coords _direction _alive _movepoints _canattack) (break `/Game/TankChess/Game/Units/Tanks/Blueprints/STankTempState` (`local.TempState`)))
  (bind (_coords_2 _direction_2 _alive_2 _movepoints_2 _canattack_2) (break `/Game/TankChess/Game/Units/Tanks/Blueprints/STankTempState` (`local.TempState`)))
  (bind (_coords_3 _direction_3) (break `/Game/TankChess/Game/Units/Tanks/Blueprints/STankTempState` (`local.TempState`)))
  (if (> (`.MovePoints_6_9A2DC2C14EF4D5B31385F79E3D7ABDDF` (break `/Game/TankChess/Game/Units/Tanks/Blueprints/STankTempState` TempState)) 0)
    (switch `/Game/TankChess/Game/Units/UnitComponents/Blueprints/Implementations/MovementComponents/EMovement` (`local.Movement`)
      (:`NewEnumerator0`
        (bind _delta (`/Game/TankChess/Game/Units/Tanks/Blueprints/BPFL_TankDataMaps.GetDeltaCoordsByDirection` _direction_3))
        (set `local.Delta` _delta)
        (bind (_cell _find) (message `/Game/TankChess/Game/BPI_GsmeStateMain.GetCell` (`GameplayStatics.GetGameState`) (`/Game/TankChess/Game/Units/Tanks/Blueprints/BPFL_TankDataMaps.AddCoords` (`.Coords_8_936E25CA4A7D91E89559729E7B48FC8A` (break `/Game/TankChess/Game/Units/Tanks/Blueprints/STankTempState` (`local.TempState`))) (`local.Delta`)) :!label _label))
        (if _find
          (bind _asbp_cell_base (cast `/Game/TankChess/Game/Field/Blueprints/BP_CellBase` _cell)
            (:`then`
              (bind _asbp_base_tank (cast `/Game/TankChess/Game/Units/Tanks/Blueprints/BP_BaseTank` (`self.GetOwner`)))
              (if (not (`|EnumEquality` (`/Game/TankChess/Game/Units/Tanks/Blueprints/BP_BaseTank.Side` _asbp_base_tank) (`/Game/TankChess/Game/Field/Blueprints/BP_CellBase.OwnerSide` _asbp_cell_base)))
                (if (and (`KismetArrayLibrary.Array_Contains` (`self.PossibleLandscapes`) (`/Game/TankChess/Game/Field/Blueprints/BP_Cell.Landscape` _cell)) (not (`KismetSystemLibrary.IsValid` (`/Game/TankChess/Game/Field/Blueprints/BP_Cell.Tank` _cell)))) :!label _label_2
                  (set `local.OutputState` (make `/Game/TankChess/Game/Units/Tanks/Blueprints/STankTempState` (`/Game/TankChess/Game/Units/Tanks/Blueprints/BPFL_TankDataMaps.AddCoords` _coords_2 (`local.Delta`)) _direction_2 _alive_2 (select `bool` (`|EnumEquality` (`local.Movement`) "NewEnumerator1") :`false` (- _movepoints_2 1)) _canattack_2))
                  (return (`local.OutputState`) true))))
            (:`CastFailed`
              (goto _label_2)))))
      (:`NewEnumerator1`
        (bind _delta_2 (`/Game/TankChess/Game/Units/Tanks/Blueprints/BPFL_TankDataMaps.GetDeltaCoordsByDirection` _direction_3))
        (set `local.Delta` (`/Game/TankChess/Game/Units/Tanks/Blueprints/BPFL_TankDataMaps.MultiplyCoords` _delta_2 -1))
        (goto _label))
      (:`NewEnumerator2`
        (bind _newdirection (`/Game/TankChess/Game/Units/Tanks/Blueprints/BPFL_TankDataMaps.GetDirectionAfterRotate` (`local.Movement`) (`.Direction_10_8B0820AD4CC46A6F3B6CE0889A8B0FBE` (break `/Game/TankChess/Game/Units/Tanks/Blueprints/STankTempState` (`local.TempState`))) :!label _label_3))
        (set `local.OutputState` (make `/Game/TankChess/Game/Units/Tanks/Blueprints/STankTempState` _coords _newdirection _alive (- _movepoints 1) _canattack))
        (return (`local.OutputState`) true))
      (:`NewEnumerator3`
        (goto _label_3)))))

(fn `CalculateWays`
  (params (TempState :type "/Game/TankChess/Game/Units/Tanks/Blueprints/STankTempState Structure") (TargetCoords :type "/Game/TankChess/Game/Field/Blueprints/SFieldCellCoords Structure"))
  (returns (Ways :type "Map of /Game/TankChess/Game/Units/Tanks/Blueprints/EDirection Enum to /Game/TankChess/Game/Units/UnitComponents/Blueprints/Implementations/MovementComponents/SCalculatedWay Structure"))
  (locals (NodesForCheck :type "Array of /Game/TankChess/Game/Units/UnitComponents/Blueprints/Implementations/MovementComponents/BP_RecursiveMovementNode Object Reference") (OutputWays :type "Map of /Game/TankChess/Game/Units/Tanks/Blueprints/EDirection Enum to /Game/TankChess/Game/Units/UnitComponents/Blueprints/Implementations/MovementComponents/SCalculatedWay Structure") (MaxPoints :type "Map of /Game/TankChess/Game/Units/Tanks/Blueprints/EDirection Enum to Integer"))
  (bind _returnvalue (`|GenericCreateObject` "/Game/TankChess/Game/Units/UnitComponents/Blueprints/Implementations/MovementComponents/BP_RecursiveMovementNode.BP_RecursiveMovementNode_C"))
  (set `/Game/TankChess/Game/Units/UnitComponents/Blueprints/Implementations/MovementComponents/BP_RecursiveMovementNode.TempState` TempState _returnvalue)
  (bind _children (`/Game/TankChess/Game/Units/UnitComponents/Blueprints/Implementations/MovementComponents/BP_RecursiveMovementNode.MakeChildren` _returnvalue self))
  (bind _output_get (set `local.NodesForCheck` _children))
  (for _array_element _output_get
    (bind _tempstate (`/Game/TankChess/Game/Units/UnitComponents/Blueprints/Implementations/MovementComponents/BP_RecursiveMovementNode.TempState` _array_element))
    (if (`self.Check Different with Start Position` _tempstate)
      (bind (_coords _direction _alive _movepoints) (break `/Game/TankChess/Game/Units/Tanks/Blueprints/STankTempState` _tempstate))
      (if (and (`/Game/TankChess/Game/Units/Tanks/Blueprints/BPFL_TankDataMaps.EqualCoords` _coords (`local.TargetCoords`)) (> _movepoints (`BlueprintMapLibrary.Map_Find` (`local.MaxPoints`) _direction)))
        (`BlueprintMapLibrary.Map_Add` (`local.MaxPoints`) _direction _movepoints)
        (bind _way (`/Game/TankChess/Game/Units/UnitComponents/Blueprints/Implementations/MovementComponents/BP_RecursiveMovementNode.GetCalculatedWay` _array_element))
        (`BlueprintMapLibrary.Map_Add` (`local.OutputWays`) _direction _way))
      (bind _children_2 (`/Game/TankChess/Game/Units/UnitComponents/Blueprints/Implementations/MovementComponents/BP_RecursiveMovementNode.MakeChildren` _array_element self))
      (`KismetArrayLibrary.Array_Append` (`local.NodesForCheck`) _children_2)))
  (return (`local.OutputWays`)))