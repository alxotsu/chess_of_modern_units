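; Base movement component for TankChess tanks that validates and executes Move actions on the owning BP_BaseTank.
; A move either replays its movement steps on a temporary tank state, or, without steps, looks up ways to the target coords by final direction.
; Step-based validation rejects impossible steps and unchanged end poses; execution applies the resulting coords and direction.
; CalculateMovement and CalculateWays are empty stubs, leaving movement rules to subclasses.
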(fn `CalculateMovement`
  (params (TempState :type "/Game/TankChess/Game/Units/Tanks/Blueprints/STankTempState Structure") (Movement :type "/Game/TankChess/Game/Units/UnitComponents/Blueprints/Implementations/MovementComponents/EMovement Enum" :default "NewEnumerator0"))
  (returns (NewTempState :type "/Game/TankChess/Game/Units/Tanks/Blueprints/STankTempState Structure") (IsPossible :type Boolean))
  (return (struct) false))

(fn `CalculateWays`
  (params (TempState :type "/Game/TankChess/Game/Units/Tanks/Blueprints/STankTempState Structure") (TargetCoords :type "/Game/TankChess/Game/FieldCell/Blueprints/SFieldCellCoords Structure"))
  (returns (Ways :type "Map of /Game/TankChess/Game/Units/Tanks/Blueprints/EDirection Enum to /Game/TankChess/Game/Units/UnitComponents/Blueprints/Implementations/MovementComponents/SCalculatedWay Structure"))
  (return))

(fn `Check Different with Start Position`
  (params (FinalState :type "/Game/TankChess/Game/Units/Tanks/Blueprints/STankTempState Structure (by ref)"))
  (returns (IsDifferent :type Boolean))
  (bind (_coords _direction) (break `/Game/TankChess/Game/Units/Tanks/Blueprints/STankTempState` FinalState))
  (bind _asbp_base_tank (cast `/Game/TankChess/Game/Units/Tanks/Blueprints/BP_BaseTank` (`self.GetOwner`)))
  (bind (_coords_2 _direction_2) (break `/Game/TankChess/Game/Units/Tanks/Blueprints/STankTempState` (`/Game/TankChess/Game/Units/Tanks/Blueprints/BP_BaseTank.GetTempState` _asbp_base_tank)))
  (return (not (and (`/Game/TankChess/Game/Units/Tanks/Blueprints/BPFL_TankDataMaps.EqualCoords` _coords_2 _coords) (`|EnumEquality` _direction_2 _direction)))))

(fn `MakeMove`
  (params (Move :type "/Game/TankChess/Game/Units/Tanks/Blueprints/STankMove Structure") (TempState :type "/Game/TankChess/Game/Units/Tanks/Blueprints/STankTempState Structure"))
  (returns (NewTempState :type "/Game/TankChess/Game/Units/Tanks/Blueprints/STankTempState Structure"))
  (locals (Tank :type "/Game/TankChess/Game/Units/Tanks/Blueprints/BP_BaseTank Object Reference") (TempTankState :type "/Game/TankChess/Game/Units/Tanks/Blueprints/STankTempState Structure"))
  (bind (_action _activecomponent _params) (break `/Game/TankChess/Game/Units/Tanks/Blueprints/STankMove` Move))
  (bind _tank (`local.Tank`))
  (bind _temptankstate (`local.TempTankState`))
  (bind _tank_2 (`local.Tank`))
  (bind (_coords _direction _target _movements) (break `/Game/TankChess/Game/Units/Tanks/Blueprints/STankMoveParams` _params))
  (bind (_coords_2 _direction_2) (break `/Game/TankChess/Game/Units/Tanks/Blueprints/STankTempState` _temptankstate))
  (switch `/Game/TankChess/Game/Units/UnitComponents/Blueprints/EUnitAction` _action
    (:`NewEnumerator5`
      (bind _asbp_base_tank (cast `/Game/TankChess/Game/Units/Tanks/Blueprints/BP_BaseTank` (`self.GetOwner`)))
      (set `local.Tank` _asbp_base_tank)
      (if (`KismetArrayLibrary.Array_IsEmpty` _movements)
        (bind _ways (`self.CalculateWays` TempState _coords))
        (bind (_movements_2 _tankstateatend) (break `/Game/TankChess/Game/Units/UnitComponents/Blueprints/Implementations/MovementComponents/SCalculatedWay` (`BlueprintMapLibrary.Map_Find` _ways _direction)))
        (bind (_coords_3 _direction_3) (break `/Game/TankChess/Game/Units/Tanks/Blueprints/STankTempState` _tankstateatend))
        (`/Game/TankChess/Game/Units/Tanks/Blueprints/BP_BaseTank.SetCoords` _tank_2 _coords_3)
        (`/Game/TankChess/Game/Units/Tanks/Blueprints/BP_BaseTank.SetDirection` _tank_2 _direction_3)
        (return _tankstateatend)
        (else
          (set `local.TempTankState` (`local.TempState`))
          (for _array_element _movements
            (bind _newtempstate (`self.CalculateMovement` (`local.TempTankState`) _array_element))
            (set `local.TempTankState` _newtempstate))
          (`/Game/TankChess/Game/Units/Tanks/Blueprints/BP_BaseTank.SetCoords` _tank _coords_2)
          (`/Game/TankChess/Game/Units/Tanks/Blueprints/BP_BaseTank.SetDirection` _tank _direction_2)
          (return _temptankstate))))))

(fn `ValidateMove_internal`
  (params (Move :type "/Game/TankChess/Game/Units/Tanks/Blueprints/STankMove Structure") (TempState :type "/Game/TankChess/Game/Units/Tanks/Blueprints/STankTempState Structure"))
  (returns (IsValid :type Boolean) (NewTempState :type "/Game/TankChess/Game/Units/Tanks/Blueprints/STankTempState Structure"))
  (locals (LocalState :type "/Game/TankChess/Game/Units/Tanks/Blueprints/STankTempState Structure"))
  (bind (_action _activecomponent _params) (break `/Game/TankChess/Game/Units/Tanks/Blueprints/STankMove` Move))
  (bind (_coords _direction _target _movements) (break `/Game/TankChess/Game/Units/Tanks/Blueprints/STankMoveParams` _params))
  (switch `/Game/TankChess/Game/Units/UnitComponents/Blueprints/EUnitAction` _action
    (:`NewEnumerator5`
      (if (`KismetArrayLibrary.Array_IsNotEmpty` _movements)
        (set `local.LocalState` (`local.TempState`))
        (for _array_element _movements
          (bind (_newtempstate _ispossible) (`self.CalculateMovement` (`local.LocalState`) _array_element))
          (if _ispossible
            (set `local.LocalState` _newtempstate)
            (else
              (return false))))
        (return (`self.Check Different with Start Position` (`local.LocalState`)) (`local.LocalState`))
        (else
          (bind _ways (`self.CalculateWays` TempState _coords))
          (bind (_value _returnvalue) (`BlueprintMapLibrary.Map_Find` _ways _direction))
          (return _returnvalue (`.TankStateAtEnd_7_387AC2E64E0FC3B2DE6F94B074C7DC27` (break `/Game/TankChess/Game/Units/UnitComponents/Blueprints/Implementations/MovementComponents/SCalculatedWay` _value))))))))