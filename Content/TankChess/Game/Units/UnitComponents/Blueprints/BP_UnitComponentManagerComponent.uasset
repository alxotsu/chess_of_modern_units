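; Actor component that manages the item components equipped on a tank unit.
; AddItem and RemoveItem create or destroy components on the owner by class, allowing one per class, track them in the Items set and register or unregister the owning BP_BaseTank.
; GetComponent resolves a Move to its component, using the move's ActiveComponent class if valid, otherwise the first item whose PossibleActions contains the move's action.
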(fn `AddItem`
  (params (Item :type "/Game/TankChess/Game/Units/UnitComponents/Blueprints/BP_BaseUnitComponent Class Reference"))
  (bind _returnvalue (`self.GetOwner`))
  (if (not (`self.ItemEquiped` Item))
    (bind _returnvalue_2 (`|AddComponentByClass` _returnvalue Item))
    (`BlueprintSetLibrary.Set_Add` (`self.Items`) _returnvalue_2)
    (bind _asbp_base_tank (cast `/Game/TankChess/Game/Units/Tanks/Blueprints/BP_BaseTank` _returnvalue))
    (`/Game/TankChess/Game/Units/UnitComponents/Blueprints/BP_BaseUnitComponent.AddOwner` _returnvalue_2 _asbp_base_tank)))

(fn `GetComponent`
  (params (Move :type "/Game/TankChess/Game/Units/Tanks/Blueprints/STankMove Structure"))
  (returns (Component :type "/Game/TankChess/Game/Units/UnitComponents/Blueprints/BP_BaseUnitComponent Object Reference"))
  (bind (_action _activecomponent) (break `/Game/TankChess/Game/Units/Tanks/Blueprints/STankMove` Move))
  (if (`KismetSystemLibrary.IsValidClass` _activecomponent)
    (return (`Actor.GetComponentByClass` (`self.GetOwner`) _activecomponent))
    (else
      (bind _result (`BlueprintSetLibrary.Set_ToArray` (`self.Items`)))
      (for _array_element _result
        (if (`KismetArrayLibrary.Array_Contains` (`/Game/TankChess/Game/Units/UnitComponents/Blueprints/BP_BaseUnitComponent.PossibleActions` _array_element) (`.Action_8_E01479DF4968718A51B1E6A6220B5AD6` (break `/Game/TankChess/Game/Units/Tanks/Blueprints/STankMove` Move)))
          (return _array_element))))))

(fn `ItemEquiped`
  (params (Item :type "/Game/TankChess/Game/Units/UnitComponents/Blueprints/BP_BaseUnitComponent Class Reference"))
  (returns (Equiped :type Boolean))
  (return (`KismetSystemLibrary.IsValid` (`Actor.GetComponentByClass` (`self.GetOwner`) Item))))

(fn `RemoveItem`
  (params (Item :type "/Game/TankChess/Game/Units/UnitComponents/Blueprints/BP_BaseUnitComponent Class Reference"))
  (bind _returnvalue (`self.GetOwner`))
  (bind _returnvalue_2 (`Actor.GetComponentByClass` _returnvalue Item))
  (if (`self.ItemEquiped` Item)
    (`BlueprintSetLibrary.Set_Remove` (`self.Items`) _returnvalue_2)
    (bind _asbp_base_tank (cast `/Game/TankChess/Game/Units/Tanks/Blueprints/BP_BaseTank` _returnvalue)
      (:`then`
        (`/Game/TankChess/Game/Units/UnitComponents/Blueprints/BP_BaseUnitComponent.RemoveOwner` _returnvalue_2 _asbp_base_tank))
      (:`CastFailed`
        _))
    (`self.K2_DestroyComponent` _returnvalue_2)))