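; Tank chess unit that builds and displays itself from its UnitConfig, starting in the construction script.
; Setters update the config and visuals: DT_UnitModules meshes on sockets, grid position, facing, tipped mesh when dead, and side color via dynamic materials.
; VisualizeMoves delegates each move to the active module's behavior class, added as a short-lived component and destroyed after the call.
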(fn `SetAlive`
  (params (Alive :type Boolean))
  (bind (_unit_config_mainmodule _unit_config_moduleonsockets _unit_config_coords _unit_config_direction _unit_config_alive _unit_config_side _unit_config_tempstate) (break `/Game/TankChess/Game/Units/Blueprints/SUnitConfig` (`self.Unit Config`)))
  (set `self.Unit Config` (make `/Game/TankChess/Game/Units/Blueprints/SUnitConfig` _unit_config_mainmodule _unit_config_moduleonsockets _unit_config_coords _unit_config_direction Alive _unit_config_side _unit_config_tempstate))
  (`SceneComponent.K2_SetRelativeRotation` (`self.Mesh`) (`KismetMathLibrary.MakeRotator` (select `bool` Alive :`false` 90.0 :!type "Float (single-precision)")) false false))

(fn `SetCoords`
  (params (Coords :type "/Game/TankChess/Game/Field/Blueprints/SFieldCellCoords Structure"))
  (bind (_xcoord _ycoord) (break `/Game/TankChess/Game/Field/Blueprints/SFieldCellCoords` Coords))
  (bind (_unit_config_mainmodule _unit_config_moduleonsockets _unit_config_coords _unit_config_direction _unit_config_alive _unit_config_side _unit_config_tempstate) (break `/Game/TankChess/Game/Units/Blueprints/SUnitConfig` (`self.Unit Config`)))
  (set `self.Unit Config` (make `/Game/TankChess/Game/Units/Blueprints/SUnitConfig` _unit_config_mainmodule _unit_config_moduleonsockets Coords _unit_config_direction _unit_config_alive _unit_config_side _unit_config_tempstate))
  (`SceneComponent.K2_SetWorldLocation` (`self.CapsuleComponent`) (`KismetMathLibrary.MakeVector` (`KismetMathLibrary.Conv_IntToDouble` (* _xcoord 100)) (`KismetMathLibrary.Conv_IntToDouble` (* _ycoord 100))) false false))

(fn `SetDirection`
  (params (Direction :type "/Game/TankChess/Game/Units/Blueprints/EDirection Enum" :default "NewEnumerator0"))
  (locals (RotateForDirection :type "Map of /Game/TankChess/Game/Units/Blueprints/EDirection Enum to Float (double-precision)"))
  (bind (_unit_config_mainmodule _unit_config_moduleonsockets _unit_config_coords _unit_config_direction _unit_config_alive _unit_config_side _unit_config_tempstate) (break `/Game/TankChess/Game/Units/Blueprints/SUnitConfig` (`self.Unit Config`)))
  (bind _capsulecomponent (`self.CapsuleComponent`))
  (bind (_returnvalue_roll _returnvalue_pitch) (`KismetMathLibrary.BreakRotator` (`SceneComponent.K2_GetComponentRotation` _capsulecomponent)))
  (set `self.Unit Config` (make `/Game/TankChess/Game/Units/Blueprints/SUnitConfig` _unit_config_mainmodule _unit_config_moduleonsockets _unit_config_coords Direction _unit_config_alive _unit_config_side _unit_config_tempstate))
  (`SceneComponent.K2_SetWorldRotation` _capsulecomponent (`KismetMathLibrary.MakeRotator` _returnvalue_roll _returnvalue_pitch (`BlueprintMapLibrary.Map_Find` (`local.RotateForDirection`) Direction)) false false))

(fn `SetSide`
  (params (Side :type "/Game/TankChess/Game/Player/EPlayerSide Enum" :default "NewEnumerator0"))
  (locals (Color :type "LinearColor Structure") (DynmMI :type "MaterialInstanceDynamic Object Reference"))
  (bind (_unit_config_mainmodule _unit_config_moduleonsockets _unit_config_coords _unit_config_direction _unit_config_alive _unit_config_side _unit_config_tempstate) (break `/Game/TankChess/Game/Units/Blueprints/SUnitConfig` (`self.Unit Config`)))
  (bind _dynmmi (`local.DynmMI`))
  (set `self.Unit Config` (make `/Game/TankChess/Game/Units/Blueprints/SUnitConfig` _unit_config_mainmodule _unit_config_moduleonsockets _unit_config_coords _unit_config_direction _unit_config_alive Side _unit_config_tempstate))
  (set `local.Color` (select `/Game/TankChess/Game/Player/EPlayerSide` Side :`NewEnumerator1` (struct :`R` 1.0 :`G` 1.0 :`B` 1.0 :`A` 1.0) :!type "LinearColor Structure"))
  (for _array_element (`self.K2_GetComponentsByClass` "/Script/Engine.SkeletalMeshComponent")
    (for _index (range (`PrimitiveComponent.GetNumMaterials` _array_element))
      (bind _returnvalue (`PrimitiveComponent.GetMaterial` _array_element _index))
      (bind _asmaterial_instance_dynamic (cast `MaterialInstanceDynamic` _returnvalue)
        (:`then`
          (set `local.DynmMI` _asmaterial_instance_dynamic))
        (:`CastFailed`
          (bind _returnvalue_2 (`KismetMaterialLibrary.CreateDynamicMaterialInstance` _returnvalue))
          (set `local.DynmMI` _returnvalue_2)))
      (`MaterialInstanceDynamic.SetVectorParameterValue` _dynmmi "SideColor" (`local.Color`))
      (`PrimitiveComponent.SetMaterial` _array_element _index _dynmmi))))

(fn `SetUpModules`
  (params (MainModule :type Name) (ModuleOnSockets :type "Map of Name to Name"))
  (bind (_unit_config_mainmodule _unit_config_moduleonsockets _unit_config_coords _unit_config_direction _unit_config_alive _unit_config_side _unit_config_tempstate) (break `/Game/TankChess/Game/Units/Blueprints/SUnitConfig` (`self.Unit Config`)))
  (bind _moduleonsockets (`local.ModuleOnSockets`))
  (set `self.Unit Config` (make `/Game/TankChess/Game/Units/Blueprints/SUnitConfig` MainModule ModuleOnSockets _unit_config_coords _unit_config_direction _unit_config_alive _unit_config_side _unit_config_tempstate))
  (`ActorComponent.K2_DestroyComponent` (`SceneComponent.GetChildrenComponents` (`self.Mesh`) false))
  (bind _returnvalue (`|GetDataTableRow` "/Game/TankChess/Game/Units/Blueprints/Modules/DT_UnitModules.DT_UnitModules" (`local.MainModule`))
    (:`then`
      (`SkeletalMeshComponent.SetSkeletalMeshAsset` (`self.Mesh`) (`.SkeletalMesh_7_2A2D0F5A4F381951D55B90AC50BD1F5D` (break `/Game/TankChess/Game/Units/Blueprints/Modules/TableStructures/SModuleDescription` _returnvalue)))
      (bind _keys (`BlueprintMapLibrary.Map_Keys` _moduleonsockets))
      (for _array_element _keys
        (bind _returnvalue_2 (`|GetDataTableRow` "/Game/TankChess/Game/Units/Blueprints/Modules/DT_UnitModules.DT_UnitModules" (`BlueprintMapLibrary.Map_Find` _moduleonsockets _array_element))
          (:`then`
            (bind _returnvalue_3 (`AddComponent|NODE_AddSkeletalMeshComponent-0`))
            (`SkeletalMeshComponent.SetSkeletalMeshAsset` _returnvalue_3 (`.SkeletalMesh_7_2A2D0F5A4F381951D55B90AC50BD1F5D` (break `/Game/TankChess/Game/Units/Blueprints/Modules/TableStructures/SModuleDescription` _returnvalue_2)))
            (`SceneComponent.K2_AttachToComponent` _returnvalue_3 (`self.Mesh`) _array_element "KeepRelative" "KeepRelative" "KeepRelative" true)))))))

(fn `UserConstructionScript`
  (`self.VisualizeConfig` (`self.Unit Config`)))

(fn `VisualizeConfig`
  (params (UnitConfig :type "/Game/TankChess/Game/Units/Blueprints/SUnitConfig Structure"))
  (bind (_mainmodule _moduleonsockets _coords _direction _alive _side) (break `/Game/TankChess/Game/Units/Blueprints/SUnitConfig` UnitConfig))
  (`|ExecutionSequence`
    (:`then_0`
      (`self.SetUpModules` _mainmodule _moduleonsockets))
    (:`then_1`
      (`self.SetCoords` _coords))
    (:`then_2`
      (`self.SetDirection` _direction))
    (:`then_3`
      (`self.SetAlive` _alive))
    (:`then_4`
      (`self.SetSide` _side))))

(fn `VisualizeMoves`
  (params (Moves :type "Array of /Game/TankChess/Game/Units/Blueprints/SUnitMove Structure"))
  (locals (ModuleClass :type "/Game/TankChess/Game/Units/Blueprints/Modules/BP_BaseUnitModuleComponent Class Reference"))
  (bind (_unit_config_mainmodule _unit_config_moduleonsockets) (break `/Game/TankChess/Game/Units/Blueprints/SUnitConfig` (`self.Unit Config`)))
  (for _array_element Moves
    (bind _activecomponent (break `/Game/TankChess/Game/Units/Blueprints/SUnitMove` _array_element))
    (if (== _activecomponent "Main")
      (bind _returnvalue (`|GetDataTableRow` "/Game/TankChess/Game/Units/Blueprints/Modules/DT_UnitModules.DT_UnitModules" _unit_config_mainmodule)
        (:`then`
          (set `local.ModuleClass` (break `/Game/TankChess/Game/Units/Blueprints/Modules/TableStructures/SModuleDescription` _returnvalue))))
      (else
        (bind _returnvalue_2 (`|GetDataTableRow` "/Game/TankChess/Game/Units/Blueprints/Modules/DT_UnitModules.DT_UnitModules" (`BlueprintMapLibrary.Map_Find` _unit_config_moduleonsockets _activecomponent))
          (:`then`
            (set `local.ModuleClass` (break `/Game/TankChess/Game/Units/Blueprints/Modules/TableStructures/SModuleDescription` _returnvalue_2))))))
    (bind _returnvalue_3 (`|AddComponentByClass` (`local.ModuleClass`) _activecomponent))
    (`/Game/TankChess/Game/Units/Blueprints/Modules/BP_BaseUnitModuleComponent.VisualizeMove` _returnvalue_3 _array_element)
    (`ActorComponent.K2_DestroyComponent` _returnvalue_3)))