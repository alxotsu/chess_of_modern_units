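; Movement module component for TankChess grid units, handling steps, turns and directional armor checks.
; ComputeMove returns a new field state after checking move points, occupancy and DT_UnitModules landscape types; base cells require matching ownership and an antenna module, and reversing spends all points.
; GetPossibleMoves filters every movement through ComputeMove, while VisualizeMove separately updates the owning BP_Unit.
; ApplyDamage succeeds only when firepower exceeds armor on the struck side.
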(fn `ApplyDamage`
  (params (FirePower :type Integer) (Direction :type "/Game/TankChess/Game/Units/Blueprints/EDirection Enum" :default "NewEnumerator0") (UnitConfig :type "/Game/TankChess/Game/Units/Blueprints/SUnitConfig Structure"))
  (returns (NewUnitConfig :type "/Game/TankChess/Game/Units/Blueprints/SUnitConfig Structure") (Possible :type Boolean))
  (bind (_mainmodule _moduleonsockets _coords _direction _alive _side _tempstate) (break `/Game/TankChess/Game/Units/Blueprints/SUnitConfig` UnitConfig))
  (bind _diametral (`/Game/TankChess/Game/Units/Blueprints/BPFL_CoordsAndDirectionTransforms.GetDiametralDirection` Direction))
  (bind _returnvalue (`|GetDataTableRow` "/Game/TankChess/Game/Units/Blueprints/Modules/DT_UnitModules.DT_UnitModules" _mainmodule)
    (:`then`
      (bind _relativedirection (`/Game/TankChess/Game/Units/Blueprints/BPFL_CoordsAndDirectionTransforms.GetRelativeDirection` _direction _diametral))
      (if (> FirePower (`BlueprintMapLibrary.Map_Find` (break `/Game/TankChess/Game/Units/Blueprints/Modules/TableStructures/SModuleSettings` (`.Settings_12_A8061B9948A0E1B34868A88E70641730` (break `/Game/TankChess/Game/Units/Blueprints/Modules/TableStructures/SModuleDescription` _returnvalue))) _relativedirection))
        (return (make `/Game/TankChess/Game/Units/Blueprints/SUnitConfig` _mainmodule _moduleonsockets _coords _direction false _side _tempstate) true)
        (else
          (return (struct) false))))))

(fn `ComputeMove`
  (params (FieldState :type "/Game/TankChess/Game/Field/Blueprints/SFieldState Structure") (UnitConfig :type "/Game/TankChess/Game/Units/Blueprints/SUnitConfig Structure") (Move :type "/Game/TankChess/Game/Units/Blueprints/SUnitMove Structure"))
  (returns (NewFieldState :type "/Game/TankChess/Game/Field/Blueprints/SFieldState Structure") (NewUnitConfig :type "/Game/TankChess/Game/Units/Blueprints/SUnitConfig Structure") (Possible :type Boolean))
  (locals (Delta :type "/Game/TankChess/Game/Field/Blueprints/SFieldCellCoords Structure"))
  (bind (_move_activecomponent _move_targetcoords _move_movement) (break `/Game/TankChess/Game/Units/Blueprints/SUnitMove` (`local.Move`)))
  (bind (_unitconfig_mainmodule _unitconfig_moduleonsockets _unitconfig_coords _unitconfig_direction _unitconfig_alive _unitconfig_side) (break `/Game/TankChess/Game/Units/Blueprints/SUnitConfig` (`local.UnitConfig`)))
  (bind (_unitconfig_mainmodule_2 _unitconfig_moduleonsockets_2 _unitconfig_coords_2 _unitconfig_direction_2) (break `/Game/TankChess/Game/Units/Blueprints/SUnitConfig` (`local.UnitConfig`)))
  (bind (_move_activecomponent_2 _move_targetcoords_2 _move_movement_2) (break `/Game/TankChess/Game/Units/Blueprints/SUnitMove` (`local.Move`)))
  (bind _unitconfig (`local.UnitConfig`))
  (bind _unitconfig_2 (`local.UnitConfig`))
  (bind (_cellfound _unitfound _landscapetype) (`/Game/TankChess/Game/BPFL_CellsAndUnits.GetCell` (`local.FieldState`) (`/Game/TankChess/Game/Units/Blueprints/BPFL_CoordsAndDirectionTransforms.AddCoords` _unitconfig_coords_2 (`local.Delta`))))
  (bind _sunitconfig (make `/Game/TankChess/Game/Units/Blueprints/SUnitConfig` (break `/Game/TankChess/Game/Units/Blueprints/SUnitConfig` _unitconfig) (`.ModuleOnSockets_65_93C0F6A14F5C249A946557A0ACBCDE35` (break `/Game/TankChess/Game/Units/Blueprints/SUnitConfig` _unitconfig)) (`/Game/TankChess/Game/Units/Blueprints/BPFL_CoordsAndDirectionTransforms.AddCoords` (`.Coords_47_E98C47904C4A4C6B43CCA291531B50D8` (break `/Game/TankChess/Game/Units/Blueprints/SUnitConfig` _unitconfig)) (`local.Delta`)) (`.Direction_56_4F2B10F847F49B1199F4DC823B142897` (break `/Game/TankChess/Game/Units/Blueprints/SUnitConfig` _unitconfig)) (`.Alive_50_F54C53F84EFA66D3B0170BB8E9F0CD80` (break `/Game/TankChess/Game/Units/Blueprints/SUnitConfig` _unitconfig)) (`.Side_59_393DC6B94AC999E7C6758C8FD57E2723` (break `/Game/TankChess/Game/Units/Blueprints/SUnitConfig` _unitconfig)) (make `/Game/TankChess/Game/Units/Blueprints/SUnitTempState` (select `bool` (`|EnumEquality` _move_movement "NewEnumerator1") :`false` (- (break `/Game/TankChess/Game/Units/Blueprints/SUnitTempState` (`.TempState_62_5ABFF3A34B4DD39392594A92040E2E81` (break `/Game/TankChess/Game/Units/Blueprints/SUnitConfig` _unitconfig))) 1)) (`.CanUse_23_BE99ED37467B2319636ED0A69AB3D10F` (break `/Game/TankChess/Game/Units/Blueprints/SUnitTempState` (`.TempState_62_5ABFF3A34B4DD39392594A92040E2E81` (break `/Game/TankChess/Game/Units/Blueprints/SUnitConfig` _unitconfig)))))))
  (if (> (break `/Game/TankChess/Game/Units/Blueprints/SUnitTempState` (`.TempState_62_5ABFF3A34B4DD39392594A92040E2E81` (break `/Game/TankChess/Game/Units/Blueprints/SUnitConfig` UnitConfig))) 0)
    (switch `/Game/TankChess/Game/Units/Blueprints/Modules/MovementModules/EMovements` _move_movement_2
      (:`NewEnumerator0`
        _)
      (:`NewEnumerator1`
        _)
      (:`NewEnumerator2`
        (bind _newdirection (`/Game/TankChess/Game/Units/Blueprints/BPFL_CoordsAndDirectionTransforms.GetDirectionAfterRotate` _move_movement_2 (`.Direction_56_4F2B10F847F49B1199F4DC823B142897` (break `/Game/TankChess/Game/Units/Blueprints/SUnitConfig` _unitconfig_2)) :!label _label))
        (bind _sunitconfig_2 (make `/Game/TankChess/Game/Units/Blueprints/SUnitConfig` (break `/Game/TankChess/Game/Units/Blueprints/SUnitConfig` _unitconfig_2) (`.ModuleOnSockets_65_93C0F6A14F5C249A946557A0ACBCDE35` (break `/Game/TankChess/Game/Units/Blueprints/SUnitConfig` _unitconfig_2)) (`.Coords_47_E98C47904C4A4C6B43CCA291531B50D8` (break `/Game/TankChess/Game/Units/Blueprints/SUnitConfig` _unitconfig_2)) _newdirection (`.Alive_50_F54C53F84EFA66D3B0170BB8E9F0CD80` (break `/Game/TankChess/Game/Units/Blueprints/SUnitConfig` _unitconfig_2)) (`.Side_59_393DC6B94AC999E7C6758C8FD57E2723` (break `/Game/TankChess/Game/Units/Blueprints/SUnitConfig` _unitconfig_2)) (make `/Game/TankChess/Game/Units/Blueprints/SUnitTempState` (- (break `/Game/TankChess/Game/Units/Blueprints/SUnitTempState` (`.TempState_62_5ABFF3A34B4DD39392594A92040E2E81` (break `/Game/TankChess/Game/Units/Blueprints/SUnitConfig` _unitconfig_2))) 1) (`.CanUse_23_BE99ED37467B2319636ED0A69AB3D10F` (break `/Game/TankChess/Game/Units/Blueprints/SUnitTempState` (`.TempState_62_5ABFF3A34B4DD39392594A92040E2E81` (break `/Game/TankChess/Game/Units/Blueprints/SUnitConfig` _unitconfig_2)))))))
        (bind _newfieldstate (`/Game/TankChess/Game/BPFL_CellsAndUnits.ChangeUnit` (`local.FieldState`) (`.Coords_47_E98C47904C4A4C6B43CCA291531B50D8` (break `/Game/TankChess/Game/Units/Blueprints/SUnitConfig` _unitconfig_2)) _sunitconfig_2))
        (return _newfieldstate _sunitconfig_2 true))
      (:`NewEnumerator3`
        (goto _label)))
    (bind _delta (`/Game/TankChess/Game/Units/Blueprints/BPFL_CoordsAndDirectionTransforms.GetDeltaCoordsByDirection` _unitconfig_direction_2))
    (bind _output_get (set `local.Delta` _delta))
    (if (`|EnumEquality` _move_movement_2 "NewEnumerator1")
      (set `local.Delta` (`/Game/TankChess/Game/Units/Blueprints/BPFL_CoordsAndDirectionTransforms.MultiplyCoords` _output_get -1)))
    (bind _returnvalue (`|GetDataTableRow` "/Game/TankChess/Game/Units/Blueprints/Modules/DT_UnitModules.DT_UnitModules" _unitconfig_mainmodule_2)
      (:`then`
        (if (and _cellfound (not _unitfound) (`BlueprintSetLibrary.Set_Contains` (`.possibleLandscapeTypes_18_325AA1B743E4368F4960A1A4BF9C1399` (break `/Game/TankChess/Game/Units/Blueprints/Modules/TableStructures/SModuleSettings` (`.Settings_12_A8061B9948A0E1B34868A88E70641730` (break `/Game/TankChess/Game/Units/Blueprints/Modules/TableStructures/SModuleDescription` _returnvalue)))) _landscapetype))
          (if (`|EnumEquality` _landscapetype "NewEnumerator3")
            (bind _owner (message `/Game/TankChess/Game/BPI_GameStateMain.GetOwnerOfBaseCell` (`GameplayStatics.GetGameState`) (`/Game/TankChess/Game/Units/Blueprints/BPFL_CoordsAndDirectionTransforms.AddCoords` _unitconfig_coords (`local.Delta`))))
            (if (`|EnumEquality` _owner _unitconfig_side)
              (bind _values (`BlueprintMapLibrary.Map_Values` _unitconfig_moduleonsockets))
              (for _array_element _values
                (bind _returnvalue_2 (`|GetDataTableRow` "/Game/TankChess/Game/Units/Blueprints/Modules/DT_UnitModules.DT_UnitModules" _array_element)
                  (:`then`
                    (castclass `/Game/TankChess/Game/Units/Blueprints/Modules/OtherModules/BP_ComTankAntenneModuleComponent` (break `/Game/TankChess/Game/Units/Blueprints/Modules/TableStructures/SModuleDescription` _returnvalue_2))
                    (bind _newfieldstate_2 (`/Game/TankChess/Game/BPFL_CellsAndUnits.ChangeUnit` (`local.FieldState`) (`.Coords_47_E98C47904C4A4C6B43CCA291531B50D8` (break `/Game/TankChess/Game/Units/Blueprints/SUnitConfig` _unitconfig)) _sunitconfig :!label _label_2))
                    (return _newfieldstate_2 _sunitconfig true)))))
            (return (struct) (struct) false)
            (else
              (goto _label_2)))
          (else
            (return (struct) (struct) false)))))
    (else
      (return (struct) (struct) false))))

(fn `GetPossibleMoves`
  (params (FieldState :type "/Game/TankChess/Game/Field/Blueprints/SFieldState Structure") (UnitConfig :type "/Game/TankChess/Game/Units/Blueprints/SUnitConfig Structure"))
  (returns (PossibleMoves :type "Set of /Game/TankChess/Game/Units/Blueprints/SUnitMove Structure"))
  (locals (Moves :type "Set of /Game/TankChess/Game/Units/Blueprints/SUnitMove Structure"))
  (bind _enumvalue (foreach `/Game/TankChess/Game/Units/Blueprints/Modules/MovementModules/EMovements` false)
    (:`LoopBody`
      (bind _sunitmove (make `/Game/TankChess/Game/Units/Blueprints/SUnitMove` (`self.SocketName`) (struct :`XCoord` -2 :`YCoord` -2) _enumvalue))
      (bind (_newfieldstate _newunitconfig _possible) (`self.ComputeMove` FieldState UnitConfig _sunitmove))
      (if _possible
        (`BlueprintSetLibrary.Set_Add` (`local.Moves`) _sunitmove)))
    (:`then`
      (return (`local.Moves`)))))

(fn `VisualizeMove`
  (params (Move :type "/Game/TankChess/Game/Units/Blueprints/SUnitMove Structure"))
  (locals (Delta :type "/Game/TankChess/Game/Field/Blueprints/SFieldCellCoords Structure"))
  (bind (_activecomponent _targetcoords _movement) (break `/Game/TankChess/Game/Units/Blueprints/SUnitMove` Move))
  (bind _asbp_unit (cast `/Game/TankChess/Game/Units/Blueprints/BP_Unit` (`self.GetOwner`)))
  (switch `/Game/TankChess/Game/Units/Blueprints/Modules/MovementModules/EMovements` _movement
    (:`NewEnumerator0`
      (bind (_unit_config_mainmodule _unit_config_moduleonsockets _unit_config_coords _unit_config_direction) (break `/Game/TankChess/Game/Units/Blueprints/SUnitConfig` (`/Game/TankChess/Game/Units/Blueprints/BP_Unit.Unit Config` _asbp_unit)))
      (bind _delta (`/Game/TankChess/Game/Units/Blueprints/BPFL_CoordsAndDirectionTransforms.GetDeltaCoordsByDirection` _unit_config_direction))
      (set `local.Delta` _delta)
      (`/Game/TankChess/Game/Units/Blueprints/BP_Unit.SetCoords` _asbp_unit (`/Game/TankChess/Game/Units/Blueprints/BPFL_CoordsAndDirectionTransforms.AddCoords` _unit_config_coords (`local.Delta`)) :!label _label))
    (:`NewEnumerator1`
      (bind _delta_2 (`/Game/TankChess/Game/Units/Blueprints/BPFL_CoordsAndDirectionTransforms.GetDeltaCoordsByDirection` _unit_config_direction))
      (set `local.Delta` (`/Game/TankChess/Game/Units/Blueprints/BPFL_CoordsAndDirectionTransforms.MultiplyCoords` _delta_2 -1))
      (goto _label))
    (:`NewEnumerator2`
      (bind _newdirection (`/Game/TankChess/Game/Units/Blueprints/BPFL_CoordsAndDirectionTransforms.GetDirectionAfterRotate` _movement _unit_config_direction :!label _label_2))
      (`/Game/TankChess/Game/Units/Blueprints/BP_Unit.SetDirection` _asbp_unit _newdirection))
    (:`NewEnumerator3`
      (goto _label_2))))