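; Tank-chess weapon module component that fires along three straight lines: the unit's facing and two rotated directions.
; GetTargets scans each line within the module's data-table range, blind zone and allowed landscapes, mapping damageable other-side units to post-hit configs.
; That map drives GetPossibleMoves and ComputeMove, which spends the module and updates both units.
; Damage comes from temporarily spawning the target's main-module component to call ApplyDamage, repeated in VisualizeMove for display.
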(fn `ComputeMove`
  (params (FieldState :type "/Game/TankChess/Game/Field/Blueprints/SFieldState Structure") (UnitConfig :type "/Game/TankChess/Game/Units/Blueprints/SUnitConfig Structure") (Move :type "/Game/TankChess/Game/Units/Blueprints/SUnitMove Structure"))
  (returns (NewFieldState :type "/Game/TankChess/Game/Field/Blueprints/SFieldState Structure") (NewUnitConfig :type "/Game/TankChess/Game/Units/Blueprints/SUnitConfig Structure") (Possible :type Boolean))
  (locals (newCanUse :type "Map of Name to Boolean"))
  (bind (_mainmodule _moduleonsockets _coords _direction _alive _side _tempstate) (break `/Game/TankChess/Game/Units/Blueprints/SUnitConfig` UnitConfig))
  (bind (_activecomponent _targetcoords) (break `/Game/TankChess/Game/Units/Blueprints/SUnitMove` Move))
  (bind _sunitconfig (make `/Game/TankChess/Game/Units/Blueprints/SUnitConfig` _mainmodule _moduleonsockets _coords _direction _alive _side (make `/Game/TankChess/Game/Units/Blueprints/SUnitTempState` 0 (`local.newCanUse`))))
  (bind _targets (`self.GetTargets` FieldState UnitConfig))
  (bind (_value _returnvalue) (`BlueprintMapLibrary.Map_Find` _targets _targetcoords))
  (if _returnvalue
    (bind _output_get (set `local.newCanUse` (`.CanUse_23_BE99ED37467B2319636ED0A69AB3D10F` (break `/Game/TankChess/Game/Units/Blueprints/SUnitTempState` _tempstate))))
    (`BlueprintMapLibrary.Map_Add` _output_get _activecomponent)
    (bind _newfieldstate (`/Game/TankChess/Game/BPFL_CellsAndUnits.ChangeUnit` FieldState _coords _sunitconfig))
    (bind _newfieldstate_2 (`/Game/TankChess/Game/BPFL_CellsAndUnits.ChangeUnit` _newfieldstate _targetcoords _value))
    (return _newfieldstate_2 _sunitconfig true)
    (else
      (return (struct) (struct) false))))

(fn `GetPossibleMoves`
  (params (FieldState :type "/Game/TankChess/Game/Field/Blueprints/SFieldState Structure") (UnitConfig :type "/Game/TankChess/Game/Units/Blueprints/SUnitConfig Structure"))
  (returns (PossibleMoves :type "Set of /Game/TankChess/Game/Units/Blueprints/SUnitMove Structure"))
  (locals (Moves :type "Set of /Game/TankChess/Game/Units/Blueprints/SUnitMove Structure"))
  (bind _targets (`self.GetTargets` FieldState UnitConfig))
  (bind _keys (`BlueprintMapLibrary.Map_Keys` _targets))
  (for _array_element _keys
    (`BlueprintSetLibrary.Set_Add` (`local.Moves`) (make `/Game/TankChess/Game/Units/Blueprints/SUnitMove` (`self.SocketName`) _array_element)))
  (return (`local.Moves`)))

(fn `GetTargets`
  (params (FieldState :type "/Game/TankChess/Game/Field/Blueprints/SFieldState Structure") (UnitConfig :type "/Game/TankChess/Game/Units/Blueprints/SUnitConfig Structure"))
  (returns (Targets :type "Map of /Game/TankChess/Game/Field/Blueprints/SFieldCellCoords Structure to /Game/TankChess/Game/Units/Blueprints/SUnitConfig Structure"))
  (locals (FireDirection :type "/Game/TankChess/Game/Units/Blueprints/EDirection Enum") (Delta :type "/Game/TankChess/Game/Field/Blueprints/SFieldCellCoords Structure") (index :type Integer) (TargetMap :type "Map of /Game/TankChess/Game/Field/Blueprints/SFieldCellCoords Structure to /Game/TankChess/Game/Units/Blueprints/SUnitConfig Structure"))
  (bind (_mainmodule _moduleonsockets _coords _direction _alive _side _tempstate) (break `/Game/TankChess/Game/Units/Blueprints/SUnitConfig` UnitConfig))
  (bind (_unitconfig_mainmodule _unitconfig_moduleonsockets _unitconfig_coords) (break `/Game/TankChess/Game/Units/Blueprints/SUnitConfig` (`local.UnitConfig`)))
  (bind (_unitconfig_mainmodule_2 _unitconfig_moduleonsockets_2 _unitconfig_coords_2 _unitconfig_direction _unitconfig_alive _unitconfig_side) (break `/Game/TankChess/Game/Units/Blueprints/SUnitConfig` (`local.UnitConfig`)))
  (bind (_unitconfig_mainmodule_3 _unitconfig_moduleonsockets_3 _unitconfig_coords_3) (break `/Game/TankChess/Game/Units/Blueprints/SUnitConfig` (`local.UnitConfig`)))
  (bind (_cellfound _unitfound _landscapetype _unitconfig) (`/Game/TankChess/Game/BPFL_CellsAndUnits.GetCell` (`local.FieldState`) (`/Game/TankChess/Game/Units/Blueprints/BPFL_CoordsAndDirectionTransforms.AddCoords` _unitconfig_coords (`/Game/TankChess/Game/Units/Blueprints/BPFL_CoordsAndDirectionTransforms.MultiplyCoords` (`local.Delta`) (`local.index`)))))
  (bind (_mainmodule_2 _moduleonsockets_2 _coords_2 _direction_2 _alive_2 _side_2) (break `/Game/TankChess/Game/Units/Blueprints/SUnitConfig` _unitconfig))
  (if (`BlueprintMapLibrary.Map_Find` (`.CanUse_23_BE99ED37467B2319636ED0A69AB3D10F` (break `/Game/TankChess/Game/Units/Blueprints/SUnitTempState` _tempstate)) (`self.SocketName`))
    (`|ExecutionSequence`
      (:`then_0`
        (bind _output_get (set `local.FireDirection` _direction))
        (bind _delta (`/Game/TankChess/Game/Units/Blueprints/BPFL_CoordsAndDirectionTransforms.GetDeltaCoordsByDirection` _output_get))
        (set `local.Delta` _delta)
        (bind _returnvalue (`|GetDataTableRow` "/Game/TankChess/Game/Units/Blueprints/Modules/DT_UnitModules.DT_UnitModules" (`BlueprintMapLibrary.Map_Find` _moduleonsockets (`self.SocketName`)))
          (:`then`
            _)))
      (:`then_1`
        (bind _newdirection (`/Game/TankChess/Game/Units/Blueprints/BPFL_CoordsAndDirectionTransforms.GetDirectionAfterRotate` "NewEnumerator2" _direction))
        (bind _output_get_2 (set `local.FireDirection` _newdirection))
        (bind _delta_2 (`/Game/TankChess/Game/Units/Blueprints/BPFL_CoordsAndDirectionTransforms.GetDeltaCoordsByDirection` _output_get_2))
        (set `local.Delta` _delta_2))
      (:`then_2`
        (bind _newdirection_2 (`/Game/TankChess/Game/Units/Blueprints/BPFL_CoordsAndDirectionTransforms.GetDirectionAfterRotate` "NewEnumerator3" _direction))
        (bind _output_get_3 (set `local.FireDirection` _newdirection_2))
        (bind _delta_3 (`/Game/TankChess/Game/Units/Blueprints/BPFL_CoordsAndDirectionTransforms.GetDeltaCoordsByDirection` _output_get_3))
        (set `local.Delta` _delta_3))
      (:`then_3`
        (return (`local.TargetMap`))))
    (set `local.index` 1)
    (bind (_armor _movepointsforstart _firepower _blindzone _maxfiredistance _possiblelandscapetypes) (break `/Game/TankChess/Game/Units/Blueprints/Modules/TableStructures/SModuleSettings` (`.Settings_12_A8061B9948A0E1B34868A88E70641730` (break `/Game/TankChess/Game/Units/Blueprints/Modules/TableStructures/SModuleDescription` _returnvalue))))
    (while (and _cellfound (`BlueprintSetLibrary.Set_Contains` _possiblelandscapetypes _landscapetype) (or (<= (`local.index`) _maxfiredistance) (== _maxfiredistance -1)))
      (if (and (> (`local.index`) _blindzone) _unitfound)
        (bind _returnvalue_2 (`|GetDataTableRow` "/Game/TankChess/Game/Units/Blueprints/Modules/DT_UnitModules.DT_UnitModules" _mainmodule_2)
          (:`then`
            (bind _returnvalue_3 (`|AddComponentByClass` (`self.GetOwner`) (break `/Game/TankChess/Game/Units/Blueprints/Modules/TableStructures/SModuleDescription` _returnvalue_2) "Main"))
            (bind _asbp_base_movement_unit_module_component (cast `/Game/TankChess/Game/Units/Blueprints/Modules/MovementModules/BP_BaseMovementUnitModuleComponent` _returnvalue_3))
            (bind (_newunitconfig _possible) (`/Game/TankChess/Game/Units/Blueprints/Modules/MovementModules/BP_BaseMovementUnitModuleComponent.ApplyDamage` _asbp_base_movement_unit_module_component _firepower (`local.FireDirection`) _unitconfig))
            (if (and _possible (`|EnumInequality` _side_2 _unitconfig_side))
              (`BlueprintMapLibrary.Map_Add` (`local.TargetMap`) (`/Game/TankChess/Game/Units/Blueprints/BPFL_CoordsAndDirectionTransforms.AddCoords` _unitconfig_coords_3 (`/Game/TankChess/Game/Units/Blueprints/BPFL_CoordsAndDirectionTransforms.MultiplyCoords` (`local.Delta`) (`local.index`))) _newunitconfig))
            (`/Engine/EditorBlueprintResources/StandardMacros.IncrementInt` (`local.index`)
              (:`  `
                (`self.K2_DestroyComponent` _returnvalue_3)))))
        (else
          (`/Engine/EditorBlueprintResources/StandardMacros.IncrementInt` (`local.index`)))))
    (else
      (return))))

(fn `VisualizeMove`
  (params (Move :type "/Game/TankChess/Game/Units/Blueprints/SUnitMove Structure"))
  (locals (FirePower :type Integer :default 0) (DeltaMap :type "Map of /Game/TankChess/Game/Field/Blueprints/SFieldCellCoords Structure to /Game/TankChess/Game/Units/Blueprints/EDirection Enum"))
  (bind (_activecomponent _targetcoords) (break `/Game/TankChess/Game/Units/Blueprints/SUnitMove` Move))
  (bind _asbp_unit (cast `/Game/TankChess/Game/Units/Blueprints/BP_Unit` (`self.GetOwner`)))
  (bind (_unit_config_mainmodule _unit_config_moduleonsockets _unit_config_coords) (break `/Game/TankChess/Game/Units/Blueprints/SUnitConfig` (`/Game/TankChess/Game/Units/Blueprints/BP_Unit.Unit Config` _asbp_unit)))
  (bind _returnvalue (`|GetDataTableRow` "/Game/TankChess/Game/Units/Blueprints/Modules/DT_UnitModules.DT_UnitModules" (`BlueprintMapLibrary.Map_Find` _unit_config_moduleonsockets (`self.SocketName`)))
    (:`then`
      (set `local.FirePower` (`.FirePower_10_3428025D4CF403F8858B5B83C7B1041B` (break `/Game/TankChess/Game/Units/Blueprints/Modules/TableStructures/SModuleSettings` (`.Settings_12_A8061B9948A0E1B34868A88E70641730` (break `/Game/TankChess/Game/Units/Blueprints/Modules/TableStructures/SModuleDescription` _returnvalue)))))
      (bind _outactors (`GameplayStatics.GetAllActorsOfClass` "/Game/TankChess/Game/Units/Blueprints/BP_Unit.BP_Unit_C"))
      (for _array_element _outactors
        (bind (_unit_config_mainmodule_2 _unit_config_moduleonsockets_2 _unit_config_coords_2) (break `/Game/TankChess/Game/Units/Blueprints/SUnitConfig` (`/Game/TankChess/Game/Units/Blueprints/BP_Unit.Unit Config` _array_element)))
        (if (`/Game/TankChess/Game/Units/Blueprints/BPFL_CoordsAndDirectionTransforms.EqualCoords` _targetcoords _unit_config_coords_2)
          (bind _returnvalue_2 (`|GetDataTableRow` "/Game/TankChess/Game/Units/Blueprints/Modules/DT_UnitModules.DT_UnitModules" _unit_config_mainmodule_2)
            (:`then`
              (bind _returnvalue_3 (`|AddComponentByClass` (`self.GetOwner`) (break `/Game/TankChess/Game/Units/Blueprints/Modules/TableStructures/SModuleDescription` _returnvalue_2) "Main"))
              (bind _asbp_base_movement_unit_module_component (cast `/Game/TankChess/Game/Units/Blueprints/Modules/MovementModules/BP_BaseMovementUnitModuleComponent` _returnvalue_3))
              (bind (_xcoord _ycoord) (break `/Game/TankChess/Game/Field/Blueprints/SFieldCellCoords` (`/Game/TankChess/Game/Units/Blueprints/BPFL_CoordsAndDirectionTransforms.AddCoords` _targetcoords (`/Game/TankChess/Game/Units/Blueprints/BPFL_CoordsAndDirectionTransforms.MultiplyCoords` _unit_config_coords -1))))
              (bind _newunitconfig (`/Game/TankChess/Game/Units/Blueprints/Modules/MovementModules/BP_BaseMovementUnitModuleComponent.ApplyDamage` _asbp_base_movement_unit_module_component (`local.FirePower`) (`BlueprintMapLibrary.Map_Find` (`local.DeltaMap`) (make `/Game/TankChess/Game/Field/Blueprints/SFieldCellCoords` (`KismetMathLibrary.SignOfInteger` _xcoord) (`KismetMathLibrary.SignOfInteger` _ycoord))) (`/Game/TankChess/Game/Units/Blueprints/BP_Unit.Unit Config` _array_element)))
              (`/Game/TankChess/Game/Units/Blueprints/BP_Unit.VisualizeConfig` _array_element _newunitconfig)
              (`self.K2_DestroyComponent` _returnvalue_3))))))))