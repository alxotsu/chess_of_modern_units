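; BP_UnitHologram is a TankChess unit actor rendered as a tinted hologram.
; Its construction script runs the parent's, then calls SetColor, which stores color and light, creates a dynamic instance of M_TankHologram and applies it to every material slot on all skeletal mesh components.
; SetAlive and SetSide only rewrite their field in UnitConfig, with no visual update; the event graph holds only disabled stubs.
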(fn `Set Color`
  (params (Color :type "LinearColor Structure") (Light :type Boolean))
  (locals (HologramMaterial :type "MaterialInstanceDynamic Object Reference"))
  (set `self.HologramColor` Color)
  (set `self.Light` Light)
  (bind _returnvalue (`KismetMaterialLibrary.CreateDynamicMaterialInstance` "/Game/TankChess/Game/Units/Materials/M_TankHologram.M_TankHologram"))
  (bind _output_get (set `local.HologramMaterial` _returnvalue))
  (`MaterialInstanceDynamic.SetVectorParameterValue` _output_get "Color" (`self.HologramColor`))
  (`MaterialInstanceDynamic.SetScalarParameterValue` _output_get "Light" (`KismetMathLibrary.Conv_BoolToDouble` (`self.Light`)))
  (for _array_element (`self.K2_GetComponentsByClass` "/Script/Engine.SkeletalMeshComponent")
    (for _index (range (`PrimitiveComponent.GetNumMaterials` _array_element))
      (`PrimitiveComponent.SetMaterial` _array_element _index (`local.HologramMaterial`)))))

(fn `SetAlive`
  (params (Alive :type Boolean))
  (bind (_unit_config_mainmodule _unit_config_moduleonsockets _unit_config_coords _unit_config_direction _unit_config_alive _unit_config_side _unit_config_tempstate) (break `/Game/TankChess/Game/Units/Blueprints/SUnitConfig` (`self.Unit Config`)))
  (set `self.Unit Config` (make `/Game/TankChess/Game/Units/Blueprints/SUnitConfig` _unit_config_mainmodule _unit_config_moduleonsockets _unit_config_coords _unit_config_direction Alive _unit_config_side _unit_config_tempstate)))

(fn `SetSide`
  (params (Side :type "/Game/TankChess/Game/Player/EPlayerSide Enum" :default "NewEnumerator0"))
  (bind (_unit_config_mainmodule _unit_config_moduleonsockets _unit_config_coords _unit_config_direction _unit_config_alive _unit_config_side _unit_config_tempstate) (break `/Game/TankChess/Game/Units/Blueprints/SUnitConfig` (`self.Unit Config`)))
  (set `self.Unit Config` (make `/Game/TankChess/Game/Units/Blueprints/SUnitConfig` _unit_config_mainmodule _unit_config_moduleonsockets _unit_config_coords _unit_config_direction _unit_config_alive Side _unit_config_tempstate)))

(fn `UserConstructionScript`
  (`parent.UserConstructionScript`)
  (`self.Set Color` (`self.HologramColor`) (`self.Light`)))