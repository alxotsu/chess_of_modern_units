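; Unit component manager that equips and looks up modular components on the sockets of tank units.
; A socket-to-component map backs queries for component, class, usability and equipped type, with the "None" socket or class searches also covering the owner's main component.
; Equipping validates main component class, socket and candidate against DT_ComponentValidation, then replaces any different component with one spawned and attached to the owner's mesh.
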(fn `ComponentEquiped`
  (params (CompClass :type "/Game/TankChess/Game/Units/UnitComponents/Blueprints/BP_BaseUnitComponent Class Reference"))
  (returns (Find :type Boolean) (Compnent :type "/Game/TankChess/Game/Units/UnitComponents/Blueprints/BP_BaseUnitComponent Object Reference") (Socket :type Name))
  (if (`KismetMathLibrary.ClassIsChildOf` (`GameplayStatics.GetObjectClass` (`/Game/TankChess/Game/Units/Tanks/Blueprints/BP_BaseTank.MainComponent` (`self.UnitOwner`))) CompClass)
    (return true (`/Game/TankChess/Game/Units/Tanks/Blueprints/BP_BaseTank.MainComponent` (`self.UnitOwner`)) "None")
    (else
      (bind _keys (`BlueprintMapLibrary.Map_Keys` (`self.Components`)))
      (for _array_element _keys
        (bind _value (`BlueprintMapLibrary.Map_Find` (`self.Components`) _array_element))
        (if (`KismetMathLibrary.ClassIsChildOf` (`GameplayStatics.GetObjectClass` _value) CompClass)
          (return true _value _array_element)))
      (return false null "None"))))

(fn `EquipComponent`
  (params (Socket :type Name) (ComponentClass :type "/Game/TankChess/Game/Units/UnitComponents/Blueprints/BP_BaseUnitComponent Class Reference"))
  (returns (Return :type "/Game/TankChess/Game/Units/UnitComponents/Blueprints/BP_BaseUnitComponent Object Reference") (Equiped :type Boolean))
  (bind (_value _returnvalue) (`BlueprintMapLibrary.Map_Find` (`self.Components`) Socket))
  (bind _outrownames (`DataTableFunctionLibrary.GetDataTableRowNames` "/Game/TankChess/Game/Units/UnitComponents/Blueprints/DT_ComponentValidation.DT_ComponentValidation"))
  (for _array_element _outrownames
    (bind _returnvalue_2 (`|GetDataTableRow` "/Game/TankChess/Game/Units/UnitComponents/Blueprints/DT_ComponentValidation.DT_ComponentValidation" _array_element)
      (:`then`
        (if (and (== (break `/Game/TankChess/Game/Units/UnitComponents/Blueprints/SValidComponentsForMain` _returnvalue_2) (`GameplayStatics.GetObjectClass` (`/Game/TankChess/Game/Units/Tanks/Blueprints/BP_BaseTank.MainComponent` (`self.UnitOwner`)))) (== (`.SocketName_5_2793DECE4CAB464F1975869A8353C6B3` (break `/Game/TankChess/Game/Units/UnitComponents/Blueprints/SValidComponentsForMain` _returnvalue_2)) Socket) (`KismetArrayLibrary.Array_Contains` (`.PossibleComponents_9_DD12092B4E6C1D900ABEF9AD9A037766` (break `/Game/TankChess/Game/Units/UnitComponents/Blueprints/SValidComponentsForMain` _returnvalue_2)) ComponentClass))
          (if _returnvalue
            (if (!= ComponentClass (`GameplayStatics.GetObjectClass` _value))
              (`self.K2_DestroyComponent` _value)
              (bind _returnvalue_3 (`|AddComponentByClass` (`self.GetOwner`) ComponentClass false (`KismetMathLibrary.MakeTransform` (0.0 0.0 0.0)) :!label _label))
              (`SceneComponent.K2_AttachToComponent` _returnvalue_3 (`Character.Mesh` (`self.UnitOwner`)) Socket "KeepRelative" "KeepRelative" "KeepRelative" true)
              (`BlueprintMapLibrary.Map_Add` (`self.Components`) Socket _returnvalue_3)
              (set `/Game/TankChess/Game/Units/UnitComponents/Blueprints/BP_BaseUnitComponent.SocketName` Socket _returnvalue_3)
              (return _returnvalue_3 false))
            (else
              (goto _label)))))))
  (return null false))

(fn `GetComponentBySocket`
  (params (SockName :type Name))
  (returns (Component :type "/Game/TankChess/Game/Units/UnitComponents/Blueprints/BP_BaseUnitComponent Object Reference"))
  (if (== SockName "None")
    (return (`/Game/TankChess/Game/Units/Tanks/Blueprints/BP_BaseTank.MainComponent` (`self.UnitOwner`)))
    (else
      (return (`BlueprintMapLibrary.Map_Find` (`self.Components`) SockName)))))

(fn `GetComponentSockets`
  (returns (Components :type "Map of Name to /Game/TankChess/Game/Units/UnitComponents/Blueprints/BP_BaseUnitComponent Class Reference"))
  (locals (Output :type "Map of Name to /Game/TankChess/Game/Units/UnitComponents/Blueprints/BP_BaseUnitComponent Class Reference"))
  (bind _components (`self.Components`))
  (bind _keys (`BlueprintMapLibrary.Map_Keys` _components))
  (for _array_element _keys
    (`BlueprintMapLibrary.Map_Add` (`local.Output`) _array_element (`GameplayStatics.GetObjectClass` (`BlueprintMapLibrary.Map_Find` _components _array_element))))
  (return (`local.Output`)))

(fn `GetSocketsUsable`
  (returns (Components :type "Map of Name to Boolean"))
  (locals (Output :type "Map of Name to Boolean"))
  (bind _components (`self.Components`))
  (bind _keys (`BlueprintMapLibrary.Map_Keys` _components))
  (for _array_element _keys
    (`BlueprintMapLibrary.Map_Add` (`local.Output`) _array_element (`/Game/TankChess/Game/Units/UnitComponents/Blueprints/BP_BaseUnitComponent.Usable` (`BlueprintMapLibrary.Map_Find` _components _array_element))))
  (return (`local.Output`)))