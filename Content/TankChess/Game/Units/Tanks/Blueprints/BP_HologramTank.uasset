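; BP_HologramTank is a hologram copy of a parent tank, placed on the board by grid coordinates.
; SetParrent copies the parent's config and skeletal mesh, and SetTempState_0 saves a temporary state and applies its coordinates, direction and alive flag as config.
; SetMaterial puts one material on slot 0 of every child primitive, mirroring each matching parent component's visibility.
; SetCoords converts grid cells to world location at 100 units per cell.
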(fn `SetCoords`
  (params (Coords :type "/Game/TankChess/Game/Field/Blueprints/SFieldCellCoords Structure"))
  (bind (_xcoord _ycoord) (break `/Game/TankChess/Game/Field/Blueprints/SFieldCellCoords` Coords))
  (set `self.coords` Coords)
  (`SceneComponent.K2_SetWorldLocation` (`self.DefaultSceneRoot`) (`KismetMathLibrary.MakeVector` (* _xcoord 100.0) (* _ycoord 100.0)) false false))

(fn `SetMaterial`
  (params (Material :type "MaterialInstance Object Reference"))
  (for (_array_element _array_index) (`SceneComponent.GetChildrenComponents` (`self.DefaultSceneRoot`) true)
    (bind _asprimitive_component (cast `PrimitiveComponent` _array_element))
    (`PrimitiveComponent.SetMaterial` _asprimitive_component 0 Material)
    (`SceneComponent.SetVisibility` _asprimitive_component (`SceneComponent.IsVisible` (`|GetArrayItem` (`SceneComponent.GetChildrenComponents` (`/Game/TankChess/Game/Units/Tanks/Blueprints/BP_BaseTank.DefaultSceneRoot` (`self.parent`)) true) _array_index)) false)))

(fn `SetParrent`
  (params (parent :type "/Game/TankChess/Game/Units/Tanks/Blueprints/BP_BaseTank Object Reference"))
  (bind _output_get (set `self.parent` parent))
  (`self.SetConfig` (`self.GetConfig` _output_get))
  (`SkeletalMeshComponent.SetSkeletalMeshAsset` (`self.TankMesh`) (`SkeletalMeshComponent.GetSkeletalMeshAsset` (`/Game/TankChess/Game/Units/Tanks/Blueprints/BP_BaseTank.TankMesh` (`self.parent`)))))

(fn `SetPlayerSide`
  (params (PlayerSide :type "/Game/TankChess/Game/Player/EPlayerSide Enum" :default "NewEnumerator0")))

(fn `SetTempState_0`
  (params (TempState :type "/Game/TankChess/Game/Units/Tanks/Blueprints/STankTempState Structure (by ref)"))
  (bind (_coords _direction _alive) (break `/Game/TankChess/Game/Units/Tanks/Blueprints/STankTempState` TempState))
  (set `self.SavedTempState` TempState)
  (`self.SetConfig` (make `/Game/TankChess/Game/Units/Tanks/Blueprints/STankConfig` null _coords _direction _alive)))

(fn `UserConstructionScript`
  (`parent.UserConstructionScript`))