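; Blueprint function library of grid and tank-state helpers for TankChess.
; Map lookups resolve rotated, opposite and coordinate-delta directions, alongside basic cell coordinate math.
; Relative direction comes from rotating both inputs right until the observer reaches the enum's first entry.
; Config equality compares map keys and values as ordered arrays and ignores MovePoints, while config lookup falls back to the tank's own config.
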(fn `AddCoords`
  (params (Coords1 :type "/Game/TankChess/Game/Field/Blueprints/SFieldCellCoords Structure") (Coords2 :type "/Game/TankChess/Game/Field/Blueprints/SFieldCellCoords Structure"))
  (returns (CoordsOut :type "/Game/TankChess/Game/Field/Blueprints/SFieldCellCoords Structure"))
  (bind (_xcoord _ycoord) (break `/Game/TankChess/Game/Field/Blueprints/SFieldCellCoords` Coords1))
  (bind (_xcoord_2 _ycoord_2) (break `/Game/TankChess/Game/Field/Blueprints/SFieldCellCoords` Coords2))
  (return (make `/Game/TankChess/Game/Field/Blueprints/SFieldCellCoords` (+ _xcoord _xcoord_2) (+ _ycoord_2 _ycoord))))

(fn `EqualCoords`
  (params (Coords1 :type "/Game/TankChess/Game/Field/Blueprints/SFieldCellCoords Structure") (Coords2 :type "/Game/TankChess/Game/Field/Blueprints/SFieldCellCoords Structure"))
  (returns (Equal :type Boolean))
  (bind (_xcoord _ycoord) (break `/Game/TankChess/Game/Field/Blueprints/SFieldCellCoords` Coords1))
  (bind (_xcoord_2 _ycoord_2) (break `/Game/TankChess/Game/Field/Blueprints/SFieldCellCoords` Coords2))
  (return (and (== _xcoord _xcoord_2) (== _ycoord _ycoord_2))))

(fn `FindTankConfig`
  (params (TankConfigs :type "Map of /Game/TankChess/Game/Units/Tanks/Blueprints/BP_BaseTank Object Reference to /Game/TankChess/Game/Units/Tanks/Blueprints/STankConfig Structure") (Tank :type "/Game/TankChess/Game/Units/Tanks/Blueprints/BP_BaseTank Object Reference"))
  (returns (Config :type "/Game/TankChess/Game/Units/Tanks/Blueprints/STankConfig Structure"))
  (bind (_value _returnvalue) (`BlueprintMapLibrary.Map_Find` TankConfigs Tank))
  (if _returnvalue
    (return _value)
    (else
      (return (`/Game/TankChess/Game/Units/Tanks/Blueprints/BP_BaseTank.GetConfig` Tank)))))

(fn `GetDeltaCoordsByDirection`
  (params (Direction :type "/Game/TankChess/Game/Units/Tanks/Blueprints/EDirection Enum" :default "NewEnumerator0"))
  (returns (Delta :type "/Game/TankChess/Game/Field/Blueprints/SFieldCellCoords Structure"))
  (locals (DeltaMap :type "Map of /Game/TankChess/Game/Units/Tanks/Blueprints/EDirection Enum to /Game/TankChess/Game/Field/Blueprints/SFieldCellCoords Structure"))
  (return (`BlueprintMapLibrary.Map_Find` (`local.DeltaMap`) Direction)))

(fn `GetDiametralDirection`
  (params (Direction :type "/Game/TankChess/Game/Units/Tanks/Blueprints/EDirection Enum" :default "NewEnumerator0"))
  (returns (Diametral :type "/Game/TankChess/Game/Units/Tanks/Blueprints/EDirection Enum"))
  (locals (Directions :type "Map of /Game/TankChess/Game/Units/Tanks/Blueprints/EDirection Enum to /Game/TankChess/Game/Units/Tanks/Blueprints/EDirection Enum"))
  (return (`BlueprintMapLibrary.Map_Find` (`local.Directions`) Direction)))

(fn `GetDirectionAfterRotate`
  (params (Rotate :type "/Game/TankChess/Game/Units/UnitComponents/Blueprints/MovementComponents/EMovement Enum" :default "NewEnumerator0") (Direction :type "/Game/TankChess/Game/Units/Tanks/Blueprints/EDirection Enum" :default "NewEnumerator0"))
  (returns (NewDirection :type "/Game/TankChess/Game/Units/Tanks/Blueprints/EDirection Enum"))
  (locals (RightRotate :type "Map of /Game/TankChess/Game/Units/Tanks/Blueprints/EDirection Enum to /Game/TankChess/Game/Units/Tanks/Blueprints/EDirection Enum") (LeftRotate :type "Map of /Game/TankChess/Game/Units/Tanks/Blueprints/EDirection Enum to /Game/TankChess/Game/Units/Tanks/Blueprints/EDirection Enum"))
  (switch `/Game/TankChess/Game/Units/UnitComponents/Blueprints/MovementComponents/EMovement` Rotate
    (:`NewEnumerator2`
      (return (`BlueprintMapLibrary.Map_Find` (`local.LeftRotate`) Direction)))
    (:`NewEnumerator3`
      (return (`BlueprintMapLibrary.Map_Find` (`local.RightRotate`) Direction)))))

(fn `GetRelativeDirection`
  (params (AbsoluteDirection :type "/Game/TankChess/Game/Units/Tanks/Blueprints/EDirection Enum" :default "NewEnumerator0") (ObserverDirection :type "/Game/TankChess/Game/Units/Tanks/Blueprints/EDirection Enum" :default "NewEnumerator0"))
  (returns (RelativeDirection :type "/Game/TankChess/Game/Units/Tanks/Blueprints/EDirection Enum"))
  (locals (TempObserverDirection :type "/Game/TankChess/Game/Units/Tanks/Blueprints/EDirection Enum" :default "NewEnumerator0") (TempAbsoluteDirection :type "/Game/TankChess/Game/Units/Tanks/Blueprints/EDirection Enum" :default "NewEnumerator0"))
  (set `local.TempAbsoluteDirection` AbsoluteDirection)
  (bind _output_get (set `local.TempObserverDirection` ObserverDirection))
  (while (`|EnumInequality` _output_get "NewEnumerator0")
    (bind _newdirection (`self.GetDirectionAfterRotate` "NewEnumerator3" (`local.TempObserverDirection`)))
    (set `local.TempObserverDirection` _newdirection)
    (bind _newdirection_2 (`self.GetDirectionAfterRotate` "NewEnumerator3" (`local.TempAbsoluteDirection`)))
    (set `local.TempAbsoluteDirection` _newdirection_2))
  (return (`local.TempAbsoluteDirection`)))

(fn `MultiplyCoords`
  (params (Coords :type "/Game/TankChess/Game/Field/Blueprints/SFieldCellCoords Structure") (Multyplier :type Integer))
  (returns (CoordsOut :type "/Game/TankChess/Game/Field/Blueprints/SFieldCellCoords Structure"))
  (bind (_xcoord _ycoord) (break `/Game/TankChess/Game/Field/Blueprints/SFieldCellCoords` Coords))
  (return (make `/Game/TankChess/Game/Field/Blueprints/SFieldCellCoords` (* _xcoord Multyplier) (* _ycoord Multyplier))))

(fn `TankConfigsEqual`
  (params (`first config` :type "/Game/TankChess/Game/Units/Tanks/Blueprints/STankConfig Structure") (`second config` :type "/Game/TankChess/Game/Units/Tanks/Blueprints/STankConfig Structure"))
  (returns (Equal :type Boolean))
  (bind (_maincomponentclass _coords _direction _alive _side _components _tempstate) (break `/Game/TankChess/Game/Units/Tanks/Blueprints/STankConfig` `first config`))
  (bind (_maincomponentclass_2 _coords_2 _direction_2 _alive_2 _side_2 _components_2 _tempstate_2) (break `/Game/TankChess/Game/Units/Tanks/Blueprints/STankConfig` `second config`))
  (`|ExecutionSequence`
    (:`then_0`
      (bind _keys (`BlueprintMapLibrary.Map_Keys` _components))
      (bind _values (`BlueprintMapLibrary.Map_Values` _components))
      (bind _keys_2 (`BlueprintMapLibrary.Map_Keys` (`.CanUse_23_BE99ED37467B2319636ED0A69AB3D10F` (break `/Game/TankChess/Game/Units/Tanks/Blueprints/STankTempState` _tempstate))))
      (bind _values_2 (`BlueprintMapLibrary.Map_Values` (`.CanUse_23_BE99ED37467B2319636ED0A69AB3D10F` (break `/Game/TankChess/Game/Units/Tanks/Blueprints/STankTempState` _tempstate)))))
    (:`then_1`
      (bind _keys_3 (`BlueprintMapLibrary.Map_Keys` _components_2))
      (bind _values_3 (`BlueprintMapLibrary.Map_Values` _components_2))
      (bind _keys_4 (`BlueprintMapLibrary.Map_Keys` (`.CanUse_23_BE99ED37467B2319636ED0A69AB3D10F` (break `/Game/TankChess/Game/Units/Tanks/Blueprints/STankTempState` _tempstate_2))))
      (bind _values_4 (`BlueprintMapLibrary.Map_Values` (`.CanUse_23_BE99ED37467B2319636ED0A69AB3D10F` (break `/Game/TankChess/Game/Units/Tanks/Blueprints/STankTempState` _tempstate_2)))))
    (:`then_2`
      (return (and (`KismetArrayLibrary.Array_Identical` _values_2 _values_4) (`KismetArrayLibrary.Array_Identical` _keys_2 _keys_4) (`KismetArrayLibrary.Array_Identical` _values _values_3) (`KismetArrayLibrary.Array_Identical` _keys _keys_3) (== _maincomponentclass _maincomponentclass_2) (== (break `/Game/TankChess/Game/Field/Blueprints/SFieldCellCoords` _coords) (break `/Game/TankChess/Game/Field/Blueprints/SFieldCellCoords` _coords_2)) (== (`.YCoord_12_230624BA45D1462C62A7DA860B56371E` (break `/Game/TankChess/Game/Field/Blueprints/SFieldCellCoords` _coords)) (`.YCoord_12_230624BA45D1462C62A7DA860B56371E` (break `/Game/TankChess/Game/Field/Blueprints/SFieldCellCoords` _coords_2))) (`|EnumEquality` _direction _direction_2) (== _alive _alive_2) (`|EnumEquality` _side _side_2) true)))))