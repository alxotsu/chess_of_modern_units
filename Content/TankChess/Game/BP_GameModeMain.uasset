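; Game mode for the turn-based TankChess game, validating moves, checking for victory and alternating Black and White turns.
; MakeMove runs ProcessMove for the side to play, then CheckVictory, then either posts the end state to GameState or updates tanks' temporary states and switches player.
; A side wins by having a tank on a BP_CellBase, or when the opponent has no living tanks or loses all commander-antenna tanks, ignoring holograms.
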(event `self.ReceiveBeginPlay`
  (bind _asbp_game_instance (cast `/Game/TankChess/Core/BP_GameInstance` (`GameplayStatics.GetGameInstance`)))
  (message `/Game/TankChess/Game/BPI_GsmeStateMain.SetGameState` (`GameplayStatics.GetGameState`) (`/Game/TankChess/Core/BP_GameInstance.GameState` _asbp_game_instance)))

(event `/Game/TankChess/Game/BPI_GameModeMode.NextPlayer`
  (bind _returnvalue (`GameplayStatics.GetGameState`))
  (bind _playerside (message `/Game/TankChess/Game/Player/BPI_HavePlayerSide.GetPlayerSide` _returnvalue))
  (bind _output (message `/Game/TankChess/Game/Player/BPI_HavePlayerSide.SetPlayerSide` _returnvalue (select `/Game/TankChess/Game/Player/EPlayerSide` _playerside :`NewEnumerator0` "NewEnumerator1" :`NewEnumerator1` "NewEnumerator0" :!type "/Game/TankChess/Game/Player/EPlayerSide Enum")))
  (message `/Game/TankChess/Game/Player/BPI_HavePlayerSide.SetPlayerSide` (`GameplayStatics.GetPlayerController` 0) _output))

(fn `CheckVictory`
  (returns (Victory :type Boolean) (Victor :type "/Game/TankChess/Game/Player/EPlayerSide Enum"))
  (locals (HaveAliveTanks :type "Map of /Game/TankChess/Game/Player/EPlayerSide Enum to Boolean") (HaveComTanks :type "Map of /Game/TankChess/Game/Player/EPlayerSide Enum to Boolean") (HaveAliveComTanks :type "Map of /Game/TankChess/Game/Player/EPlayerSide Enum to Boolean"))
  (`|ExecutionSequence`
    (:`then_0`
      (bind _outactors (`GameplayStatics.GetAllActorsOfClass` "/Game/TankChess/Game/Field/Blueprints/BP_CellBase.BP_CellBase_C"))
      (for _array_element _outactors
        (bind _tank (`/Game/TankChess/Game/Field/Blueprints/BP_Cell.Tank` _array_element))
        (`/Engine/EditorBlueprintResources/StandardMacros.IsValid` _tank
          (:`Is Valid`
            (return true (`/Game/TankChess/Game/Units/Tanks/Blueprints/BP_BaseTank.Side` _tank))))))
    (:`then_1`
      (bind _outactors_2 (`GameplayStatics.GetAllActorsOfClass` "/Game/TankChess/Game/Units/Tanks/Blueprints/BP_BaseTank.BP_BaseTank_C"))
      (for _array_element_2 _outactors_2
        (cast `/Game/TankChess/Game/Units/Tanks/Blueprints/BP_HologramTank` _array_element_2
          (:`CastFailed`
            (if (`/Game/TankChess/Game/Units/Tanks/Blueprints/BP_BaseTank.Alive` _array_element_2)
              (bind _side (`/Game/TankChess/Game/Units/Tanks/Blueprints/BP_BaseTank.Side` _array_element_2))
              (`BlueprintMapLibrary.Map_Add` (`local.HaveAliveTanks`) _side true))
            (if (`/Game/TankChess/Game/Units/UnitComponents/Blueprints/BP_UnitComponentManagerComponent.ItemEquiped` (`/Game/TankChess/Game/Units/Tanks/Blueprints/BP_BaseTank.ItemManager` _array_element_2) "/Game/TankChess/Game/Units/UnitComponents/Blueprints/Implementations/BP_ComanderAntenneComponent.BP_ComanderAntenneComponent_C")
              (`BlueprintMapLibrary.Map_Add` (`local.HaveComTanks`) _side true)
              (if (`/Game/TankChess/Game/Units/Tanks/Blueprints/BP_BaseTank.Alive` _array_element_2)
                (`BlueprintMapLibrary.Map_Add` (`local.HaveAliveComTanks`) _side true))))))
      (bind _enumvalue (foreach `/Game/TankChess/Game/Player/EPlayerSide` false)
        (:`LoopBody`
          (if (`BlueprintMapLibrary.Map_Find` (`local.HaveAliveTanks`) _enumvalue)
            (if (and (`BlueprintMapLibrary.Map_Find` (`local.HaveComTanks`) _enumvalue) (not (`BlueprintMapLibrary.Map_Find` (`local.HaveAliveComTanks`) _enumvalue)))
              (return true (select `/Game/TankChess/Game/Player/EPlayerSide` _enumvalue :`NewEnumerator0` "NewEnumerator1" :`NewEnumerator1` "NewEnumerator0" :!type "/Game/TankChess/Game/Player/EPlayerSide Enum")))
            (else
              (return true (select `/Game/TankChess/Game/Player/EPlayerSide` _enumvalue :`NewEnumerator0` "NewEnumerator1" :`NewEnumerator1` "NewEnumerator0" :!type "/Game/TankChess/Game/Player/EPlayerSide Enum")))))))
    (:`then_2`
      (return false "NewEnumerator0"))))

(fn `MakeMove`
  (params (Tank :type "/Game/TankChess/Game/Units/Tanks/Blueprints/BP_BaseTank Object Reference") (Moves :type "Array of /Game/TankChess/Game/Units/Tanks/Blueprints/STankMove Structure (by ref)"))
  (returns (Valid :type Boolean))
  (bind _valid (`self.ProcessMove` Tank Moves))
  (if _valid
    (bind (_victory _victor) (`self.CheckVictory`))
    (if _victory
      (message `/Game/TankChess/Game/BPI_GsmeStateMain.SetEmdGameState` (`GameplayStatics.GetGameState`) (make `/Game/TankChess/Game/SEndGameState` _victor true))
      (return true)
      (else
        (`|ExecutionSequence`
          (:`then_0`
            (bind _outactors (`GameplayStatics.GetAllActorsOfClass` "/Game/TankChess/Game/Units/Tanks/Blueprints/BP_BaseTank.BP_BaseTank_C"))
            (for _array_element _outactors
              (`/Game/TankChess/Game/Units/Tanks/Blueprints/BP_BaseTank.Update Temp State` _array_element)))
          (:`then_1`
            (`self.NextPlayer`)
            (return true)))))
    (else
      (return false))))

(fn `ProcessMove`
  (params (Tank :type "/Game/TankChess/Game/Units/Tanks/Blueprints/BP_BaseTank Object Reference") (Move :type "Array of /Game/TankChess/Game/Units/Tanks/Blueprints/STankMove Structure"))
  (returns (Valid :type Boolean) (OutputState :type "/Game/TankChess/Game/Units/Tanks/Blueprints/STankTempState Structure"))
  (bind _playerside (message `/Game/TankChess/Game/Player/BPI_HavePlayerSide.GetPlayerSide` (`GameplayStatics.GetGameState`)))
  (if (`|EnumEquality` _playerside (`/Game/TankChess/Game/Units/Tanks/Blueprints/BP_BaseTank.Side` Tank))
    (bind _isvalid (`/Game/TankChess/Game/Units/Tanks/Blueprints/BP_BaseTank.ValidateMove` Tank Move))
    (if _isvalid
      (bind _finalstate (`/Game/TankChess/Game/Units/Tanks/Blueprints/BP_BaseTank.MakeMove` Tank Move))
      (return true _finalstate)
      (else
        _)))
  (return false))

(fn `UserConstructionScript`)