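; BP_Field is the TankChess board actor that builds the playing field from a game state and exports it back.
; SetFieldState clears the board, spawns a coordinate-keyed cell map with landscapes and a base row for each side beyond the Y edges, then spawns configured tanks.
; UpdateFieldState positions cells and their tanks and alternates checkerboard materials.
; GetFieldState gathers landscapes and tank configs, inferring field size from the last map key.
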(event `self.ReceiveDestroyed`
  (`self.ClearField`))

(fn `ClearField`
  (bind _values (`BlueprintMapLibrary.Map_Values` (`self.Cells`)))
  (for _array_element _values
    (`self.K2_DestroyActor` (`/Game/TankChess/Game/Field/Blueprints/BP_Cell.Tank` _array_element))
    (`self.K2_DestroyActor` _array_element))
  (`BlueprintMapLibrary.Map_Clear` (`self.Cells`)))

(fn `GetFieldSize`
  (returns (X :type Integer) (Y :type Integer))
  (bind _keys (`BlueprintMapLibrary.Map_Keys` (`self.Cells`)))
  (bind (_xcoord _ycoord) (break `/Game/TankChess/Game/Field/Blueprints/SFieldCellCoords` (`|GetArrayItem` _keys (- (`KismetArrayLibrary.Array_Length` _keys) 1))))
  (return (+ _xcoord 1) (+ _ycoord 0)))

(fn `GetFieldState`
  (returns (FieldState :type "/Game/TankChess/Core/S_GameState Structure"))
  (locals (TankConfigs :type "Array of /Game/TankChess/Game/Units/Tanks/Blueprints/STankConfig Structure") (Landscapes :type "Map of /Game/TankChess/Game/Field/Blueprints/SFieldCellCoords Structure to /Game/TankChess/Game/Field/Blueprints/ELandscapeType Enum"))
  (bind (_x _y) (`self.GetFieldSize`))
  (bind _values (`BlueprintMapLibrary.Map_Values` (`self.Cells`)))
  (for _array_element _values
    (bind _landscape (`/Game/TankChess/Game/Field/Blueprints/BP_Cell.Landscape` _array_element))
    (if (`|EnumInequality` _landscape "NewEnumerator0")
      (`BlueprintMapLibrary.Map_Add` (`local.Landscapes`) (`/Game/TankChess/Game/Field/Blueprints/BP_Cell.Coords` _array_element) _landscape))
    (bind _tank (`/Game/TankChess/Game/Field/Blueprints/BP_Cell.Tank` _array_element))
    (`/Engine/EditorBlueprintResources/StandardMacros.IsValid` _tank
      (:`Is Valid`
        (`KismetArrayLibrary.Array_Add` (`local.TankConfigs`) (`/Game/TankChess/Game/Units/Tanks/Blueprints/BP_BaseTank.GetConfig` _tank)))))
  (return (make `/Game/TankChess/Core/S_GameState` _x _y (`local.Landscapes`) (`local.TankConfigs`) "NewEnumerator0" (struct))))

(fn `SetFieldState`
  (params (GameState :type "/Game/TankChess/Core/S_GameState Structure"))
  (bind (_fieldsizex _fieldsizey _fieldlandscapes _fieldtanks) (break `/Game/TankChess/Core/S_GameState` GameState))
  (bind _cells (`self.Cells`))
  (`self.ClearField`)
  (`|ExecutionSequence`
    (:`then_0`
      (for _index (range _fieldsizex)
        (for _index_2 (range _fieldsizey)
          (bind _returnvalue (`|SpawnActorFromClass` "/Game/TankChess/Game/Field/Blueprints/BP_Cell.BP_Cell_C" (`KismetMathLibrary.MakeTransform` (0.0 0.0 0.0)) "Undefined" "MultiplyWithRoot" null null))
          (bind _sfieldcellcoords (make `/Game/TankChess/Game/Field/Blueprints/SFieldCellCoords` _index _index_2))
          (`BlueprintMapLibrary.Map_Add` _cells _sfieldcellcoords _returnvalue)
          (set `/Game/TankChess/Game/Field/Blueprints/BP_Cell.Coords` _sfieldcellcoords _returnvalue)
          (bind (_value _returnvalue_2) (`BlueprintMapLibrary.Map_Find` (`.FieldLandscapes_18_CD4EF2A64C7A24FCE76F409D8E0F77F9` (break `/Game/TankChess/Core/S_GameState` (`local.GameState`))) _sfieldcellcoords))
          (if _returnvalue_2
            (`/Game/TankChess/Game/Field/Blueprints/BP_Cell.SetLandscapeType` _returnvalue _value)))
        (bind _returnvalue_3 (`|SpawnActorFromClass` "/Game/TankChess/Game/Field/Blueprints/BP_CellBase.BP_CellBase_C" (`KismetMathLibrary.MakeTransform` (0.0 0.0 0.0)) "Undefined" "MultiplyWithRoot" null null))
        (bind _sfieldcellcoords_2 (make `/Game/TankChess/Game/Field/Blueprints/SFieldCellCoords` _index -1))
        (`BlueprintMapLibrary.Map_Add` _cells _sfieldcellcoords_2 _returnvalue_3)
        (set `/Game/TankChess/Game/Field/Blueprints/BP_Cell.Coords` _sfieldcellcoords_2 _returnvalue_3)
        (set `/Game/TankChess/Game/Field/Blueprints/BP_CellBase.OwnerSide` "NewEnumerator1" _returnvalue_3)
        (bind _returnvalue_4 (`|SpawnActorFromClass` "/Game/TankChess/Game/Field/Blueprints/BP_CellBase.BP_CellBase_C" (`KismetMathLibrary.MakeTransform` (0.0 0.0 0.0)) "Undefined" "MultiplyWithRoot" null null))
        (bind _sfieldcellcoords_3 (make `/Game/TankChess/Game/Field/Blueprints/SFieldCellCoords` _index (`.FieldSizeY_12_0239A41A4C932A91DB378797E67E94F5` (break `/Game/TankChess/Core/S_GameState` (`local.GameState`)))))
        (`BlueprintMapLibrary.Map_Add` (`self.Cells`) _sfieldcellcoords_3 _returnvalue_4)
        (set `/Game/TankChess/Game/Field/Blueprints/BP_Cell.Coords` _sfieldcellcoords_3 _returnvalue_4)
        (set `/Game/TankChess/Game/Field/Blueprints/BP_CellBase.OwnerSide` "NewEnumerator0" _returnvalue_4)))
    (:`then_1`
      (for _array_element _fieldtanks
        (bind _returnvalue_5 (`|SpawnActorFromClass` (`.Class_2_7A09680943D84828EF1AE5B72B04360D` (break `/Game/TankChess/Game/Units/Tanks/Blueprints/STankConfig` _array_element)) (`KismetMathLibrary.MakeTransform` (0.0 0.0 0.0)) "Undefined" "MultiplyWithRoot" null null))
        (`/Game/TankChess/Game/Units/Tanks/Blueprints/BP_BaseTank.SetConfig` _returnvalue_5 _array_element)
        (`/Game/TankChess/Game/Units/Tanks/Blueprints/BP_BaseTank.Update Temp State` _returnvalue_5)))
    (:`then_2`
      (`self.UpdateFieldState`))))

(fn `UpdateFieldState`
  (locals (MaterialForCell :type "MaterialInstance Object Reference" :default "/Script/Engine.MaterialInstanceConstant'/Game/TankChess/Game/Field/Materials/MI_CellDark.MI_CellDark'"))
  (bind _values (`BlueprintMapLibrary.Map_Values` (`self.Cells`)))
  (for _array_element _values
    (bind _coords (`/Game/TankChess/Game/Field/Blueprints/BP_Cell.Coords` _array_element))
    (if (or (!= (`.YCoord_12_230624BA45D1462C62A7DA860B56371E` (break `/Game/TankChess/Game/Field/Blueprints/SFieldCellCoords` _coords)) 0) (== (mod (`.Y` (`self.GetFieldSize`)) 2) 1))
      (if (== (`local.MaterialForCell`) (`self.LightCellMaterial`))
        (set `local.MaterialForCell` (`self.DarkCellMaterial`))
        (else
          (set `local.MaterialForCell` (`self.LightCellMaterial`)))))
    (bind (_xcoord _ycoord) (break `/Game/TankChess/Game/Field/Blueprints/SFieldCellCoords` _coords))
    (`SceneComponent.K2_SetWorldLocation` (`/Game/TankChess/Game/Field/Blueprints/BP_Cell.DefaultSceneRoot` _array_element) (`KismetMathLibrary.MakeVector` (* _xcoord 100.0) (* _ycoord 100.0)) false false)
    (`PrimitiveComponent.SetMaterial` (`/Game/TankChess/Game/Field/Blueprints/BP_Cell.Cube1` _array_element) 0 (`local.MaterialForCell`))
    (bind _tank (`/Game/TankChess/Game/Field/Blueprints/BP_Cell.Tank` _array_element))
    (`/Engine/EditorBlueprintResources/StandardMacros.IsValid` _tank
      (:`Is Valid`
        (`/Game/TankChess/Game/Units/Tanks/Blueprints/BP_BaseTank.SetCoords` _tank _coords)))))

(fn `UserConstructionScript`)